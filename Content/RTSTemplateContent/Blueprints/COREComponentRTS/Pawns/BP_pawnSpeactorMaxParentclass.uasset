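; Parent spectator pawn for the RTS template that acts as a player-controlled camera, with panning and height-based zoom.
; Move and zoom axes feed movement input along fixed world axes, while held ZoomIn/ZoomOut actions open Tick gates for continuous vertical movement.
; The mouse wheel instead applies a swept local Z offset.
; Possession caches the player controller, but the initial-rotation OnRep is empty, with its rotation and debug logic left disconnected.
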(event EventTick
  (params (DeltaSeconds :type Float%20%28single-precision%29))
  (Utilities|FlowControl|Sequence
    (:then_0
      (Utilities|FlowControl|Gate true
        (:Exit
          (Pawn|Input|AddMovementInput (Math|Vector|MakeVector 0.0 0.0 -5e+01) 5.0 false))))
    (:then_1
      (Utilities|FlowControl|Gate true
        (:Exit
          (Pawn|Input|AddMovementInput (Math|Vector|MakeVector 0.0 0.0 5e+01) 5.0 false))))))

(event EventPossessed
  (params (NewController :type Controller%20Object%20Reference))
  (bind _asplayer_controller (Utilities|Casting|CastToPlayerController NewController)))

(event EventBeginPlay)

(event EventActorBeginOverlap
  (params (OtherActor :type Actor%20Object%20Reference)))

(event Input|ActionEvents|InputActionZoomIn
  (params (Key :type Key%20Structure :default "None"))
  (:Pressed
    (Utilities|FlowControl|Gate true) ; enters at Open
  )
  (:Released
    (Utilities|FlowControl|Gate true) ; enters at Close
  ))

(event Input|ActionEvents|InputActionZoomOut
  (params (Key :type Key%20Structure :default "None"))
  (:Pressed
    (Utilities|FlowControl|Gate true) ; enters at Open
  )
  (:Released
    (Utilities|FlowControl|Gate true) ; enters at Close
  ))

(event Input|AxisEvents|InputAxisZoomMouseWheel
  (params (AxisValue :type Float%20%28single-precision%29))
  (Class|Actor|AddActorLocalTransform (Math|Transform|MakeTransform (Math|Vector|MakeVector 0.0 0.0 (* AxisValue -1e+03))) true false))

(event Input|AxisEvents|InputAxisMoveRight
  (params (AxisValue :type Float%20%28single-precision%29))
  ;[1 1 1] Prevents the camera from not douign waht i want
  ;;[0.1221 1 0] Inputs
  (Pawn|Input|AddMovementInput (Math|Vector|MakeVector 0.0 (* AxisValue -1e+03) 0.0) 5.0 false))

(event Input|AxisEvents|InputAxisZoomInOut
  (params (AxisValue :type Float%20%28single-precision%29))
  ;[1 1 1] Prevents the camera from not douign waht i want
  ;;[0.1221 1 0] Inputs
  (Pawn|Input|AddMovementInput (Math|Vector|MakeVector 0.0 0.0 (* AxisValue -25.0)) 3.0 false))

(event Input|AxisEvents|InputAxisMoveForward
  (params (AxisValue :type Float%20%28single-precision%29))
  ;[1 1 1] Prevents the camera from not douign waht i want
  ;;[0.1221 1 0] Inputs
  (Pawn|Input|AddMovementInput (Math|Vector|MakeVector (* AxisValue 1e+03) 0.0 0.0) 5.0 false))

(fn ConstructionScript)

(fn OnRepCOREInitialRotationfromPlayer)