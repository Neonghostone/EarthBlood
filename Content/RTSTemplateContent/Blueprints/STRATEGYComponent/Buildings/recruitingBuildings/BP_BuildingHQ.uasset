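; BP_BuildingHQ is the headquarters recruiting building for the RTS template, with its behavior inherited from its parent class.
; It overrides the select-to-recruit and unselect-to-build events, calling the parent and then casting the controller and its HUD to the RTS classes.
; Nothing follows those casts, and the construction script only calls the parent, so the graphs add no HQ-specific logic.
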(event EventBeginPlay)

(event EventActorBeginOverlap
  (params (OtherActor :type Actor%20Object%20Reference)))

(event EventTick
  (params (DeltaSeconds :type Float%20%28single-precision%29)))

(event EventSTRATEGYBuildingGetUnselectedtoBuild
  (params (ControllerUnselecting :type Controller%20Object%20Reference))
  (|CallParentFunction ControllerUnselecting)
  (bind _asbp_player_controller_rtsmax_par (Utilities|Casting|CastToBP_PlayerControllerRTSMaxPar ControllerUnselecting))
  (Utilities|Casting|CastToBP_HUDMaxParentClass (HUD|GetHUD _asbp_player_controller_rtsmax_par)))

(event EventSTRATEGYBuildingGetSelectedtoRecruit
  (params (Controller :type Controller%20Object%20Reference))
  (|CallParentFunction Controller)
  (bind _asbp_player_controller_rtsmax_par (Utilities|Casting|CastToBP_PlayerControllerRTSMaxPar Controller))
  (Utilities|Casting|CastToBP_HUDMaxParentClass (HUD|GetHUD _asbp_player_controller_rtsmax_par)))

(fn ConstructionScript
  (|CallParentFunction))