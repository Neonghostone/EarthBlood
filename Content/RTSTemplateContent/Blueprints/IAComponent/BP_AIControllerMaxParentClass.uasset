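; AI controller base for RTS characters that aggro on nearby enemy-team characters, chase them and attack.
; An enum state machine runs on three looping timers for attention, movement and aggression.
; Attention picks the closest enemy and switches state within aggro range; movement then pathfinds to it while aggression fires the primary weapon through timed press, release and cooldown.
; Many state hooks are empty stubs, and transitions show debug text.
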(event EventBeginPlay
  (|CallParentFunction)
  ;[1 1 1] Start the timers
  (bind _returnvalue (Utilities|Time|SetTimerbyFunctionName 0 "Timer_MovementTick" (Variables|Default|GetAI_TimerTickLevel) true))
  (Variables|Default|SetHandle_MovementTickTimer _returnvalue)
  (bind _returnvalue_2 (Utilities|Time|SetTimerbyFunctionName 0 "Timer_AgressiveTick" (Variables|Default|GetAI_TimerTickLevel) true))
  (Variables|Default|SetHandle_AgressiveTickTimer _returnvalue_2)
  (bind _returnvalue_3 (Utilities|Time|SetTimerbyFunctionName 0 "Timer_AtentionTick" (Variables|Default|GetAI_TimerTickLevel) true))
  (Variables|Default|Sethandle_AtentionTickTimer _returnvalue_3)
  (bind _asbp_inv_character_max_parent (Utilities|Casting|CastToBP_InvCharacterMaxParent (Pawn|GetControlledPawn)))
  (Default|DEBUGCONTROLLERUpdateStateText _asbp_inv_character_max_parent))

(event EventTick
  (params (DeltaSeconds :type Float%20%28single-precision%29))
  (switch Utilities|FlowControl|Switch|SwitchonEN_AIState (Variables|Default|GetAI_ActualState)))

(fn ConstructionScript)

(fn GetEnemy
  ;[1 1 1] Nulled this funcion does nothing do much
)

(fn GotoStateEndStateBeginState
  (params (NewStateToEnter :type EN_AIState%20Enum) (PreviousStateToLeave :type EN_AIState%20Enum))
  (bind _output_get (Variables|Default|SetAI_ActualState NewStateToEnter))
  (bind _asbp_inv_character_max_parent (Utilities|Casting|CastToBP_InvCharacterMaxParent (Pawn|GetControlledPawn)))
  (Default|DEBUGCONTROLLERUpdateStateText _asbp_inv_character_max_parent)
  (Utilities|FlowControl|Sequence
    (:then_0
      ;[1 0 0.0669] ENDState stuff
      (switch Utilities|FlowControl|Switch|SwitchonEN_AIState _output_get
        (:NewEnumerator0
          (CallFunction|StateENDWaitingforAgro))))
    (:then_1
      ;[0.1208 1 0.1775] STARTState stuff
      (switch Utilities|FlowControl|Switch|SwitchonEN_AIState _output_get
        (:NewEnumerator1
          (CallFunction|StateBEGINGettingClosetoEnemy))))))

(fn TimerMovementTick
  ;[1 1 1] Ticked Each Empanació level
  (switch Utilities|FlowControl|Switch|SwitchonEN_AIState (Variables|Default|GetAI_ActualState)
    (:NewEnumerator1
      (CallFunction|StateLATNTGettingClosetoEnemyMovement))))

(fn TimerAgressiveTick
  (switch Utilities|FlowControl|Switch|SwitchonEN_AIState (Variables|Default|GetAI_ActualState)
    (:NewEnumerator1
      (CallFunction|PerformPrimaryWeaponAttack))))

(fn TimerAtentionTick
  (switch Utilities|FlowControl|Switch|SwitchonEN_AIState (Variables|Default|GetAI_ActualState)
    (:NewEnumerator0
      (bind _pawn (CallFunction|GetClosestEnemy))
      (if (!= _pawn 0)
        (bind _output_get (Variables|Default|SetAI_Oponent _pawn))
        (bind _bcloseenoughforagro (CallFunction|CloseEnoughforAgro _output_get))
        (if _bcloseenoughforagro
          (CallFunction|GotoStateEndStateBeginState "NewEnumerator1" (Variables|Default|GetAI_ActualState)))))))

(fn ChangeTimerTick
  (params (newTicKLevel :type Float%20%28single-precision%29)))

(fn CloseEnoughforAgro
  (params (oponenttocheck :type Actor%20Object%20Reference))
  (if (< (Math|Vector|VectorLength (- (Transformation|GetActorLocation oponenttocheck) (Transformation|GetActorLocation (Pawn|GetControlledPawn)))) (Math|Conversions|ToFloat(Integer) (Variables|Default|Getagrodistance)))
    (return true)
    (else
      (return false))))

(fn StateLATNTGettingClosetoEnemyMovement
  (AI|Navigation|MovetoLocation (Transformation|GetActorLocation (Variables|Default|GetAI_Oponent)) -1.0 true true true))

(fn StateLATNTGettingClosetoEnemyAgressive)

(fn StateLATNTGettingClosetoEnemyAtention)

(fn StateLATNTWaitingforAgroAtention)

(fn StateLATNTWaitingforAgroMovement)

(fn StateLATNTWaitingforAgroAgressive)

(fn StateBEGINGettingClosetoEnemy
  (bind _ascharacter (Utilities|Casting|CastToCharacter (Pawn|GetControlledPawn)))
  (Rendering|Debug|DrawDebugString (Transformation|GetActorLocation _ascharacter) "AGROOO!" 0 "(R=1.000000,G=0.000000,B=0.006608,A=1.000000)" 5.0))

(fn StateENDGettingClosetoEnemy)

(fn StateBEGINWaitingforAgro)

(fn StateENDWaitingforAgro
  (Rendering|Debug|DrawDebugString (Transformation|GetActorLocation (Pawn|GetControlledPawn)) "AGROO!!!!" 0 "(R=1.000000,G=0.000000,B=0.078098,A=1.000000)" 8.0))

(fn GetClosestEnemy
  (bind _returnvalue (Pawn|GetControlledPawn))
  (bind _outactors (Actor|GetAllActorsOfClass "/Game/RTSTemplateContent/Blueprints/COREComponentMelee/BP_InvCharacterMaxParent.BP_InvCharacterMaxParent_C"))
  (bind _array_element (Utilities|Array|ForEachLoopwithBreak _outactors)
    (:LoopBody
      ;[1 1 1] Make sure we dont become our own enemy
      (if (!= _array_element (Pawn|GetControlledPawn))
        ;[1 1 1] Make sure it's not of our team
        (bind _asbp_inv_character_max_parent (Utilities|Casting|CastToBP_InvCharacterMaxParent _returnvalue))
        (if (!= (Math|Conversions|ToByte(Integer) (Variables|/Game/RTSTemplateContent/Blueprints/COREComponentMelee/BP_InvCharacterMaxParent.BP_InvCharacterMaxParent_C|GetTeamNum _array_element)) (Math|Conversions|ToByte(Integer) (Variables|/Game/RTSTemplateContent/Blueprints/COREComponentMelee/BP_InvCharacterMaxParent.BP_InvCharacterMaxParent_C|GetTeamNum _asbp_inv_character_max_parent)))
          ;[1 1 1] SetWho closest pawn is
          (if (> (LocalVariables|GetClosestDistance) (Math|Vector|VectorLengthSquared (- (Transformation|GetActorLocation _returnvalue) (Transformation|GetActorLocation _array_element))))
            (LocalVariables|SetClosestDistance (Math|Vector|VectorLengthSquared (- (Transformation|GetActorLocation _returnvalue) (Transformation|GetActorLocation _array_element))))
            (LocalVariables|SetClosestPawn _array_element)))))
    (:Completed
      ;[1 1 1] Return the nearest enemy we can  find
      (return (LocalVariables|GetClosestPawn)))))

(fn PerformPrimaryWeaponAttack
  (if (not (Utilities|Time|IsTimerActivebyHandle (Variables|Default|GetHandle_PerformingAttackHandle)))
    (bind _returnvalue (Utilities|Time|SetTimerbyFunctionName 0 "PerformAttackTimeBasedCoolDown" 2.0))
    (Variables|Default|SetHandle_PerformingAttackHandle _returnvalue)
    (CallFunction|PerformLoadWeapon)
    (Utilities|Time|SetTimerbyFunctionName 0 "PerformReleaseWeapon" 1.0)))

(fn PerformAttackTimeBasedCoolDown)

(fn PerformLoadWeapon
  (bind _asbp_inv_character_max_parent (Utilities|Casting|CastToBP_InvCharacterMaxParent (Pawn|GetControlledPawn)))
  (if (!= (Variables|/Game/RTSTemplateContent/Blueprints/COREComponentMelee/BP_InvCharacterMaxParent.BP_InvCharacterMaxParent_C|GetPrimaryWeaponItem _asbp_inv_character_max_parent) 0)
    (Default|PawnStartFire _asbp_inv_character_max_parent)))

(fn PerformReleaseWeapon
  (bind _asbp_inv_character_max_parent (Utilities|Casting|CastToBP_InvCharacterMaxParent (Pawn|GetControlledPawn)))
  (if (!= (Variables|/Game/RTSTemplateContent/Blueprints/COREComponentMelee/BP_InvCharacterMaxParent.BP_InvCharacterMaxParent_C|GetPrimaryWeaponItem _asbp_inv_character_max_parent) 0)
    (Default|PawnStopFire _asbp_inv_character_max_parent)))