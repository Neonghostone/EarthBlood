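; Base inventory actor that holds a replicated, unlimited list of items for its owning character.
; On authority, AddItemInInventory stores the item, assigns it the inventory's owner and marks it picked.
; If a BP_InvCharacterMaxParent owner has no primary weapon, that item is equipped as primary.
; AddSavedItem spawns an item from its saved archetype class at the owner's transform, then adds it the same way.
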(event EventBeginPlay)

(event Collision|EventActorBeginOverlap
  (params (OtherActor :type Actor%20Object%20Reference)))

(event EventTick
  (params (DeltaSeconds :type Float%20%28single-precision%29)))

(fn ConstructionScript)

(fn OnRepinInventoryItems)

(fn AddIteminInventory
  (params (ItemToAdd :type BP%20Inv%20Item%20Max%20Item%20Object%20Reference))
  ;[1 1 1] #0 Make sure this only runs rom the ser ver sidde
  (Networking|SwitchHasAuthority
    (:Authority
      ;[1 1 1] #1 No necessary INV Limits So make infinitev,And assign owner
      (Utilities|Array|Add (Variables|Default|GetInInventoryItems) ItemToAdd)
      (Actor|SetOwner ItemToAdd (Components|GetOwner))
      (Variables|/Game/RTSTemplateContent/Blueprints/COREComponentMelee/Items/BP_InvItemMaxItem.BP_InvItemMaxItem_C|SetbPicked ItemToAdd true)
      ;[1 1 1] # 2 PrimaryWeapon assigning
      (bind _asbp_inv_character_max_parent (Utilities|Casting|CastToBP_InvCharacterMaxParent (Components|GetOwner)))
      (if (== (Variables|/Game/RTSTemplateContent/Blueprints/COREComponentMelee/BP_InvCharacterMaxParent.BP_InvCharacterMaxParent_C|GetPrimaryWeaponItem _asbp_inv_character_max_parent) 0)
        ;[1 1 1] # 3 Equip
        (bind _output_get (Variables|/Game/RTSTemplateContent/Blueprints/COREComponentMelee/BP_InvCharacterMaxParent.BP_InvCharacterMaxParent_C|SetPrimaryWeaponItem _asbp_inv_character_max_parent ItemToAdd))
        (Default|ItemEquip _output_get)
        (Variables|/Game/RTSTemplateContent/Blueprints/COREComponentMelee/Items/BP_InvItemMaxItem.BP_InvItemMaxItem_C|SetbSetToPrimaryWeapon ItemToAdd true)))))

(fn AddSavedItem
  (params (TheSavedItem :type ST%20Saved%20Item%20Structure))
  (bind _itemspawned (CallFunction|SpawnItemfromArchetype (.Archetype (Utilities|Struct|BreakST_SavedItem TheSavedItem))))
  (CallFunction|AddIteminInventory _itemspawned))

(fn SpawnItemfromArchetype
  (params (Archetype :type BP%20Inv%20Item%20Max%20Item%20Class%20Reference))
  (bind _returnvalue (Components|GetOwner))
  (bind _returnvalue_2 (Game|SpawnActorfromClass Archetype (Transformation|GetActorTransform _returnvalue) "Undefined" _returnvalue 0))
  (return _returnvalue_2))