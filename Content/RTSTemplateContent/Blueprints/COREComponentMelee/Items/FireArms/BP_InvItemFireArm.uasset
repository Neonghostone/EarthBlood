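; Firearm inventory item that fires projectiles and toggles ironsight aiming on its owning character.
; Primary fire spawns the projectile class at the weapon's FireSocket on authority only; other fire modes toggle aim.
; Aiming reparents the camera to the weapon, lerps it in weapon-local space on Tick, then attaches it to the eye or sight spring arm.
; Becoming primary weapon attaches the sight arm to WeaponAimSocket; fire effects are an empty stub.
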(event Custom|ClientOwnerAttachSpringArmAswell
  ;[0.1287 0.1558 1] EquipCallFunctions
  (Development|PrintString (Utilities|String|Append "FROM TSIItemFireArm Client side calling attach spring ar to and the owner is" (Utilities|GetDisplayName (Components|GetOwner))))
  (CallFunction|AttachSpringArmtoWeapSock))

(event EventStartFire
  (params (FireModeNum :type Byte))
  ;[0.6781 1 0.5488] Start stop fire
  (|CallParentFunction 0)
  (if (== FireModeNum 0)
    ;;[1 0.7599 0.283] Shooting functionality SHOOTS!
    (CallFunction|SpawnProjectileServer)
    (elif (Variables|Default|GetIsAimingWithIronsights)
      ;;[0.5355 0.57 0.523] Aiming functionality EYESIGHT
      (CallFunction|DetachCamandKeepPosition)
      ;;;[1 1 1] SetStartLerping From WEAPON to EYES
      (if (Variables|Default|GetCanChangeAimNow)
        (Variables|Default|SetIsLrpWeaponToEyes true)
        (Variables|Default|SetCanChangeAimNow false))
      (else
        ;;[0.5355 0.57 0.523] Aiming functionality IRONSIGHTS !
        (CallFunction|DetachCamandKeepPosition)
        ;;;[1 1 1] SetStartLerping From EYES to WEAPON
        (if (Variables|Default|GetCanChangeAimNow)
          (Variables|Default|SetIsLrpEyesToWeapon true)
          (Variables|Default|SetCanChangeAimNow false))))))

(event EventOnRepBSettoPrimaryWeapon
  ;[0.1287 0.1558 1] EquipCallFunctions
  (|CallParentFunction)
  (CallFunction|AttachSpringArmtoWeapSock))

(event EventItemEquip
  ;[0.1287 0.1558 1] EquipCallFunctions
  (|CallParentFunction))

(event EventBeginPlay)

(event Collision|EventActorBeginOverlap
  (params (OtherActor :type Actor%20Object%20Reference)))

(event EventTick
  (params (DeltaSeconds :type Float%20%28single-precision%29))
  (bind _castowner (CallFunction|GetCastPOwnerTSI))
  (bind _castowner_2 (CallFunction|GetCastPOwnerTSI))
  (bind _castowner_3 (CallFunction|GetCastPOwnerTSI))
  (bind _castowner_4 (CallFunction|GetCastPOwnerTSI))
  (bind _castowner_5 (CallFunction|GetCastPOwnerTSI))
  (bind _castowner_6 (CallFunction|GetCastPOwnerTSI))
  (bind _castowner_7 (CallFunction|GetCastPOwnerTSI))
  (bind _castowner_8 (CallFunction|GetCastPOwnerTSI))
  (bind _camera (Variables|/Game/RTSTemplateContent/Blueprints/COREComponentMelee/BP_InvCharacterMaxParent.BP_InvCharacterMaxParent_C|GetCamera _castowner_4))
  (bind _eyessightspring (Variables|/Game/RTSTemplateContent/Blueprints/COREComponentMelee/BP_InvCharacterMaxParent.BP_InvCharacterMaxParent_C|GetEyesSightSpring _castowner_6))
  (bind _camera_2 (Variables|/Game/RTSTemplateContent/Blueprints/COREComponentMelee/BP_InvCharacterMaxParent.BP_InvCharacterMaxParent_C|GetCamera _castowner_7))
  (bind _weaponsocketsightspring (Variables|/Game/RTSTemplateContent/Blueprints/COREComponentMelee/BP_InvCharacterMaxParent.BP_InvCharacterMaxParent_C|GetWeaponSocketSightSpring _castowner_5))
  (bind _rightarmweapon (Variables|/Game/RTSTemplateContent/Blueprints/COREComponentMelee/BP_InvCharacterMaxParent.BP_InvCharacterMaxParent_C|GetRightArmWeapon _castowner_8))
  (bind _rightarmweapon_2 (Variables|/Game/RTSTemplateContent/Blueprints/COREComponentMelee/BP_InvCharacterMaxParent.BP_InvCharacterMaxParent_C|GetRightArmWeapon _castowner_2))
  (bind _rightarmweapon_3 (Variables|/Game/RTSTemplateContent/Blueprints/COREComponentMelee/BP_InvCharacterMaxParent.BP_InvCharacterMaxParent_C|GetRightArmWeapon _castowner_3))
  (bind _rightarmweapon_4 (Variables|/Game/RTSTemplateContent/Blueprints/COREComponentMelee/BP_InvCharacterMaxParent.BP_InvCharacterMaxParent_C|GetRightArmWeapon _castowner))
  (bind _returnvalue (Transformation|GetSocketLocation _weaponsocketsightspring "EndSpringPoint"))
  (bind _returnvalue_2 (Transformation|GetWorldLocation _camera_2))
  (bind _returnvalue_3 (Transformation|GetWorldTransform _rightarmweapon_2))
  (bind _returnvalue_4 (Transformation|GetWorldTransform _rightarmweapon_3))
  (bind _returnvalue_5 (Transformation|GetSocketLocation _eyessightspring "SpringEndpoint"))
  (bind _returnvalue_6 (Transformation|GetWorldLocation _camera))
  (bind _returnvalue_7 (Transformation|GetWorldTransform _rightarmweapon_4))
  (bind _returnvalue_8 (Transformation|GetWorldTransform _rightarmweapon))
  (bind _returnvalue_9 (Math|Transform|InverseTransformLocation _returnvalue_7 _returnvalue_2))
  (bind _returnvalue_10 (Math|Transform|InverseTransformLocation _returnvalue_3 _returnvalue))
  (bind _returnvalue_11 (Math|Transform|InverseTransformLocation _returnvalue_8 _returnvalue_6))
  (bind _returnvalue_12 (Math|Transform|InverseTransformLocation _returnvalue_4 _returnvalue_5))
  (Utilities|FlowControl|Sequence
    (:then_0
      ;[1 1 1] Lerp the from Aimsocket to eye
      ;;[1 1 1] 0 Check if shall lerp to the EYES now
      (if (Variables|Default|GetIsLrpWeaponToEyes)
        ;;[1 1 1] 3  Set camera Socket Locatio
        (Transformation|SetRelativeLocation (Variables|/Game/RTSTemplateContent/Blueprints/COREComponentMelee/BP_InvCharacterMaxParent.BP_InvCharacterMaxParent_C|GetCamera (CallFunction|GetCastPOwnerTSI)) (Math|Vector|Lerp(Vector) _returnvalue_11 _returnvalue_12 0.25) false false)
        (if (< (Math|Vector|VectorLengthSquared (- _returnvalue_12 _returnvalue_11)) 0.1)
          ;;[1 1 1] 4 Set current state variables
          (if (Variables|Default|GetIsLrpWeaponToEyes)
            (Variables|Default|SetCanChangeAimNow true)
            (Variables|Default|SetIsAimingWithIronsights false)
            ;;[1 1 1] 5 Finally attach the camera
            (Class|SceneComponent|Attachto (Variables|/Game/RTSTemplateContent/Blueprints/COREComponentMelee/BP_InvCharacterMaxParent.BP_InvCharacterMaxParent_C|GetCamera (CallFunction|GetCastPOwnerTSI)) (Variables|/Game/RTSTemplateContent/Blueprints/COREComponentMelee/BP_InvCharacterMaxParent.BP_InvCharacterMaxParent_C|GetEyesSightSpring (CallFunction|GetCastPOwnerTSI)) "SpringEndpoint" "KeepWorldPosition" true)
            (Variables|Default|SetIsLrpWeaponToEyes false)))))
    (:then_1
      ;[1 1 1] Lerp the From Eye to Aimsocket transition
      ;;[1 1 1] 0 check if shall Lerp To the WEAPON now
      (if (Variables|Default|GetIsLrpEyesToWeapon)
        ;;[1 1 1] 3 SetCameraNewLocationFromLerped location
        (Transformation|SetRelativeLocation (Variables|/Game/RTSTemplateContent/Blueprints/COREComponentMelee/BP_InvCharacterMaxParent.BP_InvCharacterMaxParent_C|GetCamera (CallFunction|GetCastPOwnerTSI)) (Math|Vector|Lerp(Vector) _returnvalue_9 _returnvalue_10 0.25) false false) ; SetThenewLocationrelativeTo
        ;;[1 1 1] 4 Set current state variables
        (if (< (Math|Vector|VectorLengthSquared (- _returnvalue_10 _returnvalue_9)) 0.1)
          (Variables|Default|SetCanChangeAimNow true)
          (Variables|Default|SetIsAimingWithIronsights true)
          ;;[1 1 1] 5 Finally attach the camera to the socket spring, and also set in wich aiming STATE is this weapon
          (Class|SceneComponent|Attachto (Variables|/Game/RTSTemplateContent/Blueprints/COREComponentMelee/BP_InvCharacterMaxParent.BP_InvCharacterMaxParent_C|GetCamera (CallFunction|GetCastPOwnerTSI)) (Variables|/Game/RTSTemplateContent/Blueprints/COREComponentMelee/BP_InvCharacterMaxParent.BP_InvCharacterMaxParent_C|GetWeaponSocketSightSpring (CallFunction|GetCastPOwnerTSI)) "SpringEndpoint" "KeepWorldPosition" true)
          (Variables|Default|SetIsLrpEyesToWeapon false))))))

(fn ConstructionScript
  (|CallParentFunction))

(fn SpawnProjectileServer
  (bind _castowner (CallFunction|GetCastPOwnerTSI))
  (bind _rightarmweapon (Variables|/Game/RTSTemplateContent/Blueprints/COREComponentMelee/BP_InvCharacterMaxParent.BP_InvCharacterMaxParent_C|GetRightArmWeapon _castowner))
  (bind _returnvalue (Transformation|GetSocketTransform _rightarmweapon "FireSocket" "RTS_World"))
  (bind (_location _rotation) (Math|Transform|BreakTransform _returnvalue))
  (Networking|SwitchHasAuthority
    (:Authority
      (Development|PrintString (Utilities|String|Append "FROM TSIItem SpawnProjectile Getting socketloc" (Utilities|GetDisplayName _rightarmweapon)))
      (Game|SpawnActorfromClass (Variables|Default|GetProjectileClass) (Math|Transform|MakeTransform _location _rotation (Transformation|GetActorScale3D self)) "AdjustIfPossibleButDontSpawnIfColliding" 0 0))))

(fn AttachSpringArmtoWeapSock
  (bind _castowner (CallFunction|GetCastPOwnerTSI))
  (Class|SceneComponent|Attachto (Variables|/Game/RTSTemplateContent/Blueprints/COREComponentMelee/BP_InvCharacterMaxParent.BP_InvCharacterMaxParent_C|GetWeaponSocketSightSpring _castowner) (Variables|/Game/RTSTemplateContent/Blueprints/COREComponentMelee/BP_InvCharacterMaxParent.BP_InvCharacterMaxParent_C|GetRightArmWeapon _castowner) "WeaponAimSocket" "KeepRelativeOffset" true)
  (Development|PrintText (Utilities|Text|ToText(String) (Utilities|String|Append "FROM TSIItemFireArm AttachSpringArmToPosition, trying to  the owner is" (Utilities|GetDisplayName (CallFunction|GetCastPOwnerTSI)))) true true "(R=1.000000,G=0.000000,B=0.471066,A=1.000000)"))

(fn DetachCamandKeepPosition
  (bind _castowner (CallFunction|GetCastPOwnerTSI))
  (bind _camera (Variables|/Game/RTSTemplateContent/Blueprints/COREComponentMelee/BP_InvCharacterMaxParent.BP_InvCharacterMaxParent_C|GetCamera _castowner))
  (Class|SceneComponent|DetachfromParent _camera true true)
  (Class|SceneComponent|Attachto _camera (Variables|/Game/RTSTemplateContent/Blueprints/COREComponentMelee/BP_InvCharacterMaxParent.BP_InvCharacterMaxParent_C|GetRightArmWeapon (CallFunction|GetCastPOwnerTSI)) "None" "KeepWorldPosition" true))

(fn PlayFireEffectsandSounds)