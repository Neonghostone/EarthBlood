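; BP_InvItemMaxItem is an inventory item that pawns pick up and equip.
; Pickup adds it to the pawn's inventory and sets Picked, whose OnRep hides the static mesh and disables collision.
; Equipping passes its skeletal mesh to the owning BP_InvCharacterMaxParent, while unequip is an empty stub.
; Fire functions maintain left/right mouse-hold flags for CORE control queries, though StopFire switches on constant 0, clearing only left.
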(event EventBeginPlay)

(event Collision|EventActorBeginOverlap
  (params (OtherActor :type Actor%20Object%20Reference)))

(event EventTick
  (params (DeltaSeconds :type Float%20%28single-precision%29)))

(fn ConstructionScript)

(fn StartFire
  (params (FireModeNum :type Byte))
  (switch int (Math|Conversions|ToInteger(Byte) FireModeNum)
    (:0
      (Variables|Default|SetbLeftMousePressedHold true))
    (:1
      (Variables|Default|SetbRightMousePressedHold true))))

(fn StopFire
  (params (FireModeNum :type Byte))
  (switch int 0
    (:0
      (Variables|Default|SetbLeftMousePressedHold false))
    (:1
      (Variables|Default|SetbRightMousePressedHold false))))

(fn ItemGetPicked
  (params (PawnPicking :type BP%20Inv%20Character%20Max%20Parent%20Object%20Reference))
  (Default|AddIteminInventory (Variables|/Game/RTSTemplateContent/Blueprints/COREComponentMelee/BP_InvCharacterMaxParent.BP_InvCharacterMaxParent_C|GetInventoryReference PawnPicking) self)
  (Variables|ItemProps|SetbPicked true))

(fn ItemEquip
  ;[1 1 1] For equipping this make it so the actual skel mesh changes, also check through a log if function is reached
  (bind _asbp_inv_character_max_parent (Utilities|Casting|CastToBP_InvCharacterMaxParent (Components|GetOwner)))
  (Variables|/Game/RTSTemplateContent/Blueprints/COREComponentMelee/BP_InvCharacterMaxParent.BP_InvCharacterMaxParent_C|SetRepAclSkeletalMAttachRA _asbp_inv_character_max_parent (Variables|ItemProps|GetSkeletalMeshForEquiping)))

(fn ItemUnEquip)

(fn OnRepBPicked
  (if (Math|Boolean|Equal(Boolean) (Variables|ItemProps|GetbPicked) true)
    (Rendering|SetVisibility (Variables|Default|GetItemStaMesh) false false)
    (Collision|SetActorEnableCollision false)
    (else
      (Rendering|SetVisibility (Variables|Default|GetItemStaMesh) true false)
      (Collision|SetActorEnableCollision true))))

(fn GetCastPOwnerTSI
  (bind _asbp_inv_character_max_parent (Utilities|Casting|CastToBP_InvCharacterMaxParent (Components|GetOwner)))
  (return _asbp_inv_character_max_parent))

(fn OnRepBSettoPrimaryWeapon)

(fn COREControlsBRightMousePressed?
  (return (Variables|Default|GetbRightMousePressedHold)))

(fn COREControlsBLeftMousePressed?
  (return (Variables|Default|GetbLeftMousePressedHold)))