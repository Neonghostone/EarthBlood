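; Melee weapon item with a charged attack: fire press plays a wind-up, and release unleashes the swing once a minimum load time has passed.
; Timer handles act as state flags for loading, unleashing and tracing.
; While tracing, Tick sweeps debug-drawn line traces between previous and current positions of four blade sockets.
; Skeletal-mesh hits damage other characters once per swing, without authority checks; hit records reset afterwards.
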(event EventStartFire
  (params (FireModeNum :type Byte))
  ;[1 1 1] CORE_CONTROLS_RightClick_LeftClick
  (|CallParentFunction FireModeNum)
  (switch int (Math|Conversions|ToInteger(Byte) FireModeNum)
    (:0
      ;;[1 1 1] SAFETY: Make Sure it's not Loading attack if unleashing or loading attack already
      (if (not (CallFunction|COREBoolIsLoadingAttack))
        (if (not (CallFunction|COREBoolIsUnleashingAttack))
          (CallFunction|CORELoadAttack))))))

(event EventStopFire
  (params (FireModeNum :type Byte))
  ;[1 1 1] CORE_CONTROLS_RightClick_LeftClick
  (|CallParentFunction FireModeNum)
  (switch int (Math|Conversions|ToInteger(Byte) FireModeNum)
    (:0
      ;;[1 1 1] SAFETY: Not Unleash if not loading and unleashing already
      (if (CallFunction|COREBoolMinLoadTimeHasPassed)
        (if (CallFunction|COREBoolIsLoadingAttack)
          (if (not (CallFunction|COREBoolIsUnleashingAttack))
            (CallFunction|COREUnleashAttack)))))))

(event EventBeginPlay)

(event Collision|EventActorBeginOverlap
  (params (OtherActor :type Actor%20Object%20Reference)))

(event EventTick
  (params (DeltaSeconds :type Float%20%28single-precision%29))
  ;[1 1 1] Tick
  (if (Utilities|Time|IsTimerActivebyHandle (Variables|Default|GetCORE_TracingHandle))
    (CallFunction|CORECollisionTraceFunctBladeType)))

(fn ConstructionScript
  (|CallParentFunction))

(fn CORETimeBasedIsTimeActiveShallPerformMeleeTrace)

(fn CORECollisionTraceFunctBladeType
  (bind _returnvalue (Components|GetOwner))
  (if (Math|Vector|Equal(Vector) (Variables|Default|GetLastTraceLoc0) "0, 0, 0" 0.0001)
    (Utilities|FlowControl|Sequence
      (:then_0
        ;[1 1 1] Assign a primary location to all lastTraceLocs
        (bind _asbp_inv_character_max_parent (Utilities|Casting|CastToBP_InvCharacterMaxParent _returnvalue))
        (Variables|Default|SetLastTraceLoc0 (Transformation|GetSocketLocation (Variables|/Game/RTSTemplateContent/Blueprints/COREComponentMelee/BP_InvCharacterMaxParent.BP_InvCharacterMaxParent_C|GetRightArmWeapon _asbp_inv_character_max_parent) "TraceSocket0")))
      (:then_1
        (bind _asbp_inv_character_max_parent_2 (Utilities|Casting|CastToBP_InvCharacterMaxParent _returnvalue))
        (Variables|Default|SetLastTraceLoc1 (Transformation|GetSocketLocation (Variables|/Game/RTSTemplateContent/Blueprints/COREComponentMelee/BP_InvCharacterMaxParent.BP_InvCharacterMaxParent_C|GetRightArmWeapon _asbp_inv_character_max_parent_2) "TraceSocket1")))
      (:then_2
        (bind _asbp_inv_character_max_parent_3 (Utilities|Casting|CastToBP_InvCharacterMaxParent _returnvalue))
        (Variables|Default|SetLastTraceLoc2 (Transformation|GetSocketLocation (Variables|/Game/RTSTemplateContent/Blueprints/COREComponentMelee/BP_InvCharacterMaxParent.BP_InvCharacterMaxParent_C|GetRightArmWeapon _asbp_inv_character_max_parent_3) "TraceSocket2")))
      (:then_3
        (bind _asbp_inv_character_max_parent_4 (Utilities|Casting|CastToBP_InvCharacterMaxParent _returnvalue))
        (Variables|Default|SetLastTraceLoc3 (Transformation|GetSocketLocation (Variables|/Game/RTSTemplateContent/Blueprints/COREComponentMelee/BP_InvCharacterMaxParent.BP_InvCharacterMaxParent_C|GetRightArmWeapon _asbp_inv_character_max_parent_4) "TraceSocket3"))
        (Utilities|FlowControl|Sequence :!label _label
          (:then_0
            (bind _asbp_inv_character_max_parent_5 (Utilities|Casting|CastToBP_InvCharacterMaxParent _returnvalue))
            (Rendering|Debug|DrawDebugLine (Variables|Default|GetLastTraceLoc0) (Transformation|GetSocketLocation (Variables|/Game/RTSTemplateContent/Blueprints/COREComponentMelee/BP_InvCharacterMaxParent.BP_InvCharacterMaxParent_C|GetRightArmWeapon _asbp_inv_character_max_parent_5) "TraceSocket0") (Math|Color|MakeColor 255.0 0.0 0.0) 2.0 1.2)
            ;[1 1 1] Shall perform MP trace from Server only ? for now just client side
            (CallFunction|CORECollisionMultiLineTraceStartEnd (Variables|Default|GetLastTraceLoc0) (Transformation|GetSocketLocation (Variables|/Game/RTSTemplateContent/Blueprints/COREComponentMelee/BP_InvCharacterMaxParent.BP_InvCharacterMaxParent_C|GetRightArmWeapon _asbp_inv_character_max_parent_5) "TraceSocket0"))
            (Variables|Default|SetLastTraceLoc0 (Transformation|GetSocketLocation (Variables|/Game/RTSTemplateContent/Blueprints/COREComponentMelee/BP_InvCharacterMaxParent.BP_InvCharacterMaxParent_C|GetRightArmWeapon _asbp_inv_character_max_parent_5) "TraceSocket0")))
          (:then_1
            (bind _asbp_inv_character_max_parent_6 (Utilities|Casting|CastToBP_InvCharacterMaxParent _returnvalue))
            (Rendering|Debug|DrawDebugLine (Variables|Default|GetLastTraceLoc1) (Transformation|GetSocketLocation (Variables|/Game/RTSTemplateContent/Blueprints/COREComponentMelee/BP_InvCharacterMaxParent.BP_InvCharacterMaxParent_C|GetRightArmWeapon _asbp_inv_character_max_parent_6) "TraceSocket1") (Math|Color|MakeColor 255.0 0.0 0.0) 2.0 1.2)
            (CallFunction|CORECollisionMultiLineTraceStartEnd (Variables|Default|GetLastTraceLoc1) (Transformation|GetSocketLocation (Variables|/Game/RTSTemplateContent/Blueprints/COREComponentMelee/BP_InvCharacterMaxParent.BP_InvCharacterMaxParent_C|GetRightArmWeapon _asbp_inv_character_max_parent_6) "TraceSocket1"))
            (Variables|Default|SetLastTraceLoc1 (Transformation|GetSocketLocation (Variables|/Game/RTSTemplateContent/Blueprints/COREComponentMelee/BP_InvCharacterMaxParent.BP_InvCharacterMaxParent_C|GetRightArmWeapon _asbp_inv_character_max_parent_6) "TraceSocket1")))
          (:then_2
            (bind _asbp_inv_character_max_parent_7 (Utilities|Casting|CastToBP_InvCharacterMaxParent _returnvalue))
            (Rendering|Debug|DrawDebugLine (Variables|Default|GetLastTraceLoc2) (Transformation|GetSocketLocation (Variables|/Game/RTSTemplateContent/Blueprints/COREComponentMelee/BP_InvCharacterMaxParent.BP_InvCharacterMaxParent_C|GetRightArmWeapon _asbp_inv_character_max_parent_7) "TraceSocket2") (Math|Color|MakeColor 255.0 0.0 0.0) 2.0 1.2)
            (CallFunction|CORECollisionMultiLineTraceStartEnd (Variables|Default|GetLastTraceLoc2) (Transformation|GetSocketLocation (Variables|/Game/RTSTemplateContent/Blueprints/COREComponentMelee/BP_InvCharacterMaxParent.BP_InvCharacterMaxParent_C|GetRightArmWeapon _asbp_inv_character_max_parent_7) "TraceSocket2"))
            (Variables|Default|SetLastTraceLoc2 (Transformation|GetSocketLocation (Variables|/Game/RTSTemplateContent/Blueprints/COREComponentMelee/BP_InvCharacterMaxParent.BP_InvCharacterMaxParent_C|GetRightArmWeapon _asbp_inv_character_max_parent_7) "TraceSocket2")))
          (:then_3
            (bind _asbp_inv_character_max_parent_8 (Utilities|Casting|CastToBP_InvCharacterMaxParent _returnvalue))
            (Rendering|Debug|DrawDebugLine (Variables|Default|GetLastTraceLoc3) (Transformation|GetSocketLocation (Variables|/Game/RTSTemplateContent/Blueprints/COREComponentMelee/BP_InvCharacterMaxParent.BP_InvCharacterMaxParent_C|GetRightArmWeapon _asbp_inv_character_max_parent_8) "TraceSocket3") (Math|Color|MakeColor 255.0 0.0 0.0) 2.0 1.2)
            (CallFunction|CORECollisionMultiLineTraceStartEnd (Variables|Default|GetLastTraceLoc3) (Transformation|GetSocketLocation (Variables|/Game/RTSTemplateContent/Blueprints/COREComponentMelee/BP_InvCharacterMaxParent.BP_InvCharacterMaxParent_C|GetRightArmWeapon _asbp_inv_character_max_parent_8) "TraceSocket3"))
            (Variables|Default|SetLastTraceLoc3 (Transformation|GetSocketLocation (Variables|/Game/RTSTemplateContent/Blueprints/COREComponentMelee/BP_InvCharacterMaxParent.BP_InvCharacterMaxParent_C|GetRightArmWeapon _asbp_inv_character_max_parent_8) "TraceSocket3"))))))
    (else
      (goto _label))))

(fn CORETimeBasedIsTimeActiveShallPerformMinLoadAttack
  ;[1 1 1] SAFET Make sure that we are loading the attack that we have LeftMousePressed still and tha twe are not unleashing the attack to attack again
  (if (CallFunction|COREBoolIsLoadingAttack)
    (if (not (CallFunction|COREControlsBLeftMousePressed?))
      (if (not (CallFunction|COREBoolIsUnleashingAttack))
        (CallFunction|COREUnleashAttack)))))

(fn CORETimeBasedIsTimeActiveUnleashingAttack
  (CallFunction|CORECollisionCleanHitActorsCleanLastLocs))

(fn CORELoadAttack
  ;[1 1 1] SAFETY: Make Sure it's not Loading attack if unleashing or loading attack already
  (if (not (CallFunction|COREBoolIsLoadingAttack))
    (if (not (CallFunction|COREBoolIsUnleashingAttack))
      (bind _returnvalue (Utilities|Time|SetTimerbyFunctionName 0 "CORE_TimeBasedIsTimeActiveLoadAttack" 1e+03))
      (Variables|Default|SetCORE_LoadintgAttackHandleInfinite _returnvalue)
      (bind _returnvalue_2 (Utilities|Time|SetTimerbyFunctionName 0 "CORE_TimeBasedIsTimeActiveShallPerformMinLoadAttack" 0.55))
      (Variables|Default|SetCORE_LoadingMintimeHandle _returnvalue_2)
      (bind _asbp_inv_character_max_parent (Utilities|Casting|CastToBP_InvCharacterMaxParent (Components|GetOwner)))
      (bind _asbp_inv_character_max_parent_2 (Utilities|Casting|CastToBP_InvCharacterMaxParent (Components|GetOwner)))
      (Default|StartPlayingAnimation _asbp_inv_character_max_parent (Variables|/Game/RTSTemplateContent/Blueprints/COREComponentMelee/BP_InvCharacterMaxParent.BP_InvCharacterMaxParent_C|GetPrepareOneHandedAttackUniPH _asbp_inv_character_max_parent_2)))))

(fn COREUnleashAttack
  ;[1 1 1] SAFETY: Do Not Unleash attack if we are not Loading the attack   Do not either if we are unleashing añlready an attack
  (if (CallFunction|COREBoolIsLoadingAttack)
    (if (not (CallFunction|COREBoolIsUnleashingAttack))
      (bind _asbp_inv_character_max_parent (Utilities|Casting|CastToBP_InvCharacterMaxParent (Components|GetOwner)))
      (Class|KismetSystemLibrary|ClearTimerHandle (Variables|Default|GetCORE_LoadintgAttackHandleInfinite))
      (Class|KismetSystemLibrary|ClearTimerHandle (Variables|Default|GetCORE_LoadingMintimeHandle))
      (bind _asbp_inv_character_max_parent_2 (Utilities|Casting|CastToBP_InvCharacterMaxParent (Components|GetOwner)))
      (Default|StartPlayingAnimation _asbp_inv_character_max_parent (Variables|/Game/RTSTemplateContent/Blueprints/COREComponentMelee/BP_InvCharacterMaxParent.BP_InvCharacterMaxParent_C|GetOneHandedAttackUniPH_0 _asbp_inv_character_max_parent_2))
      (bind _returnvalue (Utilities|Time|SetTimerbyFunctionName 0 "CORE_TimeBasedIsTimeActiveUnleashingAttack" 1.5))
      (Variables|Default|SetCORE_UnleashingAttackHandle _returnvalue)
      (bind _returnvalue_2 (Utilities|Time|SetTimerbyFunctionName 0 "CORE_TimeBasedIsTimeActiveShallPerformMeleeTrace" 0.75))
      (Variables|Default|SetCORE_TracingHandle _returnvalue_2))))

(fn COREBoolIsLoadingAttack
  (if (Utilities|Time|IsTimerActivebyHandle (Variables|Default|GetCORE_LoadintgAttackHandleInfinite))
    (return true)
    (else
      (return false))))

(fn COREBoolMinLoadTimeHasPassed
  (if (Utilities|Time|IsTimerActivebyHandle (Variables|Default|GetCORE_LoadingMintimeHandle))
    (return false)
    (else
      (return true))))

(fn CORETimeBasedIsTimeActiveLoadAttack)

(fn COREBoolIsUnleashingAttack
  (return (Utilities|Time|IsTimerActivebyHandle (Variables|Default|GetCORE_UnleashingAttackHandle))))

(fn CORECollisionCleanHitActorsCleanLastLocs
  (Variables|Default|SetLastTraceLoc1 "0, 0, 0")
  (Variables|Default|SetLastTraceLoc2 "0, 0, 0")
  (Variables|Default|SetLastTraceLoc3 "0, 0, 0")
  (Variables|Default|SetLastTraceLoc0 "0, 0, 0")
  (Utilities|Array|Clear (Variables|Default|GetHitArrayOfActors)))

(fn CORECollisionMultiLineTraceStartEnd
  (params (Start :type Vector) (End :type Vector))
  (bind _outhits (Class|KismetSystemLibrary|LineTraceMultiforObjects Start End (Utilities|Array|MakeArray "ObjectTypeQuery1" "ObjectTypeQuery2" "ObjectTypeQuery3") false 0 "None" true))
  (for _array_element _outhits
    (CallFunction|COREDamageProcessHit _array_element)))

(fn COREDamageProcessPawnHitReaction
  (params (HitReactionStruct :type Hit%20Result%20Structure))
  (bind (_bblockinghit _binitialoverlap _time _location _impactpoint _normal _impactnormal _physmat _hitactor) (Collision|BreakHitResult HitReactionStruct))
  (if (!= _hitactor (Components|GetOwner))
    (Rendering|Debug|DrawDebugString _location "Hit!" 0 "(R=1.000000,G=1.000000,B=1.000000,A=1.000000)" 4.0)
    (bind _yesheis (CallFunction|CORECollisionIsHitActorinArray _hitactor))
    (if (not _yesheis)
      (CallFunction|CORECollisionAddHitActorinArray _hitactor)
      (Rendering|Debug|DrawDebugString _location "The Damage Hit Is" 0 "(R=0.545000,G=0.067502,B=0.000000,A=1.000000)" 3.0)
      (bind _asbp_inv_character_max_parent (Utilities|Casting|CastToBP_InvCharacterMaxParent _hitactor))
      (Default|CORETakeDamage _asbp_inv_character_max_parent 25))))

(fn COREDamageProcessHit
  (params (HitReactionStruct :type Hit%20Result%20Structure))
  (Utilities|Casting|CastToSkeletalMeshComponent (.HitComponent (Collision|BreakHitResult HitReactionStruct)))
  (CallFunction|COREDamageProcessPawnHitReaction HitReactionStruct))

(fn CORECollisionIsHitActorinArray
  (params (Actor :type Actor%20Object%20Reference))
  (if (< (Utilities|Array|FindItem (Variables|Default|GetHitArrayOfActors) Actor) 0)
    (return false) ; Since is -1 for sure is not there
    (else
      (return true) ; Since is  not -1 somewherte it is
    )))

(fn CORECollisionAddHitActorinArray
  (params (NewhitActor :type Actor%20Object%20Reference))
  (Utilities|Array|Add (Variables|Default|GetHitArrayOfActors) NewhitActor))