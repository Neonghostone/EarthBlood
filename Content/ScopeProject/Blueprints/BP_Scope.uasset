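; BP_Scope is a scope that displays a live scene capture on its lens layer.
; CreateRenderTarget activates ScopeCapture, gives it a new 512-square render target, and feeds that into Layer1's dynamic material, creating the instance from MI_BaseLayer if needed.
; BeginPlay and the construction script are empty, and the only call to CreateRenderTarget in this Blueprint is unwired, so setup does not run on its own.
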(event EventBeginPlay)

(fn ConstructionScript)

(fn CreateRenderTarget
  ;[1 1 1] Decativate this to later make sure
  (Development|PrintString "FROM scope getitng activated")
  (Components|Activation|Activate (Variables|Default|GetScope%20Capture) false)
  (bind _returnvalue (Rendering|CreateRenderTarget2D 512 512 "RTF_RGBA16f"))
  (Variables|/Script/Engine.SceneCaptureComponent2D|SetTextureTarget (Variables|Default|GetScope%20Capture) _returnvalue)
  (Utilities|IsValid (Variables|Default|GetDynamicMaterial)
    (:Is%20Valid
      (Rendering|Material|SetTextureParameterValue (Variables|Default|GetDynamicMaterial) "Texture" (Variables|/Script/Engine.SceneCaptureComponent2D|GetTextureTarget (Variables|Default|GetScope%20Capture))))
    (:Is%20Not%20Valid
      (bind _returnvalue_2 (Rendering|Material|CreateDynamicMaterialInstance (Variables|Default|GetLayer%201) 0 "/Game/ScopeProject/Materials/Scope/Instance/MI_BaseLayer.MI_BaseLayer" "None" :!class /Script/Engine.PrimitiveComponent))
      (Variables|Default|SetDynamicMaterial _returnvalue_2)
      (Rendering|Material|SetMaterial (Variables|Default|GetLayer%201) 0 (Variables|Default|GetDynamicMaterial))
      (Rendering|Material|SetTextureParameterValue (Variables|Default|GetDynamicMaterial) "Texture" (Variables|/Script/Engine.SceneCaptureComponent2D|GetTextureTarget (Variables|Default|GetScope%20Capture)))
      (return))))