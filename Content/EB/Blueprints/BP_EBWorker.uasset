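; BP_EBWorker is an RTS worker unit that players select and order to move, run, work at or sabotage buildings.
; Selection runs on authority, checks ownership through the player controller, then updates its selected list and the selection circle.
; Orders pass to the AI controller as desired locations, mostly with state changes and target buildings.
; Right-clicking a building targets its working-station arrow; hologram construction is an empty WIP stub.
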(event EventBeginPlay
  (|CallParentFunction))

(event Collision|EventActorBeginOverlap
  (params (OtherActor :type Actor%20Object%20Reference)))

(event EventTick
  (params (DeltaSeconds :type Float%20%28single-precision%29))
  (|CallParentFunction DeltaSeconds))

(event EventRTSMouseInterfunctonMouseLeftClick
  (params (ControllerThat0LeftClicked :type Player%20Controller%20Object%20Reference))
  (CallFunction|RTSInterfunctUnitGetSelected ControllerThat0LeftClicked))

(event EventRTSInterfunctHandleRightClickonLSorSMwithSelected
  (params (PlayerControllerUsing :type Player%20Controller%20Object%20Reference) (PlaceOnMap :type Vector :default "0, 0, 0"))
  (bind _returnvalue (Pawn|GetController))
  (Development|PrintString "FROM Worker got landsacape sleected and this is selceted delte print" true true "(R=0.038633,G=1.000000,B=0.000000,A=1.000000)" 1e+01)
  ;[1 1 1] Handle right click on landscape
  (if (Utilities|IsValid _returnvalue)
    (bind _asbp_ebaicontroller_max_parent_class (Utilities|Casting|CastToBP_EBAIControllerMaxParentClass _returnvalue))
    (Development|PrintString "FROM EBWorker going landscape ?  ")
    ;[1 1 1] Here error maybe
    (Default|GotoStateAIWokerorWhataver _asbp_ebaicontroller_max_parent_class "NewEnumerator0" (Variables|/Game/EB/Blueprints/BP_EBAIControllerMaxParentClass.BP_EBAIControllerMaxParentClass_C|GetAI_StateOfWorkerOrWhataver _asbp_ebaicontroller_max_parent_class))
    (bind _asbp_player_controller_rtsmax_par (Utilities|Casting|CastToBP_PlayerControllerRTSMaxPar PlayerControllerUsing))
    ;[1 1 1] Set desired location on setting to work on a building
    (bind _asbp_building_max_parent_class (Utilities|Casting|CastToBP_BuildingMaxParentClass (Variables|/Game/EB/Blueprints/BP_PlayerControllerRTSMaxPar.BP_PlayerControllerRTSMaxPar_C|GetLastRightClickActor _asbp_player_controller_rtsmax_par)))
    (Default|SetDesiredLocation _asbp_ebaicontroller_max_parent_class (Transformation|GetWorldLocation (Variables|/Game/EB/Blueprints/BP_BuildingMaxParentClass.BP_BuildingMaxParentClass_C|GetArrowComponentWorkingStationOne _asbp_building_max_parent_class)))))

(event EventRTSInterfunctUnitGetSelected
  (params (ControllerClicking :type Player%20Controller%20Object%20Reference))
  (bind _self self)
  ;[1 1 1] Get selected, in HERE THE IS ONE OF THE WORKERS DOES NOT WORK
  (Networking|SwitchHasAuthority
    (:Authority
      (bind _asbp_player_controller_rtsmax_par (Utilities|Casting|CastToBP_PlayerControllerRTSMaxPar ControllerClicking))
      (bind _isactoroneofitsactors (Default|STRATEGYIsThisActorOneOfItsActors _asbp_player_controller_rtsmax_par self))
      (if _isactoroneofitsactors
        (Utilities|Array|Add (Variables|/Game/EB/Blueprints/BP_PlayerControllerRTSMaxPar.BP_PlayerControllerRTSMaxPar_C|GetAllActorsSelected _asbp_player_controller_rtsmax_par) _self)
        (Default|HandleUnitGetSelectedDoHUdStuff _asbp_player_controller_rtsmax_par _self)
        (CallFunction|ClientSetSelectCircleVisible true)))))

(event EventRTSSendUnittoWork
  (params (BuildingToWorkAt :type BP%20Building%20Max%20Parent%20Class%20Object%20Reference))
  ;[1 1 1] USe for working already
  (bind _asbp_ebaicontroller_max_parent_class (Utilities|Casting|CastToBP_EBAIControllerMaxParentClass (Pawn|GetController)))
  (Default|SetDesiredLocation _asbp_ebaicontroller_max_parent_class (Transformation|GetActorLocation BuildingToWorkAt))
  (Variables|/Game/EB/Blueprints/BP_EBAIControllerMaxParentClass.BP_EBAIControllerMaxParentClass_C|SetBuildingToWorkAt _asbp_ebaicontroller_max_parent_class BuildingToWorkAt)
  (Default|GotoStateAIWokerorWhataver _asbp_ebaicontroller_max_parent_class "NewEnumerator5" (Variables|/Game/EB/Blueprints/BP_EBAIControllerMaxParentClass.BP_EBAIControllerMaxParentClass_C|GetAI_StateOfWorkerOrWhataver _asbp_ebaicontroller_max_parent_class)))

(event EventRTSUnitRun
  (params (RunLoc :type Vector :default "0, 0, 0"))
  ;[1 1 1] Use this for moving already
  (bind _asbp_ebaicontroller_max_parent_class (Utilities|Casting|CastToBP_EBAIControllerMaxParentClass (Pawn|GetController)))
  (Default|SetDesiredLocation _asbp_ebaicontroller_max_parent_class RunLoc)
  (Development|PrintString "FROM EB Running  to a location WORK IN PROGRESS!!!74 " true true "(R=1.000000,G=0.891769,B=0.000000,A=1.000000)"))

(event EventRTSSendUnittoSabotage
  (params (BuildingSabotaging :type BP%20Building%20Max%20Parent%20Class%20Object%20Reference))
  ;[1 1 1] Use this for sabotaging already
  (bind _asbp_ebaicontroller_max_parent_class (Utilities|Casting|CastToBP_EBAIControllerMaxParentClass (Pawn|GetController)))
  (Default|SetDesiredLocation _asbp_ebaicontroller_max_parent_class (Transformation|GetActorLocation BuildingSabotaging))
  (Default|GotoStateAIWokerorWhataver _asbp_ebaicontroller_max_parent_class "NewEnumerator6" (Variables|/Game/EB/Blueprints/BP_EBAIControllerMaxParentClass.BP_EBAIControllerMaxParentClass_C|GetAI_StateOfWorkerOrWhataver _asbp_ebaicontroller_max_parent_class))
  (Variables|/Game/EB/Blueprints/BP_EBAIControllerMaxParentClass.BP_EBAIControllerMaxParentClass_C|SetBuildingToSabotage _asbp_ebaicontroller_max_parent_class BuildingSabotaging))

(event EventRTSUnitMove
  (params (MoveLoc :type Vector :default "0, 0, 0"))
  ;[1 1 1] To move to a place
  (bind _asbp_ebaicontroller_max_parent_class (Utilities|Casting|CastToBP_EBAIControllerMaxParentClass (Pawn|GetController)))
  (Default|SetDesiredLocation _asbp_ebaicontroller_max_parent_class MoveLoc)
  (Default|GotoStateAIWokerorWhataver _asbp_ebaicontroller_max_parent_class "NewEnumerator0" "NewEnumerator0"))

(event EventRTSInterfunctUnitGetDeselected
  (params (ControllerUnselecting :type Player%20Controller%20Object%20Reference))
  ;[1 1 1] Get deselected
  (bind _asbp_player_controller_rtsmax_par (Utilities|Casting|CastToBP_PlayerControllerRTSMaxPar ControllerUnselecting))
  (bind _isactoroneofitsactors (Default|STRATEGYIsThisActorOneOfItsActors _asbp_player_controller_rtsmax_par self))
  (if _isactoroneofitsactors
    (if (not (< (Utilities|Array|FindItem (Variables|/Game/EB/Blueprints/BP_PlayerControllerRTSMaxPar.BP_PlayerControllerRTSMaxPar_C|GetAllActorsSelected _asbp_player_controller_rtsmax_par) self) 0))
      (Utilities|Array|RemoveItem (Variables|/Game/EB/Blueprints/BP_PlayerControllerRTSMaxPar.BP_PlayerControllerRTSMaxPar_C|GetAllActorsSelected _asbp_player_controller_rtsmax_par) self)
      (CallFunction|ClientSetSelectCircleVisible false))))

(fn ConstructionScript
  (|CallParentFunction))

(fn HANDLEConstructBuildingHologram
  ;[1 1 1] WIP Should be transfered here it's in PC and AI
)