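; Spawner actor that creates a team's starting nomad worker for an AI opponent; the player spawn function is an empty stub.
; SpawnOpponentsStuff calls SpawnTeamStuff, which projects the spawner's location onto the landscape via the game mode and spawns a BP_EBWorker there.
; It sets the worker's team, registers it with the AI RTS controller and re-applies ownership as a hack.
; Start-type switches exist but add no extra workers or buildings.
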(event EventBeginPlay)

(event Collision|EventActorBeginOverlap
  (params (OtherActor :type Actor%20Object%20Reference)))

(event EventTick
  (params (DeltaSeconds :type Float%20%28single-precision%29)))

(fn ConstructionScript)

(fn SpawnOpponentsStuff
  (params (StartingOfOponent :type EN_GenesisOfOpponentOrPlayer%20Enum :default "NewEnumerator0") (TeamNum :type Integer) (ControllerSpawningOwner :type Controller%20Object%20Reference))
  ;[1 1 1] If nomad just a worker if not nomad just workers if ..... self explanatory
  (CallFunction|SpawnTeamStuff StartingOfOponent StartingOfOponent TeamNum ControllerSpawningOwner))

(fn SpawnPlayerStuff)

(fn SpawnMainNomadWorkerandReturnIt
  (params (genesisOfBotOrPlayer :type EN_GenesisOfOpponentOrPlayer%20Enum :default "NewEnumerator0") (NomadWorkerLoc :type Vector) (ControllerOwner :type Controller%20Object%20Reference))
  (switch Utilities|FlowControl|Switch|SwitchonEN_GenesisOfOpponentOrPlayer genesisOfBotOrPlayer
    (:NewEnumerator0
      _)
    (:NewEnumerator1
      _)
    (:NewEnumerator2
      _))
  (bind _returnvalue (Game|SpawnActorfromClass "/Game/EB/Blueprints/BP_EBWorker.BP_EBWorker_C" (Math|Transform|MakeTransform NomadWorkerLoc) "AdjustIfPossibleButAlwaysSpawn" ControllerOwner 0))
  (return _returnvalue))

(fn SpawnTeamStuff
  (params (Selection :type EN_GenesisOfOpponentOrPlayer%20Enum :default "NewEnumerator0") (genesisOfBotOrPlayer :type EN_GenesisOfOpponentOrPlayer%20Enum :default "NewEnumerator0") (TeamNum :type Integer) (ControllerOwner :type Controller%20Object%20Reference))
  (switch Utilities|FlowControl|Switch|SwitchonEN_GenesisOfOpponentOrPlayer Selection
    (:NewEnumerator0
      _)
    (:NewEnumerator1
      _)
    (:NewEnumerator2
      _))
  (bind _asbp_ebgame_max_par (Utilities|Casting|CastToBP_EBGameMaxPar (Game|GetGameMode)))
  (bind _returnedloconplace (Default|TraceDownLandscapeandGetLoc _asbp_ebgame_max_par (Transformation|GetActorLocation)))
  (bind _returnedworker (CallFunction|SpawnMainNomadWorkerandReturnIt genesisOfBotOrPlayer _returnedloconplace ControllerOwner))
  (Variables|/Game/EB/Blueprints/TSICharacterMaxParentClassEB.TSICharacterMaxParentClassEB_C|SetTeamNum _returnedworker TeamNum)
  (bind _asbp_ebaiopponent (Utilities|Casting|CastToBP_EBAIRTSControllerOpponent ControllerOwner))
  (Development|PrintString (Utilities|String|Append "from eb sPawnerrt THE BOT IS" (Utilities|GetDisplayName _asbp_ebaiopponent) "WOKRE RIS" (Utilities|GetDisplayName _returnedworker)) true true "(R=0.157877,G=1.000000,B=0.000000,A=1.000000)" 2e+01)
  (Default|STRATEGYAddtoOwnedActors _asbp_ebaiopponent _returnedworker)
  ;[1 1 1] Hack for some reason te owner gets assigned something which is the controller 4.24 stuff
  (Actor|SetOwner _returnedworker ControllerOwner))