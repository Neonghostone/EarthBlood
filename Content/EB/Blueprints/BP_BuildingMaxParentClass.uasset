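; Parent class for RTS buildings that handles selection, worker assignment and unit recruitment.
; Overlapping workers fill limited slots, and the mesh ignores pawns until no overlapping worker is near.
; Server-side recruitment checks money and cooldown, then spawns units with owner and team, giving TSI characters a formation.
; Also provides a timed rush with random outcome and blinking material swaps tied to the option menu, with hooks for child overrides.
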(event Custom|StartTheRush
  (CallFunction|ServerDoRush))

(event Custom|ServerDoRush
  (if (Utilities|Time|IsTimerActivebyHandle (Variables|Default|GetRushHandle))
    (bind _asbp_player_controller_rtsmax_par (Utilities|Casting|CastToBP_PlayerControllerRTSMaxPar (Components|GetOwner)))
    (Default|CORELOGAddLogMessage _asbp_player_controller_rtsmax_par "Already on a rush wait" 2.0 (Utilities|Struct|MakeSlateColor "(R=0.208333,G=0.009650,B=0.000000,A=1.000000)"))
    (else
      (bind _returnvalue (Utilities|Time|SetTimerbyFunctionName 0 "RUSH_TimerBasedEndRush" 1.0))
      (Variables|Default|SetRushHandle _returnvalue))))

(event Custom|EndRushResults
  ;[1 1 1] Becareful they are overriden
  (if (Math|Random|RandomBool)
    (CallFunction|EndRushFailure)
    (else
      (CallFunction|EndRushSuccesful))))

(event Custom|ServerRecruitUnit
  (params (UnitArchetype :type Actor%20Class%20Reference))
  ;[1 1 1] Networking stuff
  (CallFunction|STATEGYRecruitUnit UnitArchetype))

(event Custom|EndRushSuccesful
  ;[1 1 1] Becareful they are overriden
  (bind _asbp_player_controller_rtsmax_par (Utilities|Casting|CastToBP_PlayerControllerRTSMaxPar (Components|GetOwner)))
  (Default|CORELOGAddLogMessage _asbp_player_controller_rtsmax_par "Rush ended succesfuly" 2.0 (Utilities|Struct|MakeSlateColor "(R=0.000000,G=1.000000,B=0.017252,A=1.000000)")))

(event Custom|EndRushFailure
  ;[1 1 1] Becareful they are overriden
  (bind _asbp_player_controller_rtsmax_par (Utilities|Casting|CastToBP_PlayerControllerRTSMaxPar (Components|GetOwner)))
  (Default|CORELOGAddLogMessage _asbp_player_controller_rtsmax_par "Rush ended in failure" 2.0 (Utilities|Struct|MakeSlateColor "(R=1.000000,G=0.000000,B=0.018600,A=1.000000)")))

(event EventRTSMouseInterfunctonMouseRightClick
  (params (ControllerThatRightMouseClicked :type Player%20Controller%20Object%20Reference))
  (bind _array_element (Utilities|Array|ForEachLoopwithBreak (Variables|/Game/EB/Blueprints/BP_PlayerControllerRTSMaxPar.BP_PlayerControllerRTSMaxPar_C|GetAllActorsSelected (.AsBP%20Player%20Controller%20RTSMax%20Par (Utilities|Casting|CastToBP_PlayerControllerRTSMaxPar (Game|GetPlayerController 0)))))
    (:LoopBody
      (bind _asbp_ebworker (Utilities|Casting|CastToBP_EBWorker _array_element))
      (Default|StartGettingClosetoWorkonBuilding _asbp_ebworker self)
      (bind _asbp_player_controller_rtsmax_par (Utilities|Casting|CastToBP_PlayerControllerRTSMaxPar ControllerThatRightMouseClicked))
      (Default|COREAssignLastActorRightClicked _asbp_player_controller_rtsmax_par self))))

(event EventBeginPlay
  (CallFunction|OVERLAPCHECKSetCollisiontToggle)
  (|CallParentFunction))

(event EventActorBeginOverlap
  (params (OtherActor :type Actor%20Object%20Reference))
  ;[1 1 1] I skiped this thing
  (bind _asbp_ebworker (Utilities|Casting|CastToBP_EBWorker OtherActor))
  (CallFunction|STRATEGYReciveNewUnitWorkinginPlace _asbp_ebworker)
  (Default|StartWorkingonBuilding _asbp_ebworker self))

(event EventTick
  (params (DeltaSeconds :type Float%20%28single-precision%29))
  (Utilities|FlowControl|Sequence
    (:then_0
      (Rendering|Components|TextRender|SetText (Variables|/Game/EB/Blueprints/UW_NumOfWorkersWorkingInBuilding.UW_NumOfWorkersWorkingInBuilding_C|GetWorkersText (.AsUW%20Num%20Of%20Workers%20Working%20in%20Building (Utilities|Casting|CastToUW_NumOfWorkersWorkingInBuilding (UserInterface|GetUserWidgetObject (Variables|Default|GetWorkersWorkingAtBuildingWidget))))) (Utilities|Text|ToText(String) (Utilities|String|Append "Workers " (Utilities|String|ToString(Integer) (Utilities|Array|Length (Variables|Default|GetAssignedWorkers))) "/" (Utilities|String|ToString(Integer) (Variables|Default|GetWorkerLimit))))))
    (:then_1
      (if (Variables|/Game/EB/Blueprints/BP_PlayerControllerRTSMaxPar.BP_PlayerControllerRTSMaxPar_C|GetbSeeDebuggingInfo (.AsBP%20Player%20Controller%20RTSMax%20Par (Utilities|Casting|CastToBP_PlayerControllerRTSMaxPar (Game|GetPlayerController 0))))
        (Rendering|Debug|DrawDebugString (+ (Transformation|GetActorLocation) "0, 0,90.000000") (Utilities|String|Append "FROM TSIchar the Civ asset is TEAM TEAM NUM =" "(" (Utilities|String|ToString(Integer) (Variables|Default|GetTeamNum)) ")") 0 "(R=1.000000,G=1.000000,B=1.000000,A=1.000000)")))
    (:then_2
      (if (not (CallFunction|OVERLAPCHECKIsAnyWorkerTooClose))
        (if (not (Variables|Default|GetbCollisionSetAlready))
          (Variables|Default|SetbCollisionSetAlready true)
          (CallFunction|OVERLAPCHECKSetCollisiontToggle))))))

(event EventRTSInterfunctUnitGetSelected
  (params (ControllerClicking :type Player%20Controller%20Object%20Reference))
  (bind _asbp_player_controller_rtsmax_par (Utilities|Casting|CastToBP_PlayerControllerRTSMaxPar ControllerClicking))
  (bind _self self)
  ;[1 1 1] Get selected
  (Utilities|FlowControl|Sequence
    (:then_0
      (bind _isactoroneofitsactors (Default|STRATEGYIsThisActorOneOfItsActors _asbp_player_controller_rtsmax_par _self))
      (if _isactoroneofitsactors
        (Utilities|Array|Add (Variables|/Game/EB/Blueprints/BP_PlayerControllerRTSMaxPar.BP_PlayerControllerRTSMaxPar_C|GetAllActorsSelected _asbp_player_controller_rtsmax_par) self)))
    (:then_1
      (bind _isactoroneofitsactors_2 (Default|STRATEGYIsThisActorOneOfItsActors _asbp_player_controller_rtsmax_par _self))
      (if _isactoroneofitsactors_2
        (CallFunction|HUDSpawnCorrespondingHUD)))))

(event Collision|EventActorEndOverlap
  (params (OtherActor :type Actor%20Object%20Reference))
  (bind _asbp_ebworker (Utilities|Casting|CastToBP_EBWorker OtherActor))
  ;[1 1 1] I skiped this thing
  (Default|StopWorkingonBuilding _asbp_ebworker self)
  (Utilities|Array|RemoveItem (Variables|Default|GetAssignedWorkers) _asbp_ebworker))

(event EventRTSInterfunctUnitGetDeselected
  (params (ControllerUnselecting :type Player%20Controller%20Object%20Reference))
  (bind _asbp_player_controller_rtsmax_par (Utilities|Casting|CastToBP_PlayerControllerRTSMaxPar ControllerUnselecting))
  (bind _allactorsselected (Variables|/Game/EB/Blueprints/BP_PlayerControllerRTSMaxPar.BP_PlayerControllerRTSMaxPar_C|GetAllActorsSelected _asbp_player_controller_rtsmax_par))
  ;[1 1 1] Get deselected
  (Utilities|FlowControl|Sequence
    (:then_0
      (bind _isactoroneofitsactors (Default|STRATEGYIsThisActorOneOfItsActors _asbp_player_controller_rtsmax_par self))
      (if _isactoroneofitsactors
        (if (not (< (Utilities|Array|FindItem _allactorsselected self) 0))
          (Utilities|Array|RemoveItem _allactorsselected self))))
    (:then_1
      (CallFunction|HUDHideAllCorrespondingHUD))))

(event EventRTSMouseInterfunctonMouseLeftClick
  (params (ControllerThat0LeftClicked :type Player%20Controller%20Object%20Reference))
  (CallFunction|STRATEGYBuildingGetSelectedtoRecruit ControllerThat0LeftClicked)
  (bind _asbp_player_controller_rtsmax_par (Utilities|Casting|CastToBP_PlayerControllerRTSMaxPar ControllerThat0LeftClicked)))

(event EventRTSMouseInterfunctonMouseOver
  (params (controllerThatMouseOvered :type Player%20Controller%20Object%20Reference))
  (Development|PrintString "FROM Building we hovering"))

(event EventRTSMouseInterFunctonMouseOut
  (params (ControllerMousseOuted :type Player%20Controller%20Object%20Reference)))

(event Custom|InitializeBlinkingMaterials
  ;[1 1 1] Implement in child classes with specific Blinking Material Instances (see "BP_AdminHutConstruction" as example)
  (for _array_element (Blinking|GetBlinkingMeshes)
    (Blinking|RegisterDefaultBlinkingMaterialstoMeshComponent _array_element)))

(event Custom|EnableBlinking
  (params (PC :type BP%20Player%20Controller%20RTS%20Max%20Par%20Object%20Reference))
  (bind _hud (Default|GetHUDMaxParent PC))
  ;[1 1 1] Starts the blinking and opens the option menu
  (Utilities|IsValid _hud
    (:Is%20Valid
      (Default|ShowRightclickOptionMenu _hud self)
      (CallFunction|ApplyMaterialSets false))))

(event Custom|DisableBlinking
  (params (PC :type BP%20Player%20Controller%20RTS%20Max%20Par%20Object%20Reference))
  (bind _hud (Default|GetHUDMaxParent PC))
  ;[1 1 1] Stops the blinking and closes the option menu
  (Utilities|IsValid _hud
    (:Is%20Valid
      (Default|HideRightclickOptionMenu _hud)
      (CallFunction|ApplyMaterialSets true))))

(event Custom|ApplyMaterialSets
  (params (ApplyOriginals :type Boolean))
  ;[1 1 1] Reassigns the original or blinking materials to every blinking mesh
  (for _array_element (Blinking|GetBlinkingMeshes)
    (if (.ReturnValue (Utilities|Map|Find (Variables|Blinking|GetBlinkingMeshIndices) _array_element))
      (for _index (range 0 (- (Rendering|Material|GetNumMaterials _array_element) 1))
        (Rendering|Material|SetMaterial _array_element _index (Utilities|Array|Get(acopy) (select ApplyOriginals (.OriginalMaterials (Utilities|Struct|BreakSTRUCT_BlinkingMaterialData (Utilities|Array|Get(acopy) (Variables|Blinking|GetBlinkingMaterialDatas) (.Value (Utilities|Map|Find (Variables|Blinking|GetBlinkingMeshIndices) _array_element))))) (.BlinkingMaterialInstances (Utilities|Struct|BreakSTRUCT_BlinkingMaterialData (Utilities|Array|Get(acopy) (Variables|Blinking|GetBlinkingMaterialDatas) (.Value (Utilities|Map|Find (Variables|Blinking|GetBlinkingMeshIndices) _array_element)))))) _index))))))

(event Custom|ToggleBlinking
  (params (PC :type BP%20Player%20Controller%20RTS%20Max%20Par%20Object%20Reference))
  ;[1 1 1] Either enables or disables the blinking / shows or hides the options menu
  (if (Default|IsCurrentRightClickMenuValidandVisible (Default|GetHUDMaxParent PC))
    (CallFunction|DisableBlinking PC)
    (else
      (CallFunction|EnableBlinking PC))))

(event EventEndPlay
  (params (EndPlayReason :type EEndPlayReason%20Enum :default "Destroyed"))
  ;[1 1 1] In case this Actor is destroyed and its Rightclick options menu is open, close the menu. Also, removes the menu from the list
  (if (Utilities|Enum|Equal(Enum) EndPlayReason "Destroyed")
    (bind _asbp_player_controller_rtsmax_par (Utilities|Casting|CastToBP_PlayerControllerRTSMaxPar (Game|GetPlayerController 0)))
    (Default|RemoveRightclickOptionMenu (Default|GetHUDMaxParent _asbp_player_controller_rtsmax_par) self)))

(fn ConstructionScript
  (if (not (Networking|IsDedicatedServer))
    (Blinking|RegisterOriginalMaterials)))

(fn STRATEGYBuildingGetSelectedtoRecruit
  (params (Controller :type Controller%20Object%20Reference))
  (bind _asbp_player_controller_rtsmax_par (Utilities|Casting|CastToBP_PlayerControllerRTSMaxPar Controller))
  ;[1 1 1] CASE we are a playerController
  (Default|COREGotoNewState _asbp_player_controller_rtsmax_par "NewEnumerator1")
  (bind _isselected (Default|COREIsActorSelected _asbp_player_controller_rtsmax_par self))
  (if (not _isselected)
    (Default|COREAddAunitintheSelectedActors _asbp_player_controller_rtsmax_par self)
    (Networking|SwitchHasAuthority
      (:Remote
        (Default|ServerClientServerSelectThisUnit _asbp_player_controller_rtsmax_par self)))))

(fn STRATEGYBuildingGetUnselectedtoBuild
  (params (ControllerUnselecting :type Controller%20Object%20Reference))
  (bind _asbp_player_controller_rtsmax_par (Utilities|Casting|CastToBP_PlayerControllerRTSMaxPar ControllerUnselecting))
  (Default|CORERemoveUnitfromSelectedActors _asbp_player_controller_rtsmax_par self))

(fn STRATEGYStartRercruitUnit
  (params (UnitArchetype :type Actor%20Class%20Reference))
  (Networking|SwitchHasAuthority
    (:Authority
      (CallFunction|STATEGYRecruitUnit UnitArchetype))
    (:Remote
      (CallFunction|ServerRecruitUnit UnitArchetype))))

(fn STATEGYRecruitUnit
  (params (UnitArchetype :type Actor%20Class%20Reference))
  (bind _returnvalue (Components|GetOwner))
  (bind _bcooldown (CallFunction|STRATEGYBHasNoCoolDownonRecruiting))
  ;[1 1 1] REMAKE THIS INTO 2 Branches and more organized SOLID SOLID SOLID
  ;;[1 1 1] remove this
  (Development|PrintString "FROM BP Max parent recuriting")
  (if _bcooldown
    (Development|PrintString (Utilities|String|Append "from bp bu8ilding is " (Utilities|String|ToString(Boolean) _bcooldown)))
    (bind _output_get (LocalVariables|SetLocalHiringFee (Math|Random|RandomIntegerinRange (Variables|Default|GetWorkerHiringFeeMin) (Variables|Default|GetWorkerHiringFeeMax))))
    ;;[1 1 1] Using an authority checkk just to change the team index now
    (Networking|SwitchHasAuthority
      (:Authority
        (if (CallFunction|STRATEGYBHasEnoughMoney _output_get)
          (bind _returnvalue_2 (Game|SpawnActorfromClass UnitArchetype (Math|Conversions|ToTransform(Vector) (Transformation|GetWorldLocation (Variables|Default|GetPointToSpawn))) "AdjustIfPossibleButAlwaysSpawn" (Components|GetOwner) 0))
          (Utilities|FlowControl|Sequence
            (:then_0
              (Utilities|FlowControl|Sequence
                (:then_0
                  (bind _asbp_player_controller_rtsmax_par (Utilities|Casting|CastToBP_PlayerControllerRTSMaxPar (Components|GetOwner)))
                  ;;[1 1 1] Worker stuff
                  (Variables|/Game/EB/Blueprints/BP_PlayerControllerRTSMaxPar.BP_PlayerControllerRTSMaxPar_C|SetRPGMoney _asbp_player_controller_rtsmax_par (- (Variables|/Game/EB/Blueprints/BP_PlayerControllerRTSMaxPar.BP_PlayerControllerRTSMaxPar_C|GetRPGMoney _asbp_player_controller_rtsmax_par) (Math|Float|Truncate (Math|Conversions|ToFloat(Integer) _output_get))))
                  (bind _playerindex (Class|TurnBasedBlueprintLibrary|GetMyPlayerIndex _asbp_player_controller_rtsmax_par))
                  (Utilities|IsValid _asbp_player_controller_rtsmax_par
                    (:Is%20Valid
                      (Default|STRATEGYAddActortoOwnedActors _asbp_player_controller_rtsmax_par _returnvalue_2))))
                (:then_1
                  (Utilities|FlowControl|Sequence
                    (:then_0
                      ;;[1 1 1] Worker
                      (bind _asbp_inv_character_max_parent (Utilities|Casting|CastToBP_InvCharacterMaxParent _returnvalue_2))
                      (Utilities|FlowControl|Sequence
                        (:then_0
                          (bind _asbp_player_controller_rtsmax_par_2 (Utilities|Casting|CastToBP_PlayerControllerRTSMaxPar (Components|GetOwner _asbp_inv_character_max_parent)))
                          (Default|STRATEGYSetNewTeam _asbp_inv_character_max_parent (Variables|/Game/EB/Blueprints/BP_PlayerControllerRTSMaxPar.BP_PlayerControllerRTSMaxPar_C|GetTeamNum _asbp_player_controller_rtsmax_par_2)))
                        (:then_1
                          (bind _asbp_ebaiopponent (Utilities|Casting|CastToBP_EBAIOpponent (Components|GetOwner _asbp_inv_character_max_parent)))
                          (Default|STRATEGYSetNewTeam _asbp_inv_character_max_parent (Math|Conversions|ToByte(Integer) (Variables|/Game/EB/Blueprints/BP_EBAIOpponent.BP_EBAIOpponent_C|GetTeamNumAIOponent _asbp_ebaiopponent))))))
                    (:then_1
                      ;;;[1 1 1] Security
                      (bind _astsicharacter_max_parent_class_in_use (Utilities|Casting|CastToTSICharacterMaxParentClassInUse _returnvalue_2))
                      (Utilities|FlowControl|Sequence
                        (:then_0
                          (bind _asbp_player_controller_rtsmax_par_3 (Utilities|Casting|CastToBP_PlayerControllerRTSMaxPar _returnvalue))
                          (Utilities|IsValid _asbp_player_controller_rtsmax_par_3
                            (:Is%20Valid
                              (Default|STRATEGYAddActortoOwnedActors _asbp_player_controller_rtsmax_par_3 _returnvalue_2)
                              ;;;[1 1 1] Spawn formation info here
                              (Default|SetTeamNum _astsicharacter_max_parent_class_in_use (Math|Conversions|ToInteger(Byte) (Variables|/Game/EB/Blueprints/BP_PlayerControllerRTSMaxPar.BP_PlayerControllerRTSMaxPar_C|GetTeamNum _asbp_player_controller_rtsmax_par_3))))))
                        (:then_1
                          (bind _asbp_ebaiopponent_2 (Utilities|Casting|CastToBP_EBAIOpponent _returnvalue))
                          (Utilities|IsValid _astsicharacter_max_parent_class_in_use
                            (:Is%20Valid
                              (Default|STRATEGYAddtoOwnedActors _asbp_ebaiopponent_2 _astsicharacter_max_parent_class_in_use)
                              (Default|SetTeamNum _astsicharacter_max_parent_class_in_use (Variables|/Game/EB/Blueprints/BP_EBAIOpponent.BP_EBAIOpponent_C|GetTeamNumAIOponent _asbp_ebaiopponent_2))))))
                      (Utilities|IsValid (Variables|/Game/TSIBPTSICntnt/TSIBlueprints/Pawns/TSICharacterMaxParentClassInUse.TSICharacterMaxParentClassInUse_C|GetFormationInfo _astsicharacter_max_parent_class_in_use)
                        (:Is%20Not%20Valid
                          (bind _returnvalue_3 (Game|SpawnActorfromClass "/Game/TSIBPTSICntnt/TSIBlueprints/FormationSystem/FormationSystemOfLeader.FormationSystemOfLeader_C" (Math|Transform|MakeTransform "0, 0, 0") "Undefined" _astsicharacter_max_parent_class_in_use _astsicharacter_max_parent_class_in_use _astsicharacter_max_parent_class_in_use 0 0 _astsicharacter_max_parent_class_in_use))
                          (Variables|/Game/TSIBPTSICntnt/TSIBlueprints/FormationSystem/FormationSystemOfLeader.FormationSystemOfLeader_C|SetUnitStruct _returnvalue_3 (Utilities|Struct|MakeSTRUCT_UnitActualFormationn _astsicharacter_max_parent_class_in_use (Utilities|Array|MakeArray)))
                          (bind _output_get_2 (Variables|/Game/TSIBPTSICntnt/TSIBlueprints/Pawns/TSICharacterMaxParentClassInUse.TSICharacterMaxParentClassInUse_C|SetFormationInfo _astsicharacter_max_parent_class_in_use _returnvalue_3))
                          (Variables|/Game/TSIBPTSICntnt/TSIBlueprints/FormationSystem/FormationSystemMaxParentClass.FormationSystemMaxParentClass_C|SetLeader _returnvalue_3 _astsicharacter_max_parent_class_in_use)
                          (Variables|/Game/TSIBPTSICntnt/TSIBlueprints/FormationSystem/FormationSystemMaxParentClass.FormationSystemMaxParentClass_C|SetGroupLeader _returnvalue_3 _astsicharacter_max_parent_class_in_use)
                          (Default|AddNewMemberinFormationCreatingGroup _returnvalue_3 _astsicharacter_max_parent_class_in_use 0 "Oxford")
                          ;;[1 1 1] Advance at all costs and fire at will
                          (Default|GiveOrdertoAllGLs _returnvalue_3 5 "0, 0, 0"))))))))
            (:then_1
              (if (not (Utilities|Time|IsTimerActivebyHandle (Variables|Default|GetCoolDownRecruitingHandle)))
                ;;[1 1 1] COOL DOWN FOr recruiting
                (Utilities|FlowControl|Sequence
                  (:then_1
                    (CallFunction|STRATEGYSetCoolDownforRecruiting 1.0)
                    (bind _asbp_player_controller_rtsmax_par_4 (Utilities|Casting|CastToBP_PlayerControllerRTSMaxPar (Game|GetPlayerController 0)))
                    (Default|StartPlayingSound _asbp_player_controller_rtsmax_par_4 "/Game/EB/Audio/Sounds/HireWorker_1a.HireWorker_1a" (Transformation|GetActorLocation self))
                    (return true)))))))))
    (else
      (Development|PrintString "FROM BP building d not recur5it")
      (return false))))

(fn STRATEGYReciveNewUnitWorkinginPlace
  (params (NewUnit :type BP%20EB%20Char%20Max%20Parent%20Object%20Reference))
  (bind _assignedworkers (Variables|Default|GetAssignedWorkers))
  (bind _outactors (Actor|GetAllActorsOfClass "BP_BuildingMaxParentClass_C"))
  (for _array_element _outactors
    (if (not (== (Utilities|Array|FindItem (Variables|BP_BuildingMaxParentClass_C|GetAssignedWorkers _array_element) NewUnit) -1))
      (return)))
  (if (< (Utilities|Array|Length _assignedworkers) (Variables|Default|GetWorkerLimit))
    (Utilities|Array|Add _assignedworkers NewUnit)))

(fn STRATEGYNewUnitStopsWorkinginPlace
  (params (NewUnit :type BP%20EB%20Char%20Max%20Parent%20Object%20Reference))
  (Utilities|Array|RemoveItem (Variables|Default|GetAssignedWorkers) NewUnit))

(fn STRATEGYBHasEnoughMoney
  (params (MoneyToSpend :type Integer))
  (if (> (Variables|/Game/EB/Blueprints/BP_PlayerControllerRTSMaxPar.BP_PlayerControllerRTSMaxPar_C|GetRPGMoney (.AsBP%20Player%20Controller%20RTSMax%20Par (Utilities|Casting|CastToBP_PlayerControllerRTSMaxPar (Game|GetPlayerController 0)))) MoneyToSpend)
    (return true)
    (else
      (return false))))

(fn STATEGYCoolDownRecruitUnit
  (params (TimeForCoolDown :type Float%20%28single-precision%29))
  (Utilities|Time|SetTimerbyFunctionName 0 "STRATEGY_TimerBasedCooldownRUnit" TimeForCoolDown))

(fn STRATEGYTimerBasedCooldownRUnit)

(fn STRATEGYBHasNoCoolDownonRecruiting
  (return (not (Utilities|Time|IsTimerActivebyHandle (Variables|Default|GetCoolDownRecruitingHandle)))))

(fn STRATEGYSetCoolDownforRecruiting
  (params (NewTimer :type Float%20%28single-precision%29))
  (bind _returnvalue (Utilities|Time|SetTimerbyFunctionName 0 "STRATEGY_TimerBasedCooldownRUnit" NewTimer))
  (Variables|Default|SetCoolDownRecruitingHandle _returnvalue))

(fn HUDSpawnCorrespondingHUD)

(fn HUDHideAllCorrespondingHUD
  (bind _asbp_player_controller_rtsmax_par (Utilities|Casting|CastToBP_PlayerControllerRTSMaxPar (Components|GetOwner)))
  (Default|HideAdminHud _asbp_player_controller_rtsmax_par))

(fn RUSHStartRush
  (CallFunction|StarttheRush))

(fn OVERLAPCHECKIsAnyWorkerTooClose
  (for _array_element (Collision|GetOverlappingActors "/Game/EB/Blueprints/BP_EBWorker.BP_EBWorker_C" :!class /Script/Engine.Actor)
    (if (<= (Math|Vector|VectorLength (- (Transformation|GetActorLocation _array_element) (Transformation|GetActorLocation self))) 1e+03)
      (return true)))
  (return false))

(fn OVERLAPCHECKSetCollisiontToggle
  (bind _self self)
  (bind _buildingsmesh (Variables|Default|GetBuildingsMesh))
  (if (Variables|Default|GetbCollisionSetAlready)
    (Collision|SetCollisionEnabled _buildingsmesh "QueryAndPhysics")
    (Collision|SetCollisionResponsetoAllChannels _buildingsmesh "ECR_Block")
    (bind _asbp_building_oil_pump_construction (Utilities|Casting|CastToBP_BuildingOilPumpConstruction _self))
    (Collision|SetCollisionEnabled (Variables|/Script/Engine.Character|GetMesh _asbp_building_oil_pump_construction) "QueryAndPhysics")
    (Collision|SetCollisionResponsetoAllChannels (Variables|/Script/Engine.Character|GetMesh _asbp_building_oil_pump_construction) "ECR_Block")
    (else
      (Collision|SetCollisionResponsetoChannel _buildingsmesh "ECC_Pawn" "ECR_Ignore")
      (bind _asbp_building_oil_pump_construction_2 (Utilities|Casting|CastToBP_BuildingOilPumpConstruction _self))
      (Collision|SetCollisionResponsetoChannel (Variables|/Script/Engine.Character|GetMesh _asbp_building_oil_pump_construction_2) "ECC_Pawn" "ECR_Ignore"))))

(fn RUSHReturnPercentageOfSuccesOfRush
  ;[1 1 1] WIP
  (return 75))

(fn RUSHTimerBasedEndRush
  (CallFunction|EndRushResults))

(fn GetBlinkingMeshes
  ;[1 1 1] Re-Implement that in buildings, which have different Mesh Components (e.g. Skeletal Mesh like the Oilpump)
  (return (Utilities|Array|MakeArray (Variables|Default|GetBuildingsMesh))))

(fn RegisterOriginalMaterials
  (bind _array (Utilities|Array|MakeArray 0))
  (for (_array_element _array_index) (Blinking|GetBlinkingMeshes)
    (Utilities|Map|Add (Variables|Blinking|GetBlinkingMeshIndices) _array_element _array_index)
    (LocalVariables|SetLocalBlinkingMaterialStruct (Utilities|Struct|MakeSTRUCT_BlinkingMaterialData _array_element _array _array))
    (for _index (range 0 (- (Rendering|Material|GetNumMaterials _array_element) 1))
      (Utilities|Array|SetArrayElem (Utilities|Struct|BreakSTRUCT_BlinkingMaterialData (LocalVariables|GetLocalBlinkingMaterialStruct)) _index (Rendering|Material|GetMaterial _array_element _index) true))
    (Utilities|Array|Add (Variables|Blinking|GetBlinkingMaterialDatas) (LocalVariables|GetLocalBlinkingMaterialStruct)))
  (CallFunction|InitializeBlinkingMaterials))

(fn RegisterSetOfBlinkingMaterialInstances
  (params (MeshComponent :type Primitive%20Component%20Object%20Reference) (Instances :type Array%20of%20Material%20Instance%20Object%20References))
  (bind _blinkingmeshindices (Variables|Blinking|GetBlinkingMeshIndices))
  (bind (_value _returnvalue) (Utilities|Map|Find _blinkingmeshindices MeshComponent))
  (if _returnvalue
    (Utilities|Struct|SetmembersinSTRUCT_BlinkingMaterialData (Utilities|Array|Get(acopy) (Variables|Blinking|GetBlinkingMaterialDatas) _value) Instances)))

(fn HidRightclickOptionsMenu
  (params (PC :type BP%20Player%20Controller%20RTS%20Max%20Par%20Object%20Reference))
  (Utilities|IsValid PC
    (:Is%20Valid
      (CallFunction|DisableBlinking PC))))

(fn RegisterDefaultBlinkingMaterialstoMeshComponent
  (params (Mesh :type Primitive%20Component%20Object%20Reference))
  (for _index (range 0 (- (Rendering|Material|GetNumMaterials Mesh) 1))
    (Utilities|Array|Add (LocalVariables|GetCurrentArrayOfInstances) "/Game/EB/3d/Buildings/MA_Blinking_FlatColor_Base.MA_Blinking_FlatColor_Base"))
  (Blinking|RegisterSetOfBlinkingMaterialInstances Mesh (LocalVariables|GetCurrentArrayOfInstances)))

(fn GetBlinkingMaterialsDebugString
  (LocalVariables|SetDebugString "Original Materials:  
")
  (for (_array_element _array_index) (.OriginalMaterials (Utilities|Struct|BreakSTRUCT_BlinkingMaterialData (Utilities|Array|Get(acopy) (Variables|Blinking|GetBlinkingMaterialDatas))))
    (LocalVariables|SetDebugString (Utilities|String|Append (LocalVariables|GetDebugString) (Utilities|String|ToString(Integer) _array_index) ": " (Utilities|GetDisplayName _array_element) " 
")))
  (return (LocalVariables|GetDebugString)))

(fn DrawBlinkingMaterialsDebugString
  (if (not (Networking|IsDedicatedServer))
    (Rendering|Debug|DrawDebugString (+ (Transformation|GetActorLocation) "0, 0,300.000000") (Blinking|GetBlinkingMaterialsDebugString) 0 "(R=1.000000,G=1.000000,B=1.000000,A=1.000000)")))