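; Parent RTS unit character that responds to player selection and right-click move orders and can build and work at buildings.
; Selection events add or remove it from the RTS controller's selected list if that controller owns it, and orders use SimpleMoveToLocation.
; Looping one-second timers advance construction progress until FinishConstruction, or replay work animations, with working also triggering the AI controller.
; Sending it to a building only records the assignment, as the move call is unwired.
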(event EventBeginPlay
  (|CallParentFunction))

(event Collision|EventActorBeginOverlap
  (params (OtherActor :type Actor%20Object%20Reference)))

(event EventTick
  (params (DeltaSeconds :type Float%20%28single-precision%29))
  (|CallParentFunction DeltaSeconds))

(event EventRTSInterfunctHandleRightClickonLSorSMwithSelected
  (params (PlayerControllerUsing :type Player%20Controller%20Object%20Reference) (PlaceOnMap :type Vector :default "0, 0, 0"))
  (bind _returnvalue (Pawn|GetController))
  (if (Utilities|IsValid _returnvalue)
    (AI|Navigation|SimpleMovetoLocation _returnvalue PlaceOnMap)))

(event EventRTSInterfunctUnitGetSelected
  (params (ControllerClicking :type Player%20Controller%20Object%20Reference))
  (bind _asbp_player_controller_rtsmax_par (Utilities|Casting|CastToBP_PlayerControllerRTSMaxPar ControllerClicking))
  (bind _isactoroneofitsactors (Default|STRATEGYIsThisActorOneOfItsActors _asbp_player_controller_rtsmax_par self))
  (if _isactoroneofitsactors
    (Utilities|Array|Add (Variables|/Game/EB/Blueprints/BP_PlayerControllerRTSMaxPar.BP_PlayerControllerRTSMaxPar_C|GetAllActorsSelected _asbp_player_controller_rtsmax_par) self)))

(event EventRTSInterfunctUnitGetDeselected
  (params (ControllerUnselecting :type Player%20Controller%20Object%20Reference))
  (bind _asbp_player_controller_rtsmax_par (Utilities|Casting|CastToBP_PlayerControllerRTSMaxPar ControllerUnselecting))
  (bind _isactoroneofitsactors (Default|STRATEGYIsThisActorOneOfItsActors _asbp_player_controller_rtsmax_par self))
  (if _isactoroneofitsactors
    (if (not (< (Utilities|Array|FindItem (Variables|/Game/EB/Blueprints/BP_PlayerControllerRTSMaxPar.BP_PlayerControllerRTSMaxPar_C|GetAllActorsSelected _asbp_player_controller_rtsmax_par) self) 0))
      (Utilities|Array|RemoveItem (Variables|/Game/EB/Blueprints/BP_PlayerControllerRTSMaxPar.BP_PlayerControllerRTSMaxPar_C|GetAllActorsSelected _asbp_player_controller_rtsmax_par) self))))

(fn ConstructionScript
  (|CallParentFunction))

(fn WorkerBuildStructureDoOnce
  (bind _actualconstructiongettingconstructed (Variables|Default|GetActualConstructionGettingConstructed))
  (Variables|/Game/EB/Blueprints/BP_ConstructionInProcessMaxParentClass.BP_ConstructionInProcessMaxParentClass_C|SetProcessPercent _actualconstructiongettingconstructed (+ (Variables|/Game/EB/Blueprints/BP_ConstructionInProcessMaxParentClass.BP_ConstructionInProcessMaxParentClass_C|GetProcessPercent _actualconstructiongettingconstructed) 26))
  (if (>= (Variables|/Game/EB/Blueprints/BP_ConstructionInProcessMaxParentClass.BP_ConstructionInProcessMaxParentClass_C|GetProcessPercent _actualconstructiongettingconstructed) 100)
    (Variables|/Game/EB/Blueprints/BP_ConstructionInProcessMaxParentClass.BP_ConstructionInProcessMaxParentClass_C|SetProcessPercent _actualconstructiongettingconstructed 100)
    (CallFunction|FinishConstruction _actualconstructiongettingconstructed)
    (Utilities|Time|ClearandInvalidateTimerbyHandle (Variables|Default|GetContructionHandle))
    (else
      (CallFunction|StartPlayingAnimation "/Game/EB/Animations/AM_WorkingOrBuildingABuilding.AM_WorkingOrBuildingABuilding"))))

(fn StartBuildingConstruction
  (params (ConstructionProcessing :type BP%20Construction%20in%20Process%20Max%20Parent%20Class%20Object%20Reference))
  (Variables|Default|SetActualConstructionGettingConstructed ConstructionProcessing)
  (bind _returnvalue (Utilities|Time|SetTimerbyFunctionName 0 "WorkerBuildStructureDoOnce" 1.0 true))
  (Variables|Default|SetContructionHandle _returnvalue))

(fn FinishConstruction
  (params (ConstructionInProcess :type BP%20Construction%20in%20Process%20Max%20Parent%20Class%20Object%20Reference))
  (bind _self self)
  (Default|GetFinished ConstructionInProcess _self (.AsController (Utilities|Casting|CastToController (Components|GetOwner _self)))))

(fn StartWorkingonBuilding
  (params (BuildingWorkingAt :type BP%20Building%20Max%20Parent%20Class%20Object%20Reference))
  (bind _returnvalue (Utilities|Time|SetTimerbyFunctionName 0 "WorkerWorkOnBuildingDoOnce" 1.0 true))
  (Variables|Default|SetWorkingAtHandle _returnvalue)
  (Variables|Default|SetActualBuildingWorkingAt 0)
  (bind _asbp_ebaicontroller_max_parent_class (Utilities|Casting|CastToBP_EBAIControllerMaxParentClass (Pawn|GetController)))
  (Default|AIWorkonAConstruction _asbp_ebaicontroller_max_parent_class))

(fn WorkerWorkonBuildingDoOnce
  (CallFunction|StartPlayingAnimation "/Game/EB/Animations/AM_WorkingAtBuilding.AM_WorkingAtBuilding"))

(fn StartGettingClosetoWorkonBuilding
  (params (Building :type BP%20Building%20Max%20Parent%20Class%20Object%20Reference))
  ;[1 1 1] Should be before moving but it's cool
  (CallFunction|SetBuildingSenttoWorkAssigned Building))

(fn StopWorkingonBuilding
  (params (ConstructionProcessing :type BP%20Building%20Max%20Parent%20Class%20Object%20Reference))
  (Variables|Default|SetActualBuildingWorkingAt 0)
  (Utilities|Time|ClearandInvalidateTimerbyHandle (Variables|Default|GetWorkingAtHandle)))

(fn SetBuildingSenttoWorkAssigned
  (params (BtoGetToWork :type Actor%20Object%20Reference))
  (Variables|Default|SetBuildingSentToWorkAtAssigned BtoGetToWork))