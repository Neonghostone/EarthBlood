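; RTS game mode template that holds team diplomacy, sends it to players on login and answers hostility checks between units.
; DeclareWar records the attacker in the target team's enemy list only.
; Helpers find a worker's player or AI controller by team, spawn formation info on lead pawns, trace to landscape and pick nearest actors.
; Messages reach all players regardless of targeting, crime reports only draw debug text, and most RTS_ query functions are empty stubs.
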(event Custom|RegisterCrimeSpawnsCopsForCriminal
  (params (CrimeLocation :type Vector) (ControllerDoingTheCrime :type Controller%20Object%20Reference) (ActorDoingTheCrime :type Actor%20Object%20Reference))
  (Rendering|Debug|DrawDebugString CrimeLocation (Utilities|String|Append "There was a crime here: " (Utilities|GetDisplayName ControllerDoingTheCrime) "TeamNum: " (Utilities|GetDisplayName (CallFunction|GetControllerbyTeamandUnit ActorDoingTheCrime))) 0 "(R=1.000000,G=0.941911,B=0.000000,A=1.000000)" 1e+05))

(event Custom|DeclareWar
  (params (TeamGettingAttacked :type Byte) (TeamAttacking :type Byte))
  (bind _returnvalue (Math|Conversions|ToInteger(Byte) TeamGettingAttacked))
  (bind _diplomacy (Variables|Default|GetDiplomacy))
  (bind _output (Utilities|Array|Get(acopy) _diplomacy _returnvalue))
  (if (== (Utilities|Array|FindItem (.diplomacyenemies _output) TeamAttacking) -1)
    (Utilities|Array|Add (.diplomacyenemies _output) TeamAttacking)))

(event Custom|BroadcastMessageDependingToWhoWIPChangeParams
  (params (PlayerSendingMessage :type Controller%20Object%20Reference) (ToAll :type Boolean) (SpecificTeam :type Byte) (Message :type String) (SpecificPlayerID :type Name) (bSpecificTeam :type Boolean) (bHasSpecialColor :type Boolean) (SpecialColorInsteadOfBlack :type Linear%20Color%20Structure :default "(R=0.000000,G=0.000000,B=0.000000,A=1.000000)") (ToSelf :type Boolean) (DurationWIP :type Float%20%28single-precision%29) (PrefixOfSentence :type String))
  ;[1 1 1] Kept simple for now since it is debugging
  (bind _outactors (Actor|GetAllActorsOfClass "/Game/EB/Blueprints/BP_PlayerControllerRTSMaxPar.BP_PlayerControllerRTSMaxPar_C"))
  (for _array_element _outactors
    (Default|ClientDotheLogMessageRoll _array_element (Utilities|String|Append (Utilities|GetDisplayName PlayerSendingMessage) PrefixOfSentence Message) DurationWIP (Utilities|Struct|MakeSlateColor SpecialColorInsteadOfBlack))))

(event EventPostLogin
  (params (NewPlayer :type Player%20Controller%20Object%20Reference))
  (bind _asbp_player_controller_rtsmax_par (Utilities|Casting|CastToBP_PlayerControllerRTSMaxPar NewPlayer))
  (Default|ClientReceiveDiplomacy _asbp_player_controller_rtsmax_par (Variables|Default|GetDiplomacy)))

(fn ConstructionScript)

(fn STRATEGYSetArrayPawnsinFormation
  (params (ArrayOfPawns :type Array%20of%20BP%20Inv%20Character%20Max%20Parent%20Object%20References))
  ;[1 1 1] Takes in array of pawns and sets them up in formation
  ;[1 1 1] Not necessary but just in case
  (Networking|SwitchHasAuthority
    (:Authority
      ;[1 1 1] Set mister leader as unit leader
      (bind (_array_element _array_index) (Utilities|Array|ForEachLoopwithBreak ArrayOfPawns)
        (:LoopBody
          (if (== _array_index 0)
            (Default|STRATEGYSrvrSpawntheFormInfo _array_element "/Game/RTSTemplateContent/Blueprints/STRATEGYComponent/FormationClasses/MostNecessaryOnes/BP_FormationInfoLeaderOfunit.BP_FormationInfoLeaderOfunit_C")))))))

(fn TraceDownLandscapeandGetLoc
  (params (SentLoc :type Vector))
  (bind (_x _y) (Math|Vector|BreakVector SentLoc))
  (bind _returnvalue (Math|Vector|MakeVector _x _y 1e+03))
  (bind (_x_2 _y_2) (Math|Vector|BreakVector _returnvalue))
  (bind _outhit (Collision|LineTraceByChannel SentLoc (Math|Vector|MakeVector _x_2 _y_2 -1e+06) "TraceTypeQuery1" false 0 "None"))
  (return (+ (.Location (Collision|BreakHitResult _outhit)) "0, 0,30.000000")))

(fn IsUnitAnEnemyorFriendlyandNeutralDiplomacy
  (params (UnitSelf :type Actor%20Object%20Reference) (UnitOther :type Actor%20Object%20Reference) (MaxProximity :type Float%20%28single-precision%29))
  ;[1 1 1] REWRITE THIS WIP
  ;;[1 1 1] Una mica barruer, if closer than proximity maybe add to enemies
  ;;;[1 1 1] Proximity disabled
  (if (< MaxProximity 5e+02)
    _
    (else
      _))
  (Utilities|FlowControl|Sequence
    (:then_0
      ;;;[1 1 1] Enemy soldier
      ;;;;[1 1 1] US
      (bind _astsicharacter_max_parent_class_from_lsf (Utilities|Casting|CastToTSICharacterMaxParentClassFromLSF UnitSelf))
      (for _array_element (.diplomacyenemies (Utilities|Array|Get(acopy) (Variables|Default|GetDiplomacy) (Variables|/Game/TSIBPTSICntnt/TSIBlueprints/Pawns/TSICharacterMaxParentClassFromLSF.TSICharacterMaxParentClassFromLSF_C|GetTeamNum _astsicharacter_max_parent_class_from_lsf)))
        (bind _astsicharacter_max_parent_class_from_lsf_2 (Utilities|Casting|CastToTSICharacterMaxParentClassFromLSF UnitOther))
        (if (== (Math|Conversions|ToByte(Integer) (Variables|/Game/TSIBPTSICntnt/TSIBlueprints/Pawns/TSICharacterMaxParentClassFromLSF.TSICharacterMaxParentClassFromLSF_C|GetTeamNum _astsicharacter_max_parent_class_from_lsf_2)) _array_element)
          (return true)))
      (return false))
    (:then_1
      ;;;[1 1 1] WORKER!!!
      ;;;;[1 1 1] US
      (bind _astsicharacter_max_parent_class_from_lsf_3 (Utilities|Casting|CastToTSICharacterMaxParentClassFromLSF UnitOther))
      (for _array_element_2 (.diplomacyenemies (Utilities|Array|Get(acopy) (Variables|Default|GetDiplomacy) (Variables|/Game/TSIBPTSICntnt/TSIBlueprints/Pawns/TSICharacterMaxParentClassFromLSF.TSICharacterMaxParentClassFromLSF_C|GetTeamNum _astsicharacter_max_parent_class_from_lsf_3)))
        (bind _astsicharacter_max_parent_class_eb (Utilities|Casting|CastToTSICharacterMaxParentClassEB UnitSelf))
        (if (== (Math|Conversions|ToByte(Integer) (Variables|/Game/EB/Blueprints/TSICharacterMaxParentClassEB.TSICharacterMaxParentClassEB_C|GetTeamNum _astsicharacter_max_parent_class_eb)) _array_element_2)
          (return true)))
      (return false))))

(fn GetControllerbyTeamandUnit
  (params (UnitChecking :type Actor%20Object%20Reference))
  ;[1 1 1] Worker or security
  (Utilities|FlowControl|Sequence
    (:then_0
      (bind _asbp_ebworker_char_max_parent (Utilities|Casting|CastToBP_EBWorkerCharMaxParent UnitChecking))
      (bind _outactors (Actor|GetAllActorsOfClass "/Script/Engine.Controller"))
      (for _array_element _outactors
        (bind _asbp_player_controller_rtsmax_par (Utilities|Casting|CastToBP_PlayerControllerRTSMaxPar _array_element)
          (:then
            (if (== (Variables|/Game/EB/Blueprints/BP_PlayerControllerRTSMaxPar.BP_PlayerControllerRTSMaxPar_C|GetTeamNum _asbp_player_controller_rtsmax_par) (Math|Conversions|ToByte(Integer) (Variables|/Game/EB/Blueprints/TSICharacterMaxParentClassEB.TSICharacterMaxParentClassEB_C|GetTeamNum _asbp_ebworker_char_max_parent)))
              (return _asbp_player_controller_rtsmax_par)))
          (:CastFailed
            (bind _asbp_ebairtscontroller_opponent (Utilities|Casting|CastToBP_EBAIRTSControllerOpponent _array_element))
            (if (== (Variables|/Game/EB/Blueprints/BP_EBAIRTSControllerOpponent.BP_EBAIRTSControllerOpponent_C|GetTeamNumAIOponent _asbp_ebairtscontroller_opponent) (Variables|/Game/EB/Blueprints/TSICharacterMaxParentClassEB.TSICharacterMaxParentClassEB_C|GetTeamNum _asbp_ebworker_char_max_parent))
              (return _asbp_ebairtscontroller_opponent))))))))

(fn SpawnGroupOfCopsforCrime
  (params (Location :type Vector))
  (return 0))

(fn SpawnCopandReturnIt
  (return 0))

(fn UTILSGetClosestActorAmongstAcfrstoActor
  (params (ActorChecking :type Actor%20Object%20Reference) (ActiorsToCheckWhoClosest :type Array%20of%20Actor%20Object%20References))
  ;[0.2718 1 0.07684] Get the smallest distance between a bunch of actors
  (for _array_element ActiorsToCheckWhoClosest
    (if (< (Transformation|GetDistanceTo _array_element ActorChecking) (LocalVariables|GetKingDistance))
      (if (!= _array_element ActorChecking)
        (LocalVariables|SetActorKingOfHill _array_element)
        (LocalVariables|SetKingDistance (Transformation|GetDistanceTo _array_element ActorChecking)))))
  (return (LocalVariables|GetActorKingOfHill)))

(fn WIPGetNameConvertReferencetoName
  (params (ControllerOrActor :type Actor%20Object%20Reference))
  (return ""))

(fn RTSConsiderifThisOilPumpIsConqueredAlready
  (params (OilResourceChecking :type BP%20Oil%20Well%20Sphere%20Resource%20Object%20Reference))
  (return false))

(fn RTSDoesGetCaughtDoingCrime
  (return false 0 0 "0, 0, 0"))

(fn RTSGetAllAIorPlayerConstructioninProgressProcess
  (params (ConstructionClass :type BP%20Construction%20in%20Process%20Max%20Parent%20Class%20Class%20Reference))
  (return 0))

(fn RTSGetAllBuildingsbyTypeOfThisPlayerORAI
  (params (BuildingType :type BP%20Building%20Max%20Parent%20Class%20Class%20Reference))
  (return 0))

(fn RTSGetAllBuildingsOfThisAIorPlayerInterorAI
  (return 0))

(fn RTSGetAllMapResources
  (return 0))

(fn RTSGetAllOilRigsOfThisAIorPlayerInterDEPRA
  (return 0))

(fn RTSGetAllSoldiersOfThisAIorPlayerInter
  (return 0))

(fn RTSGetAllUnitsOfThisAIorPlayerInter
  (return 0))

(fn RTSGetAllUnitsOfTypeforAIandPlayer
  (params (ActorType :type Actor%20Class%20Reference))
  (return 0))

(fn RTSGetAllWorkersOfThisAIorPlayerInter
  (return 0))

(fn RTSGetClosestOilWelltoAIorPlayertoConquerInter
  (return 0))

(fn RTSGetMoneyAmount
  (return 0))

(fn RTSHasAnyIdleWorkers
  (return 0))

(fn RTSHasEnoughCertainAmountMoney
  (params (MoneyToSpend :type Integer))
  (return false))

(fn RTSIsWorkerorActorBusy
  (return false))

(fn RTSRecruitUnitbyType
  (params (UnitClassType :type Actor%20Class%20Reference))
  (return 0))