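; BP_EBGameMaxPar is the core game-flow Blueprint for an RTS business game, running its calendar and setting up the AI opponent.
; A looping timer cascades day, week, month and year counters, and each month triggers wage payment on player controllers.
; BeginPlay collects spawners, creates an AI opponent on placeholder team 4 and spawns its starting units at the first spawner.
; Message broadcasting logs only hard-coded debug text; win/lose events are empty stubs.
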(event Custom|GOAL_LooseGame
  ;[1 1 1] When oponent reached the saved goal wins
)

(event Custom|GOAL_WinGame
  ;[1 1 1] When reached the saved goal wins
)

(event Custom|StartBroadcastingToWorldMessage
  (params (Message :type String) (bDoHaveOwner :type Boolean) (BussinesManSendingMessage :type Controller%20Object%20Reference))
  (CallFunction|ServerSendtoAllClientsMessage Message BussinesManSendingMessage bDoHaveOwner)
  (Development|PrintString "FROM EBGameMaxHello"))

(event Custom|ServerSendToAllClientsMessage
  (params (Message :type String) (BussinesManSendingMessage :type Controller%20Object%20Reference) (bHasOwner :type Boolean))
  (bind _outactors (Actor|GetAllActorsOfClass "/Game/EB/Blueprints/BP_PlayerControllerRTSMaxPar.BP_PlayerControllerRTSMaxPar_C"))
  (for _array_element _outactors
    (Default|CORELOGAddLogMessage _array_element "FROM EBGameMaxPar" 1e+01 (Utilities|Struct|MakeSlateColor "(R=0.000000,G=0.215381,B=1.000000,A=1.000000)"))
    (Development|PrintString "FROM EBGame iterating")))

(event Custom|ClientSendMessage
  (params (Message :type String) (Bussiness%20Message :type Controller%20Object%20Reference) (bHasOwner :type Boolean)))

(event EventBeginPlay
  (bind _returnvalue (Utilities|Time|SetTimerbyFunctionName 0 "dayPassedTimerBased" (Variables|Default|GetTimeADayIs) true))
  (Variables|Default|SetDayPassedHAndle _returnvalue)
  (CallFunction|RecollectSpawners)
  (bind _aiopponent (CallFunction|HandleSpawnAIsGeneralControllerFoeAI))
  (CallFunction|HandleSpawningBots _aiopponent)
  (Default|PostBeginPlayBegintheBussinesLife _aiopponent))

(event EventTick
  (params (DeltaSeconds :type Float%20%28single-precision%29)))

(fn ConstructionScript
  (|CallParentFunction))

(fn DayPassedTimerBased
  (bind _output_get (Variables|Default|SetTotalDaysForAWeekPassed (+ (Variables|Default|GetTotalDaysForAWeekPassed) 1)))
  (if (== _output_get 7)
    (CallFunction|WeekHasPassed)))

(fn WeekHasPassed
  (Variables|Default|SetTotalDaysForAWeekPassed 0)
  (bind _output_get (Variables|Default|SetTotalWeeksForAMonthHasPassed (+ (Variables|Default|GetTotalWeeksForAMonthHasPassed) 1)))
  (if (== _output_get 4)
    (CallFunction|MonthHasPassed)))

(fn MonthHasPassed
  (bind _outactors (Actor|GetAllActorsOfClass "/Script/Engine.PlayerController"))
  (for _array_element _outactors
    (bind _asbp_player_controller_rtsmax_par (Utilities|Casting|CastToBP_PlayerControllerRTSMaxPar _array_element))
    (Default|STRATEGYPayWages _asbp_player_controller_rtsmax_par))
  (Variables|Default|SetTotalWeeksForAMonthHasPassed 0)
  (bind _output_get (Variables|Default|SetTotalMonthForAYearHasPassed (+ (Variables|Default|GetTotalMonthForAYearHasPassed) 1)))
  (if (== _output_get 12)
    (CallFunction|YearHasPassed)))

(fn YearHasPassed
  (Variables|Default|SetTotalMonthForAYearHasPassed 0))

(fn RecollectSpawners
  ;[1 1 1] References the spawners and all of that
  (bind _outactors (Actor|GetAllActorsOfClass "/Game/EB/Blueprints/BP_SpawnerOfOpponentOrPlayer.BP_SpawnerOfOpponentOrPlayer_C"))
  (for _array_element _outactors
    (Utilities|Array|Add (Variables|Default|GetSpawners) _array_element)))

(fn HandleSpawningBots
  (params (ControllerSpawning :type Controller%20Object%20Reference))
  (Default|SpawnOpponentsStuff (Utilities|Array|Get(acopy) (Variables|Default|GetSpawners)) "NewEnumerator0" 4 ControllerSpawning))

(fn HandleSpawnAIsGeneralControllerFoeAI
  ;[1 1 1] Spawns a AI controller then reference the workers in such controller
  (bind _returnvalue (Game|SpawnActorfromClass "/Game/EB/Blueprints/BP_EBAIOpponent.BP_EBAIOpponent_C" (Math|Transform|MakeTransform "0, 0, 0") "Undefined" 0 0))
  ;[1 1 1] 4 as place holder should count the other Controllers
  (Variables|/Game/EB/Blueprints/BP_EBAIOpponent.BP_EBAIOpponent_C|SetTeamNumAIOponent _returnvalue 4)
  (return _returnvalue))