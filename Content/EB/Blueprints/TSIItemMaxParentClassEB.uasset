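; Base class for TSI items that characters pick up into an inventory and equip.
; Pickup adds the item to the pawn's inventory and sets Picked, whose RepNotify toggles mesh visibility and collision.
; Equip passes the item's skeletal mesh to the owning TSI character's attachment variable.
; Fire, unequip and primary-weapon notify are empty stubs, and the owner-test client event and server function call each other.
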(event Custom|ClientOwnertellWhoOwnerIs
  (CallFunction|ServerClientsWhoOwnerIs))

(event EventBeginPlay)

(event Collision|EventActorBeginOverlap
  (params (OtherActor :type Actor%20Object%20Reference)))

(event EventTick
  (params (DeltaSeconds :type Float%20%28single-precision%29)))

(fn ConstructionScript)

(fn StartFire
  (params (FireModeNum :type Byte)))

(fn StopFire
  (params (FireModeNum :type Byte)))

(fn ItemGetPicked
  (params (PawnPicking :type TSI%20Character%20Max%20Parent%20Class%20EB%20Object%20Reference))
  (Default|AddIteminInventory (Variables|/Game/EB/Blueprints/TSICharacterMaxParentClassEB.TSICharacterMaxParentClassEB_C|GetInventoryReference PawnPicking) self)
  (Variables|ItemProps|SetbPicked true))

(fn ItemEquip
  ;[1 1 1] For equipping this make it so the actual skel mesh changes, also check through a log if function is reached
  (bind _astsicharacter_max_parent_class_eb (Utilities|Casting|CastToTSICharacterMaxParentClassEB (Components|GetOwner)))
  (Variables|/Game/EB/Blueprints/TSICharacterMaxParentClassEB.TSICharacterMaxParentClassEB_C|SetRepAclSkeletalMAttachRA _astsicharacter_max_parent_class_eb (Variables|ItemProps|GetSkeletalMeshForEquiping)))

(fn ItemUnEquip)

(fn OnRepBPicked
  (if (Math|Boolean|Equal(Boolean) (Variables|ItemProps|GetbPicked) true)
    (Rendering|SetVisibility (Variables|Default|GetItemStaMesh) false false)
    (Collision|SetActorEnableCollision false)
    (else
      (Rendering|SetVisibility (Variables|Default|GetItemStaMesh) true false)
      (Collision|SetActorEnableCollision true))))

(fn GetCastPOwnerTSI
  (bind _astsicharacter_max_parent_class_eb (Utilities|Casting|CastToTSICharacterMaxParentClassEB (Components|GetOwner)))
  (return _astsicharacter_max_parent_class_eb))

(fn ServerClientsWhoOwnerIs
  ;[1 1 1] To Make tests about who owner is of this item to make sure things.
  (Networking|SwitchHasAuthority
    (:Authority
      (CallFunction|ClientOwnertellWhoOwnerIs))))

(fn OnRepBSettoPrimaryWeapon)