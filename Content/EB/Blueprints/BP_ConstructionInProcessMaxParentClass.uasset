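; Base RTS construction site that stands in for a building until it is finished.
; An overlapping worker's AI controller is told to build it, while Tick mirrors ProcessPercent onto a widget progress bar.
; GetFinished spawns the finished archetype at its transform, registers it with the player or AI opponent controller, then destroys the site.
; SetOwnerServer assigns ownership and adds the site to the player controller's owned actors.
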(event Custom|SetOwnerServer
  (params (Owner :type Controller%20Object%20Reference))
  (Development|PrintString "FROM BP Construciton in progress setting owner TIER0" true true "(R=0.109645,G=0.000000,B=1.000000,A=1.000000)" 1e+01)
  (Actor|SetOwner Owner)
  (Development|PrintString (Utilities|String|Append "FROM BP Construciton in progress setting owner  TIER0.5" (Utilities|GetDisplayName Owner)) true true "(R=0.109645,G=0.000000,B=1.000000,A=1.000000)" 1e+01)
  (bind _asbp_player_controller_rtsmax_par (Utilities|Casting|CastToBP_PlayerControllerRTSMaxPar Owner))
  (Default|STRATEGYAddActortoOwnedActors _asbp_player_controller_rtsmax_par self)
  (Development|PrintString "FROM BP Construciton in progress setting owner TIER 2r" true true "(R=0.109645,G=0.000000,B=1.000000,A=1.000000)" 1e+01))

(event EventBeginPlay)

(event Collision|EventActorBeginOverlap
  (params (OtherActor :type Actor%20Object%20Reference))
  (bind _asbp_ebworker (Utilities|Casting|CastToBP_EBWorker OtherActor))
  (Utilities|IsValid _asbp_ebworker
    (:Is%20Valid
      (bind _asbp_ebaicontroller_max_parent_class (Utilities|Casting|CastToBP_EBAIControllerMaxParentClass (Pawn|GetController _asbp_ebworker)))
      (Default|AIBuildAConstruction _asbp_ebaicontroller_max_parent_class self))))

(event EventTick
  (params (DeltaSeconds :type Float%20%28single-precision%29))
  (bind _asuw_construction_progress (Utilities|Casting|CastToUW_ConstructionProgress (UserInterface|GetUserWidgetObject (Variables|Default|GetWidget))))
  (Progress|SetPercent (Variables|/Game/EB/Blueprints/UW_ConstructionProgress.UW_ConstructionProgress_C|GetConstructionProcessBar _asuw_construction_progress) (/ (Math|Conversions|ToFloat(Integer) (Variables|Default|GetProcessPercent)) 1e+02)))

(fn ConstructionScript)

(fn GetFinished
  (params (WorkerFinishingBuilding :type BP%20EB%20Char%20Max%20Parent%20Object%20Reference) (ControllerFinishing :type Controller%20Object%20Reference))
  (bind _self self)
  (bind _returnvalue (Transformation|GetActorTransform _self))
  (Development|PrintString (Utilities|String|Append "FROM BP construction the contorlller finishing is" (Utilities|GetDisplayName ControllerFinishing) "the worker is" (Utilities|GetDisplayName WorkerFinishingBuilding)))
  (bind _returnvalue_2 (Game|SpawnActorfromClass (Variables|Default|GetConstructionArchetypeWhenDone) (Math|Transform|MakeTransform (+ (.location _returnvalue) "0, 0, 0") (.rotation _returnvalue) (.scale _returnvalue)) "AlwaysSpawn" ControllerFinishing 0))
  (Utilities|FlowControl|Sequence
    (:then_0
      ;[1 1 1] AI
      (bind _asbp_player_controller_rtsmax_par (Utilities|Casting|CastToBP_PlayerControllerRTSMaxPar ControllerFinishing))
      (Utilities|Array|Add (Variables|/Game/EB/Blueprints/BP_PlayerControllerRTSMaxPar.BP_PlayerControllerRTSMaxPar_C|GetAllActorsOfThisPlayerController _asbp_player_controller_rtsmax_par) _returnvalue_2)
      (CallFunction|HandleDestroySelfDoThatIsFinished :!label _label))
    (:then_1
      (bind _asbp_ebaiopponent (Utilities|Casting|CastToBP_EBAIOpponent ControllerFinishing))
      (Utilities|Array|Add (Variables|/Game/EB/Blueprints/BP_EBAIOpponent.BP_EBAIOpponent_C|GetAllActorsOfThisController _asbp_ebaiopponent) _returnvalue_2)
      (Utilities|Array|Add (Variables|/Game/EB/Blueprints/BP_EBAIOpponent.BP_EBAIOpponent_C|GetOwnedConstructions _asbp_ebaiopponent) _returnvalue_2)
      (Development|PrintString (Utilities|String|Append "FROM ConstructionProgress the builder is" (Utilities|GetDisplayName ControllerFinishing)))
      (goto _label))
    (:then_2
      (goto _label))
    (:then_3
      (CallFunction|SetOwnerServer ControllerFinishing))))

(fn HandleDestroySelfDoThatIsFinished
  (bind _self self)
  (Utilities|IsValid _self
    (:Is%20Valid
      (Actor|DestroyActor _self)
      (Utilities|Platform|CollectGarbage))))