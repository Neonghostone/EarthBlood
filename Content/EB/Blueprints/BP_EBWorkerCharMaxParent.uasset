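; Parent worker character for an RTS, handling selection by its owning player controller, right-click movement, construction and oil prospecting.
; Looping timers by function name add build progress until completion or replay work montages.
; Oil search waits, line-traces straight down for oil well spheres, then resets the AI controller and animation states.
; Oil spot spawning and the nearby-spot check are stubs, and the move toward assigned buildings is disconnected.
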(event Custom|StartFindingOil
  (params (PlaceToStart :type Vector))
  (bind (_x _y) (Math|Vector|BreakVector PlaceToStart))
  (bind _returnvalue (Pawn|GetController))
  (CallFunction|WorkerGotoState "NewEnumerator4")
  (Utilities|FlowControl|Delay (Variables|Default|GetFIndOilTime))
  (Variables|Default|SetbFoundOilTrace false)
  (bind _outhits (Class|KismetSystemLibrary|LineTraceMultiforObjects PlaceToStart (Math|Vector|MakeVector _x _y -1e+05) (Utilities|Array|MakeArray "ObjectTypeQuery1" "ObjectTypeQuery2") false 0 "ForDuration" true "(R=1.000000,G=0.000000,B=0.000000,A=1.000000)" "(R=0.000000,G=1.000000,B=0.000000,A=1.000000)" 2e+01))
  (for _array_element _outhits
    (Utilities|Casting|CastToBP_OilWellSphereResource (.HitActor (Collision|BreakHitResult _array_element)))
    (Development|PrintString "FFROM eb MAX Charyuo found oil!!! " true true "(R=0.000000,G=1.000000,B=0.069157,A=1.000000)")
    (Variables|Default|SetbFoundOilTrace true)
    ;[1 1 1] REDUNDANCY HERE, KEEP THE ANIMATION STATE AT THE PAWN OR RENAME EM
    (CallFunction|WorkerGotoState "NewEnumerator0")
    (CallFunction|SpaWNPlaceOilSpot)
    (bind _asbp_ebaicontroller_max_parent_class (Utilities|Casting|CastToBP_EBAIControllerMaxParentClass _returnvalue))
    (Default|GotoStateAIWokerorWhataver _asbp_ebaicontroller_max_parent_class "NewEnumerator0" "NewEnumerator4")
    (CallFunction|WorkerGotoState "NewEnumerator0"))
  (if (not (Variables|Default|GetbFoundOilTrace))
    (Development|PrintString "FFROM eb MAX Char you did not find oil" true true "(R=1.000000,G=0.008583,B=0.000000,A=1.000000)")
    (bind _asbp_ebaicontroller_max_parent_class_2 (Utilities|Casting|CastToBP_EBAIControllerMaxParentClass _returnvalue))
    (Default|GotoStateAIWokerorWhataver _asbp_ebaicontroller_max_parent_class_2 "NewEnumerator0" "NewEnumerator4")
    (CallFunction|WorkerGotoState "NewEnumerator0")))

(event Custom|SpawnPlaceOilSpot)

(event EventBeginPlay
  (|CallParentFunction))

(event Collision|EventActorBeginOverlap
  (params (OtherActor :type Actor%20Object%20Reference)))

(event EventTick
  (params (DeltaSeconds :type Float%20%28single-precision%29))
  (|CallParentFunction DeltaSeconds))

(event EventRTSInterfunctHandleRightClickonLSorSMwithSelected
  (params (PlayerControllerUsing :type Player%20Controller%20Object%20Reference) (PlaceOnMap :type Vector :default "0, 0, 0"))
  (bind _returnvalue (Pawn|GetController))
  (if (Utilities|IsValid _returnvalue)
    (AI|Navigation|SimpleMovetoLocation _returnvalue PlaceOnMap)))

(event EventRTSInterfunctUnitGetSelected
  (params (ControllerClicking :type Player%20Controller%20Object%20Reference))
  (bind _asbp_player_controller_rtsmax_par (Utilities|Casting|CastToBP_PlayerControllerRTSMaxPar ControllerClicking))
  (bind _isactoroneofitsactors (Default|STRATEGYIsThisActorOneOfItsActors _asbp_player_controller_rtsmax_par self))
  (if _isactoroneofitsactors
    (Utilities|Array|Add (Variables|/Game/EB/Blueprints/BP_PlayerControllerRTSMaxPar.BP_PlayerControllerRTSMaxPar_C|GetAllActorsSelected _asbp_player_controller_rtsmax_par) self)))

(event EventRTSInterfunctUnitGetDeselected
  (params (ControllerUnselecting :type Player%20Controller%20Object%20Reference))
  (bind _asbp_player_controller_rtsmax_par (Utilities|Casting|CastToBP_PlayerControllerRTSMaxPar ControllerUnselecting))
  (bind _isactoroneofitsactors (Default|STRATEGYIsThisActorOneOfItsActors _asbp_player_controller_rtsmax_par self))
  (if _isactoroneofitsactors
    (if (not (< (Utilities|Array|FindItem (Variables|/Game/EB/Blueprints/BP_PlayerControllerRTSMaxPar.BP_PlayerControllerRTSMaxPar_C|GetAllActorsSelected _asbp_player_controller_rtsmax_par) self) 0))
      (Utilities|Array|RemoveItem (Variables|/Game/EB/Blueprints/BP_PlayerControllerRTSMaxPar.BP_PlayerControllerRTSMaxPar_C|GetAllActorsSelected _asbp_player_controller_rtsmax_par) self))))

(fn ConstructionScript
  (|CallParentFunction))

(fn WorkerBuildStructureDoOnce
  (bind _actualconstructiongettingconstructed (Variables|Default|GetActualConstructionGettingConstructed))
  (Utilities|IsValid _actualconstructiongettingconstructed
    (:Is%20Valid
      (Variables|/Game/EB/Blueprints/BP_ConstructionInProcessMaxParentClass.BP_ConstructionInProcessMaxParentClass_C|SetProcessPercent _actualconstructiongettingconstructed (+ (Variables|/Game/EB/Blueprints/BP_ConstructionInProcessMaxParentClass.BP_ConstructionInProcessMaxParentClass_C|GetProcessPercent _actualconstructiongettingconstructed) 26))
      (if (>= (Variables|/Game/EB/Blueprints/BP_ConstructionInProcessMaxParentClass.BP_ConstructionInProcessMaxParentClass_C|GetProcessPercent _actualconstructiongettingconstructed) 100)
        (Variables|/Game/EB/Blueprints/BP_ConstructionInProcessMaxParentClass.BP_ConstructionInProcessMaxParentClass_C|SetProcessPercent _actualconstructiongettingconstructed 100)
        (CallFunction|FinishConstruction _actualconstructiongettingconstructed)
        (Utilities|Time|ClearandInvalidateTimerbyHandle (Variables|Default|GetContructionHandle))
        (else
          (CallFunction|StartPlayingAnimation "/Game/EB/Animations/AM_WorkingOrBuildingABuilding.AM_WorkingOrBuildingABuilding"))))
    (:Is%20Not%20Valid
      (CallFunction|StopWorkingonBuilding))))

(fn StartBuildingConstruction
  (params (ConstructionProcessing :type BP%20Construction%20in%20Process%20Max%20Parent%20Class%20Object%20Reference))
  (Variables|Default|SetActualConstructionGettingConstructed ConstructionProcessing)
  (bind _returnvalue (Utilities|Time|SetTimerbyFunctionName 0 "WorkerBuildStructureDoOnce" 1.0 true))
  (Variables|Default|SetContructionHandle _returnvalue))

(fn FinishConstruction
  (params (ConstructionInProcess :type BP%20Construction%20in%20Process%20Max%20Parent%20Class%20Object%20Reference))
  (bind _self self)
  (bind _ascontroller (Utilities|Casting|CastToController (Components|GetOwner _self))
    (:then
      (Default|GetFinished ConstructionInProcess (Utilities|Array|MakeArray _self) _ascontroller))
    (:CastFailed
      (Development|PrintString "FROM Worker error no controller"))))

(fn StartWorkingonBuilding
  (params (BuildingWorkingAt :type BP%20Building%20Max%20Parent%20Class%20Object%20Reference))
  (bind _returnvalue (Utilities|Time|SetTimerbyFunctionName 0 "WorkerWorkOnBuildingDoOnce" 1.0 true))
  (Variables|Default|SetWorkingAtHandle _returnvalue)
  (Variables|Default|SetActualBuildingWorkingAt 0)
  (bind _asbp_ebaicontroller_max_parent_class (Utilities|Casting|CastToBP_EBAIControllerMaxParentClass (Pawn|GetController)))
  (Default|AIWorkonAConstruction _asbp_ebaicontroller_max_parent_class))

(fn WorkerWorkonBuildingDoOnce
  (CallFunction|StartPlayingAnimation "/Game/EB/Animations/AM_WorkingAtBuilding.AM_WorkingAtBuilding"))

(fn StartGettingClosetoWorkonBuilding
  (params (Building :type BP%20Building%20Max%20Parent%20Class%20Object%20Reference))
  ;[1 1 1] Should be before moving but it's cool
  (CallFunction|SetBuildingSenttoWorkAssigned Building))

(fn StopWorkingonBuilding
  (params (ConstructionProcessing :type BP%20Building%20Max%20Parent%20Class%20Object%20Reference))
  (Variables|Default|SetActualBuildingWorkingAt 0)
  (Utilities|Time|ClearandInvalidateTimerbyHandle (Variables|Default|GetWorkingAtHandle)))

(fn SetBuildingSenttoWorkAssigned
  (params (BtoGetToWork :type Actor%20Object%20Reference))
  (Variables|Default|SetBuildingSentToWorkAtAssigned BtoGetToWork))

(fn WorkerGotoState
  (params (NewWorkerState :type EN_StateOfWorker%20Enum :default "NewEnumerator0"))
  (Variables|Default|SetStateOfWorkerForAnims NewWorkerState))

(fn IsThereOilSpotNear
  ;[1 1 1] Check if there are oil spots so if there are do not find more oil
  (return false))