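; Oil pump building for the RTS that earns its owning player or AI opponent money every second, scaled by working worker count.
; A looping timer runs GainOil regardless of whether oil was found.
; Rushes roll against a success chance: success grants extra payouts or advances the deprecated random oil search, while failure damages assigned workers.
; Also creates rush and recruiting widgets and draws search progress when debugging.
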(event Custom|StartSpawningrushWidgetWorking
  (bind _returnvalue (Game|GetPlayerController 0))
  ;[1 1 1] rush widget does not reach to multicast or anything but left it like this
  (bind _asbp_hudmax_parent_class (Utilities|Casting|CastToBP_HUDMaxParentClass (HUD|GetHUD _returnvalue)))
  ;[1 1 1] ASSIGN ON HUD IT DOES NOT TELL BUT ITS OVERRIDEN
  (bind _returnvalue_2 (UserInterface|CreateWidget "/Game/EB/Blueprints/UW_WorkingBuildingWidget.UW_WorkingBuildingWidget_C" _returnvalue))
  (UserInterface|Viewport|AddtoViewport _returnvalue_2 0)
  (bind _returnvalue_3 (UserInterface|CreateWidget "/Game/EB/Blueprints/UW_AdminHutRecruitingHUd.UW_AdminHutRecruitingHUD_C" _returnvalue))
  (Variables|/Game/EB/Blueprints/BP_HUDMaxParentClass.BP_HUDMaxParentClass_C|SetHUD_Admin2RecruitingHUD _asbp_hudmax_parent_class _returnvalue_3)
  (UserInterface|Viewport|AddtoViewport _returnvalue_3 0)
  (Variables|/Game/EB/Blueprints/BP_HUDMaxParentClass.BP_HUDMaxParentClass_C|SetHUD_WorkingRushWidget _asbp_hudmax_parent_class _returnvalue_2))

(event Custom|FinishOilProcessFoundOil
  (if (not (Variables|Default|GetbOilWasFound))
    (Networking|SwitchHasAuthority
      (:Authority
        (bind _asbp_player_controller_rtsmax_par (Utilities|Casting|CastToBP_PlayerControllerRTSMaxPar (Game|GetPlayerController 0)))
        (bind _asbp_hudmax_parent_class (Utilities|Casting|CastToBP_HUDMaxParentClass (HUD|GetHUD _asbp_player_controller_rtsmax_par)))
        (Default|HUDLOGAddLogMessage _asbp_hudmax_parent_class "YOU HAVE FOUND OIL!" 1e+01 (Utilities|Struct|MakeSlateColor "(R=0.000000,G=1.000000,B=0.101791,A=1.000000)"))
        (Variables|Default|SetbOilWasFound true)))))

(event Custom|FindOilProcess
  ;[1 1 1] Depra
  (Networking|SwitchHasAuthority
    (:Authority
      (bind _asbp_player_controller_rtsmax_par (Utilities|Casting|CastToBP_PlayerControllerRTSMaxPar (Game|GetPlayerController 0)))
      (for _array_element (Variables|Default|GetAssignedWorkersDEPRA)
        (bind _output_get (Variables|Default|SetPercentageOfFindOil (Math|Conversions|ToByte(Integer) (Math|Integer|Clamp(Integer) (Math|Conversions|ToInteger(Byte) (+ (Variables|Default|GetPercentageOfFindOil) (Math|Conversions|ToByte(Integer) (Math|Random|RandomInteger 4)))) 0 100))))
        (bind _asbp_hudmax_parent_class (Utilities|Casting|CastToBP_HUDMaxParentClass (HUD|GetHUD _asbp_player_controller_rtsmax_par)))
        (if (>= _output_get 100)
          (CallFunction|FinishOilProcessFoundOil)
          (else
            (Default|HUDLOGAddLogMessage _asbp_hudmax_parent_class (Utilities|String|Append "Search PRGS" "" "= " (Utilities|String|ToString(Byte) (Variables|Default|GetPercentageOfFindOil)) "%") 2.0 (Utilities|Struct|MakeSlateColor "(R=0.000000,G=0.000000,B=0.000000,A=1.000000)"))))))))

(event EventBeginPlay
  (Utilities|Time|SetTimerbyFunctionName 0 "GainOil" 1.0 true)
  (|CallParentFunction))

(event Collision|EventActorBeginOverlap
  (params (OtherActor :type Actor%20Object%20Reference))
  (|CallParentFunction OtherActor) ; This node is disabled and will not be called.\nDrag off pins to build functionality.
)

(event EventTick
  (params (DeltaSeconds :type Float%20%28single-precision%29))
  (bind _asbp_player_controller_rtsmax_par (Utilities|Casting|CastToBP_PlayerControllerRTSMaxPar (Game|GetPlayerController 0)))
  (if (Variables|/Game/EB/Blueprints/BP_PlayerControllerRTSMaxPar.BP_PlayerControllerRTSMaxPar_C|GetbSeeDebuggingInfo _asbp_player_controller_rtsmax_par)
    (Rendering|Debug|DrawDebugString (Transformation|GetActorLocation) (Utilities|String|Append " FROM rig Find = " (Utilities|String|ToString(Byte) (Variables|Default|GetPercentageOfFindOil))) 0 "(R=1.000000,G=0.917422,B=0.000000,A=1.000000)")
    (|CallParentFunction DeltaSeconds)))

(event EventHUDSpawnCorrespondingHUD)

(event EventStarttheRush
  (|CallParentFunction))

(event EventServerDoRush
  (|CallParentFunction))

(event EventEndRushResults
  (if (not (>= (Math|Random|RandomInteger 100) (Math|Conversions|ToInteger(Byte) (CallFunction|RUSHReturnPercentageOfSuccesOfRush))))
    (CallFunction|EndRushSuccesful)
    (else
      (CallFunction|EndRushFailure))))

(event EventEndRushFailure
  ;[1 1 1] Rush Failure Kill some workers
  (Utilities|FlowControl|Sequence
    (:then_0
      (Audio|PlaySound2D "/Game/EB/Audio/Sounds/Ambulance1.Ambulance1" 1.0 1.0 0.0 0 0))
    (:then_1
      (Utilities|Casting|CastToBP_PlayerControllerRTSMaxPar (Components|GetOwner))
      (bind _asbp_rtsgame_mode_tmplt (Utilities|Casting|CastToBP_RTSGameModeTmplt (Game|GetGameMode)))
      (Default|BroadcastMessageDependingtoWho _asbp_rtsgame_mode_tmplt 0 true 0 "Rush has failed" "None" false false "(R=0.000000,G=0.000000,B=0.000000,A=1.000000)" false))
    (:then_2
      (for _array_element (Variables|Default|GetAssignedWorkersDEPRA)
        (Default|EBTakeDamage _array_element 50)))))

(event EventEndRushSuccesful
  ;[1 1 1] Rush succes do find more oil and get more oil
  (Utilities|FlowControl|Sequence
    (:then_0
      (Audio|PlaySound2D "/Game/TSIBPTSICntnt/TSIAudio/FireArmSounds/AK_47.AK_47" 1.0 1.0 0.0 0 0))
    (:then_1
      (if (Variables|Default|GetbOilWasFound)
        (CallFunction|GainOil)
        (CallFunction|GainOil)
        (else
          (CallFunction|FindOilProcess)
          (CallFunction|FindOilProcess)
          (CallFunction|FindOilProcess)
          (CallFunction|FindOilProcess)
          (bind _asbp_rtsgame_mode_tmplt (Utilities|Casting|CastToBP_RTSGameModeTmplt (Game|GetGameMode)))
          (Default|BroadcastMessageDependingtoWho _asbp_rtsgame_mode_tmplt 0 true 0 "Rush unseccesful " "None" false false "(R=0.000000,G=0.000000,B=0.000000,A=1.000000)" false))))
    (:then_2
      (bind _astsiplayer_controller (Utilities|Casting|CastToTSIPlayerController (Game|GetPlayerController 0)))
      (bind _asbp_rtsgame_mode_tmplt_2 (Utilities|Casting|CastToBP_RTSGameModeTmplt (Game|GetGameMode)))
      (Default|BroadcastMessageDependingtoWho _asbp_rtsgame_mode_tmplt_2 0 true 0 "Rush  succesful" "None" false false "(R=0.000000,G=0.000000,B=0.000000,A=1.000000)" false))))

(fn ConstructionScript
  (|CallParentFunction))

(fn GainOil
  (bind _workercountworking (CallFunction|STRATEGYCountWokersontheBuildingWorking))
  (bind _returnvalue (Components|GetOwner))
  (bind _workercountworking_2 (CallFunction|STRATEGYCountWokersontheBuildingWorking))
  (bind _returnvalue_2 (* _workercountworking_2 50))
  (bind _returnvalue_3 (* _workercountworking 50))
  (bind _asbp_player_controller_rtsmax_par (Utilities|Casting|CastToBP_PlayerControllerRTSMaxPar _returnvalue))
  (bind _asbp_ebaiopponent (Utilities|Casting|CastToBP_EBAIOpponent _returnvalue))
  (Utilities|IsValid _returnvalue
    (:Is%20Valid
      (Utilities|FlowControl|Sequence
        (:then_0
          (Utilities|IsValid _asbp_player_controller_rtsmax_par
            (:Is%20Valid
              (Default|RTSRPGSetMoney _asbp_player_controller_rtsmax_par (+ (Variables|/Game/EB/Blueprints/BP_PlayerControllerRTSMaxPar.BP_PlayerControllerRTSMaxPar_C|GetRPGMoney _asbp_player_controller_rtsmax_par) _returnvalue_3) _returnvalue_3))))
        (:then_1
          (Utilities|IsValid _asbp_ebaiopponent
            (:Is%20Valid
              (Default|RTSRPGSetMoney _asbp_ebaiopponent (+ (Variables|/Game/EB/Blueprints/BP_EBAIControllerMaxParentClass.BP_EBAIControllerMaxParentClass_C|GetAIOPONENT_RPGMoney _asbp_ebaiopponent) _returnvalue_2) _returnvalue_2))))))))