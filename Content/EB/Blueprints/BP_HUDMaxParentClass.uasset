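; RTS parent HUD that draws markers on selected units and buildings, a drag-selection rectangle and a listen server/client label.
; DrawHUD reads selection from the RTS player controller; mouse press/release opens and closes a gate that draws the marquee and stores a normalized Box2D.
; BeginPlay creates main, construction and recruiting widgets on authority.
; Helpers toggle widgets, clear them and post timed, colored log messages.
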(event Custom|HideResetAllWidgetryEvent
  (CallFunction|ClientHideWidgetry))

(event Custom|ClientHideWidgetry
  (bind _foundwidgets (Widget|GetAllWidgetsOfClass "/Script/UMG.UserWidget" true))
  (for _array_element _foundwidgets
    (Widget|RemovefromParent _array_element)))

(event Custom|LeftMouseReleased
  (bind _returnvalue (Game|Player|GetOwningPlayerController))
  (bind (_locationx _locationy) (Game|Player|GetMousePosition _returnvalue))
  (Utilities|FlowControl|Gate true) ; enters at Close
)

(event Custom|StopDrawingInPurpose
  (bind _returnvalue (Game|Player|GetOwningPlayerController))
  (bind (_locationx _locationy) (Game|Player|GetMousePosition _returnvalue))
  (Utilities|FlowControl|Gate true) ; enters at Close
)

(event Custom|LeftMousePressed
  (bind _returnvalue (Game|Player|GetOwningPlayerController))
  (bind _actualmousescreenlocation (Variables|Default|GetActualMouseScreenLocation))
  (bind (_locationx _locationy) (Game|Player|GetMousePosition _returnvalue))
  ;[1 1 1] Null the box
  (Variables|Default|SetCORE_2dBoxActualOrLastSelectionBoxCoordinates "")
  ;[1 1 1] Set it's initial position
  (Variables|Default|SetCORE_2dBoxActualOrLastSelectionBoxCoordinates (Math|Box2D|MakeBox2D _actualmousescreenlocation _actualmousescreenlocation))
  (Utilities|FlowControl|Gate true) ; enters at Open
)

(event EventBeginPlay
  ;[1 1 1] Spawn the widgets
  (Networking|SwitchHasAuthority
    (:Authority
      (bind _returnvalue (UserInterface|CreateWidget "/Game/EB/Blueprints/UW_GeneralHudWorkerBuild.UW_GeneralHudWorkerBuild_C"))
      (bind _output_get (Variables|Default|SetHUD_ConstructionWidget _returnvalue))
      (bind _returnvalue_2 (UserInterface|CreateWidget "/Game/EB/Blueprints/UW_GeneralHUDWidgetMainHud.UW_GeneralHUDWidgetMainHud_C"))
      (Variables|Default|SetHUD_MainHUDWidget _returnvalue_2)
      (UserInterface|Viewport|AddtoViewport (stale _returnvalue) 3)
      (Widget|SetVisibility _output_get "Hidden")
      (bind _returnvalue_3 (UserInterface|CreateWidget "/Game/RTSTemplateContent/Blueprints/HUDUIComponent/UW_GeneralHUDWidgetRecuriting.UW_GeneralHUDWidgetRecuriting_C"))
      (UserInterface|Viewport|AddtoViewport _returnvalue_3 5)
      (Widget|SetVisibility _returnvalue_3 "Hidden")
      (Variables|Default|SetHUD_MainHUDRecruiting _returnvalue_3))))

(event EventActorBeginOverlap
  (params (OtherActor :type Actor%20Object%20Reference))
  ;[1 1 1] Spawn the widgets
)

(event EventTick
  (params (DeltaSeconds :type Float%20%28single-precision%29))
  ;[1 1 1] Spawn the widgets
)

(event EventDrawHUD
  (params (SizeX :type Integer) (SizeY :type Integer))
  (bind _returnvalue (Game|Player|GetOwningPlayerController))
  (bind _returnvalue_2 (- 0.0 0.0))
  (bind _returnvalue_3 (Game|Player|GetOwningPlayerController))
  (bind _hud_cursorwidget (Variables|Default|GetHUD_CursorWidget))
  (bind (_locationx _locationy) (Game|Player|GetMousePosition _returnvalue))
  (bind (_locationx_2 _locationy_2) (Game|Player|GetMousePosition _returnvalue_3))
  (Utilities|FlowControl|Sequence
    (:then_0
      (bind _asbp_player_controller_rtsmax_par (Utilities|Casting|CastToBP_PlayerControllerRTSMaxPar (Game|Player|GetOwningPlayerController)))
      ;[1 1 1] For all actors in game, try render a box reprezsenting if they are selected or not
      (for _array_element (Variables|/Game/EB/Blueprints/BP_PlayerControllerRTSMaxPar.BP_PlayerControllerRTSMaxPar_C|GetAllActorsSelected _asbp_player_controller_rtsmax_par)
        (if (.ReturnValue (Class|GameplayStatics|ProjectWorldtoScreen (Game|Player|GetOwningPlayerController) (Transformation|GetActorLocation _array_element) false))
          (Utilities|Casting|CastToBP_TopDownCharacterMaxParentClass _array_element
            (:then
              (HUD|DrawRect "(R=0.053618,G=1.000000,B=0.000000,A=1.000000)" (.X (Math|Vector2D|BreakVector2D (.ScreenPosition (Class|GameplayStatics|ProjectWorldtoScreen (Game|Player|GetOwningPlayerController) (Transformation|GetActorLocation _array_element) false)))) (.Y (Math|Vector2D|BreakVector2D (.ScreenPosition (Class|GameplayStatics|ProjectWorldtoScreen (Game|Player|GetOwningPlayerController) (Transformation|GetActorLocation _array_element) false)))) 1e+01 1e+01 :!label _label)
              (HUD|DrawText (Utilities|String|ToString(Vector2d) (.ScreenPosition (Class|GameplayStatics|ProjectWorldtoScreen (Game|Player|GetOwningPlayerController) (Transformation|GetActorLocation _array_element) false))) "(R=0.000000,G=0.000000,B=0.000000,A=1.000000)" (.X (Math|Vector2D|BreakVector2D (.ScreenPosition (Class|GameplayStatics|ProjectWorldtoScreen (Game|Player|GetOwningPlayerController) (Transformation|GetActorLocation _array_element) false)))) (.Y (Math|Vector2D|BreakVector2D (.ScreenPosition (Class|GameplayStatics|ProjectWorldtoScreen (Game|Player|GetOwningPlayerController) (Transformation|GetActorLocation _array_element) false)))) 0 1.0 false))
            (:CastFailed
              (Utilities|Casting|CastToBP_BuildingMaxParentClass _array_element
                (:then
                  (HUD|DrawRect "(R=0.053618,G=1.000000,B=0.000000,A=1.000000)" (.X (Math|Vector2D|BreakVector2D (.ScreenPosition (Class|GameplayStatics|ProjectWorldtoScreen (Game|Player|GetOwningPlayerController) (Transformation|GetActorLocation _array_element) false)))) (.Y (Math|Vector2D|BreakVector2D (.ScreenPosition (Class|GameplayStatics|ProjectWorldtoScreen (Game|Player|GetOwningPlayerController) (Transformation|GetActorLocation _array_element) false)))) 2e+01 2e+01)
                  (HUD|DrawText "" "(R=0.000000,G=0.000000,B=0.000000,A=1.000000)" 0.0 0.0 0 1.0 false))
                (:CastFailed
                  (goto _label))))))))
    (:then_1
      (Variables|Default|SetActualMouseScreenLocation (Math|Vector2D|MakeVector2D _locationx_2 _locationy_2))
      (Utilities|FlowControl|Sequence
        (:then_0
          (Utilities|FlowControl|Gate true
            (:Exit
              ;[1 1 1] 2 Draw aselection rectangle i case we have our mosue click hold
              (bind _asbp_player_controller_rtsmax_par_2 (Utilities|Casting|CastToBP_PlayerControllerRTSMaxPar (Game|Player|GetOwningPlayerController)))
              (bind _output_get (Variables|Default|SetCORE_CONTROLS_ClickOnScreenXYNoZActualPosition (Math|Vector2D|MakeVector2D _locationx_2 _locationy_2)))
              ;;[1 1 1] THE LAST POSITION ON SCREEN
              (bind _output_get_2 (Variables|Default|SetCORE_CONTROLS_LastClickOnScreenXYNoZ (Variables|/Game/EB/Blueprints/BP_PlayerControllerRTSMaxPar.BP_PlayerControllerRTSMaxPar_C|GetLastClickMouseScreenLoc _asbp_player_controller_rtsmax_par_2)))
              ;;[1 1 1] JUST IN CASE WE WANT TO USE IT
              (bind _output_get_3 (Variables|Default|SetCORE_SelectionBoxSize (- _output_get _output_get_2)))
              ;;[1 1 1] Determinate the rigth sides of the box, to make it a consistent max and min box
              (bind _finalbox (CallFunction|COREGiveABoxOutOf22dVects (Variables|Default|GetCORE_CONTROLS_LastClickOnScreenXYNoZ) (Variables|Default|GetActualMouseScreenLocation)))
              (bind _output_get_4 (Variables|Default|SetCORE_2dBoxActualOrLastSelectionBoxCoordinates _finalbox))
              (HUD|DrawRect "(R=1.000000,G=0.215227,B=0.090660,A=1.000000)" (.X (Math|Vector2D|BreakVector2D _output_get_2)) (.Y (Math|Vector2D|BreakVector2D _output_get_2)) (.X (Math|Vector2D|BreakVector2D _output_get_3)) (.Y (Math|Vector2D|BreakVector2D _output_get_3))))))))
    (:then_2
      ;[1 1 1] Draw two boexes representing the sides
      (HUD|DrawRect "(R=0.000000,G=0.202881,B=1.000000,A=1.000000)" (.X (Math|Vector2D|BreakVector2D (.Min (Utilities|Struct|BreakBox2D (Variables|Default|GetCORE_2dBoxActualOrLastSelectionBoxCoordinates))))) (.Y (Math|Vector2D|BreakVector2D (.Min (Utilities|Struct|BreakBox2D (Variables|Default|GetCORE_2dBoxActualOrLastSelectionBoxCoordinates))))) 5.0 5.0)
      (HUD|DrawRect "(R=1.000000,G=0.000000,B=0.119738,A=1.000000)" (.X (Math|Vector2D|BreakVector2D (.Max (Utilities|Struct|BreakBox2D (Variables|Default|GetCORE_2dBoxActualOrLastSelectionBoxCoordinates))))) (.Y (Math|Vector2D|BreakVector2D (.Max (Utilities|Struct|BreakBox2D (Variables|Default|GetCORE_2dBoxActualOrLastSelectionBoxCoordinates))))) 5.0 5.0))
    (:then_3
      ;[1 1 1] Set the mouse position in the viewport
      (if (!= _hud_cursorwidget 0)
        (Class|UserWidget|SetPositioninViewport _hud_cursorwidget (Math|Vector2D|MakeVector2D _locationx _locationy) true)))
    (:then_4
      ;[1 1 1] Draw if we are server or not
      (if (Ability|HasAuthority (Game|Player|GetOwningPlayerController))
        (HUD|DrawText "Listen Server" "(R=1.000000,G=1.000000,B=1.000000,A=1.000000)" _returnvalue_2 8e+01 "/Engine/EngineFonts/RobotoDistanceField.RobotoDistanceField" 2.0 false)
        (else
          (HUD|DrawText "Client" "(R=1.000000,G=1.000000,B=1.000000,A=1.000000)" _returnvalue_2 8e+01 "/Engine/EngineFonts/RobotoDistanceField.RobotoDistanceField" 2.0 false))))))

(fn ConstructionScript)

(fn COREGiveABoxOutOf22dVects
  (params (FirstRectVect :type Vector%202D%20Structure) (SecondRectVect :type Vector%202D%20Structure))
  (bind (_x _y) (Math|Vector2D|BreakVector2D FirstRectVect))
  (bind (_x_2 _y_2) (Math|Vector2D|BreakVector2D SecondRectVect))
  ;[1 1 1] In order to get a normal box min and nomral box max , i nned to determinate the min and the max out of them
  (if (> _x _x_2)
    (LocalVariables|SetMaxX _x)
    (LocalVariables|SetMinX _x_2)
    (else
      (LocalVariables|SetMaxX _x_2)
      (LocalVariables|SetMinX _x)))
  (if (> _y _y_2)
    (LocalVariables|SetMaxY _y)
    (LocalVariables|SetMinY _y_2)
    (else
      (LocalVariables|SetMaxY _y_2)
      (LocalVariables|SetMinY _y)))
  (return (Math|Box2D|MakeBox2D (Math|Vector2D|MakeVector2D (LocalVariables|GetMinX) (LocalVariables|GetMinY)) (Math|Vector2D|MakeVector2D (LocalVariables|GetMaxX) (LocalVariables|GetMaxY)))))

(fn HUDSpawnConstructtheGeneralHUDWidget
  (bind _returnvalue (UserInterface|CreateWidget "/Game/EB/Blueprints/UW_GeneralHUDWidgetMainHud.UW_GeneralHUDWidgetMainHud_C"))
  (bind _output_get (Variables|Default|SetHUD_MainHUDWidget _returnvalue))
  (UserInterface|Viewport|AddtoViewport _output_get 0))

(fn HUDSpawnConstructtheConstructionTimeWidget)

(fn HUDSpawnConstructtheRecruitngTimeWidget
  (params (WidgetArchetype :type User%20Widget%20Class%20Reference))
  (bind _returnvalue (UserInterface|CreateWidget WidgetArchetype))
  (bind _output_get (Variables|Default|SetHUD_MainHUDRecruiting _returnvalue))
  (return _output_get))

(fn HUDShowElementbyNum
  (params (ElementNum :type EN_NumberOfElementHUD%20Enum :default "NewEnumerator0") (Hidden :type Boolean))
  (bind _hud_cursorwidget (Variables|Default|GetHUD_CursorWidget))
  (bind _hud_constructionwidget (Variables|Default|GetHUD_ConstructionWidget))
  (bind _hud_mainhudwidget (Variables|Default|GetHUD_MainHUDWidget))
  (bind _hud_mainhudrecruiting (Variables|Default|GetHUD_MainHUDRecruiting))
  (switch Utilities|FlowControl|Switch|SwitchonEN_NumberOfElementHUD ElementNum
    (:NewEnumerator0
      (if Hidden
        (Widget|SetVisibility _hud_cursorwidget "Hidden")
        (else
          (Widget|SetVisibility _hud_cursorwidget "Visible"))))
    (:NewEnumerator1
      (if Hidden
        (Widget|SetVisibility _hud_constructionwidget "Hidden")
        (else
          (Widget|SetVisibility _hud_constructionwidget "Visible"))))
    (:NewEnumerator2
      (if Hidden
        (Widget|SetVisibility _hud_mainhudwidget "Hidden")
        (else
          (Widget|SetVisibility _hud_mainhudwidget "Visible"))))
    (:NewEnumerator3
      (if Hidden
        (Widget|SetVisibility _hud_mainhudrecruiting "Hidden")
        (else
          (Widget|SetVisibility _hud_mainhudrecruiting "Visible"))))))

(fn HUDLOGAddLogMessage
  (params (NewLogMessage :type String) (Duration :type Float%20%28single-precision%29) (ColorOfLogMessage :type Slate%20Color%20Structure))
  (bind _specifiedcolor (Utilities|Struct|BreakSlateColor ColorOfLogMessage))
  (bind _hud_mainhudwidget (Variables|Default|GetHUD_MainHUDWidget))
  (bind (_r _g _b) (Utilities|Struct|BreakLinearColor _specifiedcolor))
  (Utilities|IsValid _hud_mainhudwidget
    (:Is%20Valid
      (bind _returnvalue (UserInterface|CreateWidget "/Game/EB/Blueprints/UW_LogMessage.UW_LogMessage_C"))
      (Utilities|IsValid _returnvalue
        (:Is%20Valid
          (Widget|Panel|AddChild (Variables|/Game/EB/Blueprints/UW_GeneralHUDWidgetMainHud.UW_GeneralHUDWidgetMainHud_C|GetLogSL _hud_mainhudwidget) _returnvalue)
          (Rendering|Components|TextRender|SetText (Variables|/Game/EB/Blueprints/UW_LogMessage.UW_LogMessage_C|GetLogMessageTxt _returnvalue) (Utilities|Text|ToText(String) NewLogMessage))
          (Default|HUDLOGSetTimertoRemove _returnvalue Duration)
          (Appearance|SetColorandOpacity (Variables|/Game/EB/Blueprints/UW_LogMessage.UW_LogMessage_C|GetLogMessageTxt _returnvalue) (Utilities|Struct|MakeSlateColor (Utilities|Struct|MakeLinearColor _r _g _b 1.0)) :!class /Script/UMG.TextBlock))))))

(fn HUDSpawnConstructionNWidget2
  (bind _returnvalue (UserInterface|CreateWidget "/Game/EB/Blueprints/UW_GeneralHudWorkerBuild.UW_GeneralHudWorkerBuild_C"))
  (bind _output_get (Variables|Default|SetHUD_ConstructionWidget2 _returnvalue))
  (UserInterface|Viewport|AddtoViewport _output_get 0)
  (bind _returnvalue_2 (UserInterface|CreateWidget "/Game/EB/Blueprints/UW_GeneralHUDWidgetMainHud.UW_GeneralHUDWidgetMainHud_C"))
  (UserInterface|Viewport|AddtoViewport _returnvalue_2 0)
  (Development|PrintString "FROM HUDMAX Spawning now the CW2"))