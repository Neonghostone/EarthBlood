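; BP_AdminHutConstruction is an RTS Admin Hut building actor that handles its own selection and HUD.
; Interface select clears existing selection, then, if the clicking controller owns it, registers it and spawns working-building and recruiting widgets on player 0's HUD before calling the parent.
; Deselect removes it from that controller's selection and hides the admin HUD through the owning controller.
; GetSabotaged simply returns true, with no other logic.
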(event Custom|StartSpawningrushWidgetWorking
  (bind _returnvalue (Game|GetPlayerController 0))
  ;[1 1 1] rush widget does not reach to multicast or anything but left it like this
  (bind _asbp_hudmax_parent_class (Utilities|Casting|CastToBP_HUDMaxParentClass (HUD|GetHUD _returnvalue)))
  ;[1 1 1] ASSIGN ON HUD IT DOES NOT TELL BUT ITS OVERRIDEN
  (bind _returnvalue_2 (UserInterface|CreateWidget "/Game/EB/Blueprints/UW_WorkingBuildingWidget.UW_WorkingBuildingWidget_C" _returnvalue))
  (UserInterface|Viewport|AddtoViewport _returnvalue_2 0)
  (bind _returnvalue_3 (UserInterface|CreateWidget "/Game/EB/Blueprints/UW_AdminHutRecruitingHUd.UW_AdminHutRecruitingHUD_C" _returnvalue))
  (Variables|/Game/EB/Blueprints/BP_HUDMaxParentClass.BP_HUDMaxParentClass_C|SetHUD_Admin2RecruitingHUD _asbp_hudmax_parent_class _returnvalue_3)
  (UserInterface|Viewport|AddtoViewport _returnvalue_3 0)
  (Variables|/Game/EB/Blueprints/BP_HUDMaxParentClass.BP_HUDMaxParentClass_C|SetHUD_WorkingRushWidget _asbp_hudmax_parent_class _returnvalue_2))

(event EventBeginPlay)

(event Collision|EventActorBeginOverlap
  (params (OtherActor :type Actor%20Object%20Reference)))

(event EventTick
  (params (DeltaSeconds :type Float%20%28single-precision%29)))

(event EventRTSInterfunctUnitGetSelected
  (params (ControllerClicking :type Player%20Controller%20Object%20Reference))
  (bind _asbp_player_controller_rtsmax_par (Utilities|Casting|CastToBP_PlayerControllerRTSMaxPar ControllerClicking))
  ;[1 1 1] Get selected
  (Default|COREUnselectAllOfExistingUnits _asbp_player_controller_rtsmax_par)
  (bind _isactoroneofitsactors (Default|STRATEGYIsThisActorOneOfItsActors _asbp_player_controller_rtsmax_par self))
  (if _isactoroneofitsactors
    (Utilities|Array|Add (Variables|/Game/EB/Blueprints/BP_PlayerControllerRTSMaxPar.BP_PlayerControllerRTSMaxPar_C|GetAllActorsSelected _asbp_player_controller_rtsmax_par) self)
    (CallFunction|HUDSpawnCorrespondingHUD)))

(event EventHUDSpawnCorrespondingHUD
  ;[1 1 1] ASSIGN ON HUD IT DOES NOT TELL BUT ITS OVERRIDEN
  (CallFunction|StartSpawningrushWidgetWorking)
  (|CallParentFunction))

(event EventRTSInterfunctUnitGetDeselected
  (params (ControllerUnselecting :type Player%20Controller%20Object%20Reference))
  (bind _asbp_player_controller_rtsmax_par (Utilities|Casting|CastToBP_PlayerControllerRTSMaxPar ControllerUnselecting))
  (bind _allactorsselected (Variables|/Game/EB/Blueprints/BP_PlayerControllerRTSMaxPar.BP_PlayerControllerRTSMaxPar_C|GetAllActorsSelected _asbp_player_controller_rtsmax_par))
  ;[1 1 1] Get deselected
  (Utilities|FlowControl|Sequence
    (:then_0
      (bind _isactoroneofitsactors (Default|STRATEGYIsThisActorOneOfItsActors _asbp_player_controller_rtsmax_par self))
      (if _isactoroneofitsactors
        (if (not (< (Utilities|Array|FindItem _allactorsselected self) 0))
          (Utilities|Array|RemoveItem _allactorsselected self)
          (CallFunction|HUDHideAllCorrespondingHUD))))))

(event EventHUDHideAllCorrespondingHUD
  (bind _asbp_player_controller_rtsmax_par (Utilities|Casting|CastToBP_PlayerControllerRTSMaxPar (Components|GetOwner)))
  (Default|HideAdminHud _asbp_player_controller_rtsmax_par))

(fn ConstructionScript
  (|CallParentFunction))

(fn GetSabotaged()
  (params (Worker_sabotaging :type Boolean))
  (Variables|Default|SetGet_sabotaged%28%29 true))