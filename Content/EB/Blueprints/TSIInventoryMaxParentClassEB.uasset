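; Base inventory actor that holds the items of its owning TSI character, with a RepNotify item array whose handler is empty.
; AddItemInInventory runs on authority only, adds items without a limit, assigns their owner, and can equip one as the character's primary weapon.
; AddSavedItem rebuilds saved items by spawning their class at the owner's transform and passing them through the item's pickup call.
; The owner-debug function is an empty, unused stub.
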(event EventBeginPlay)

(event Collision|EventActorBeginOverlap
  (params (OtherActor :type Actor%20Object%20Reference)))

(event EventTick
  (params (DeltaSeconds :type Float%20%28single-precision%29)))

(fn ConstructionScript)

(fn OnRepinInventoryItems)

(fn AddIteminInventory
  (params (ItemToAdd :type TSI%20Item%20Max%20Parent%20Class%20EB%20Object%20Reference))
  ;[1 1 1] #0 Make sure this only runs rom the ser ver sidde
  (Networking|SwitchHasAuthority
    (:Authority
      ;[1 1 1] #1 No necessary INV Limits So make infinitev,And assign owner
      (Utilities|Array|Add (Variables|Default|GetInInventoryItems) ItemToAdd)
      (Actor|SetOwner ItemToAdd (Components|GetOwner))
      ;[1 1 1] # 2 PrimaryWeapon assigning
      (bind _astsicharacter_max_parent_class_eb (Utilities|Casting|CastToTSICharacterMaxParentClassEB (Components|GetOwner)))
      (if (== (Variables|/Game/EB/Blueprints/TSICharacterMaxParentClassEB.TSICharacterMaxParentClassEB_C|GetPrimaryWeaponItem _astsicharacter_max_parent_class_eb) 0)
        ;[1 1 1] # 3 Equip
        (bind _output_get (Variables|/Game/EB/Blueprints/TSICharacterMaxParentClassEB.TSICharacterMaxParentClassEB_C|SetPrimaryWeaponItem _astsicharacter_max_parent_class_eb ItemToAdd))
        (Default|ItemEquip _output_get)
        (Variables|/Game/EB/Blueprints/TSIItemMaxParentClassEB.TSIItemMaxParentClassEB_C|SetbSetToPrimaryWeapon ItemToAdd true)))))

(fn ServerClientsWhoOwnerIs
  ;[1 1 1] Created to DEbug See who owner is in the instances
)

(fn AddSavedItem
  (params (SavedItemData :type EB%20Saved%20Item%20Structure))
  (bind _itemreturned (CallFunction|SpawnItemfromArchetype (Utilities|Struct|BreakEB_SavedItem SavedItemData)))
  (Utilities|IsValid _itemreturned
    (:Is%20Valid
      (Default|ItemGetPicked _itemreturned (.AsTSICharacter%20Max%20Parent%20Class%20EB (Utilities|Casting|CastToTSICharacterMaxParentClassEB (Components|GetOwner)))))))

(fn SpawnItemfromArchetype
  (params (ItemArchetype :type TSI%20Item%20Max%20Parent%20Class%20EB%20Class%20Reference))
  (bind _returnvalue (Components|GetOwner))
  (Utilities|IsValid _returnvalue
    (:Is%20Valid
      (bind _returnvalue_2 (Game|SpawnActorfromClass ItemArchetype (Transformation|GetActorTransform _returnvalue) "AdjustIfPossibleButAlwaysSpawn" _returnvalue 0))
      (return _returnvalue_2))))