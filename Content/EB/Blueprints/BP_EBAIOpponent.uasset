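; AI strategy opponent that builds a headquarters, recruits units and moves its formations.
; A post-begin-play event claims an industrial zone, spawns an admin hut construction on the traced landscape and sends a team worker to build it.
; Difficulty-adjusted looping timers drive commander ticks: attention recruits a capped number of soldiers from the hut using AI money, while offensive orders waypoint-less formations to random nearby points.
; Defensive and aggressive ticks are empty, and several checks are stubs.
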(event Custom|AICommanderAgressive)

(event Custom|PostBeginPlayBeginTheBussinesLife
  (if (not (CallFunction|STRATEGYBisBuiuldingHQAlready))
    (if (and (< (Utilities|Array|Length (Variables|Default|GetOwnedConstructions)) 1) (< (Utilities|Array|Length (Variables|Default|GetSTARTEDConstr5uctionInProcess)) 1))
      (bind _worker (CallFunction|AIINFSelectAWorker))
      (CallFunction|AIINFHandleSelectWorkertoBuildHutQuarters _worker))))

(event Custom|AICommanderAttenttionTick
  ;[1 1 1] Delete this as should not recruit a lot
  (if (CallFunction|AIBHasAIMoneyforWorkers)
    (if (CallFunction|AIRECRUITINGBHasEnoughWorkers)
      (if (CallFunction|BHasMoneyforWorkers "NewEnumerator1")
        (Utilities|IsValid (CallFunction|AIGeterGetAdminHUT)
          (:Is%20Valid
            (if (< (Variables|Default|GetSoldiersToRecruitMaxAmountCOUNTDeleteThis) 8)
              (bind _didrecruit (CallFunction|AIRECRUITINGHandlerecruitUnit "NewEnumerator1"))
              (if _didrecruit
                (Variables|Default|SetSoldiersToRecruitMaxAmountCOUNTDeleteThis (+ (Variables|Default|GetSoldiersToRecruitMaxAmountCOUNTDeleteThis) 1))))))))))

(event Custom|AICommanderDefensiveTick)

(event Custom|AICommanderOffensiveTick
  (for _array_element (Variables|Default|GetAllActorsOfThisController)
    (bind _astsicharacter_max_parent_class_in_use (Utilities|Casting|CastToTSICharacterMaxParentClassInUse _array_element))
    (if (and true (< (Utilities|Array|Length (.waypoints (Utilities|Array|Get(acopy) (.groups (Default|GetFormationInfoStructfromLeader (Variables|/Game/TSIBPTSICntnt/TSIBlueprints/Pawns/TSICharacterMaxParentClassInUse.TSICharacterMaxParentClassInUse_C|GetFormationInfo _astsicharacter_max_parent_class_in_use)))))) 1))
      (bind _asformation_system_of_leader (Utilities|Casting|CastToFormationSystemOfLeader (Variables|/Game/TSIBPTSICntnt/TSIBlueprints/Pawns/TSICharacterMaxParentClassInUse.TSICharacterMaxParentClassInUse_C|GetFormationInfo _astsicharacter_max_parent_class_in_use)))
      (Default|GiveOrdertoAllGLs _asformation_system_of_leader 0 (+ (Transformation|GetActorLocation _astsicharacter_max_parent_class_in_use) (Math|Vector|MakeVector (Math|Random|RandomFloatinRange -3e+03 3e+03) (Math|Random|RandomFloatinRange -3e+03 3e+03) 0.0))))))

(event EventBeginPlay
  (Utilities|Time|SetTimerbyEvent (delegate Custom|AICommanderAttenttionTick) (- (Math|Random|RandomFloatinRange 1.0 1.5) (Variables|Default|GetAI_Difficulty)) true)
  (Utilities|Time|SetTimerbyEvent (delegate Custom|AICommanderDefensiveTick) (- (Math|Random|RandomFloatinRange 1.0 1.5) (Variables|Default|GetAI_Difficulty)) true)
  (Utilities|Time|SetTimerbyEvent (delegate Custom|AICommanderOffensiveTick) (- (Math|Random|RandomFloatinRange 1.0 1.5) (Variables|Default|GetAI_Difficulty)) true)
  (Utilities|Time|SetTimerbyEvent (delegate Custom|AICommanderAgressive) (- (Math|Random|RandomFloatinRange 1.0 1.5) (Variables|Default|GetAI_Difficulty)) true)
  (Utilities|FlowControl|Delay 2.0)
  ;[1 1 1] Add the log message here because it wont work on PBPlay
  (bind _asbp_hudmax_parent_class (Utilities|Casting|CastToBP_HUDMaxParentClass (HUD|GetHUD (Game|GetPlayerController 0))))
  (Default|HUDLOGAddLogMessage _asbp_hudmax_parent_class (Utilities|String|Append "(name) spends " (Utilities|String|ToString(Integer) (Variables|/Game/EB/Blueprints/BP_ParcellaZoneVolumeMaxParentClass.BP_ParcellaZoneVolumeMaxParentClass_C|GetPrice (Utilities|Array|Get(acopy) (Variables|Default|GetOwnedZones)))) "Has now " (Utilities|String|ToString(Integer) (Variables|Default|GetAIOPONENT_RPGMoney)) "And parcella") 5.0 (Utilities|Struct|MakeSlateColor "(R=1.000000,G=0.016950,B=0.000000,A=1.000000)")))

(event EventTick
  (params (DeltaSeconds :type Float%20%28single-precision%29))
  (|CallParentFunction DeltaSeconds))

(fn ConstructionScript
  (|CallParentFunction))

(fn AICommanderTickDepracated)

(fn AIHandleSelectUnits)

(fn AIINFHandleSelectWorkertoBuildHutQuarters
  (params (AIWorker :type BP%20EB%20Worker%20Object%20Reference))
  (Utilities|Array|Add (Variables|Default|GetSelectedActors) AIWorker)
  (CallFunction|AICONSTRGetIndustrialZone)
  (bind _ownedparcella (CallFunction|AICONSTRReturnOwnedParcella))
  (Utilities|IsValid _ownedparcella
    (:Is%20Valid
      (CallFunction|STRATEGYSTARTConstructionandHologramMakeItHappend "/Game/EB/Blueprints/BP_AdminHutProcessConstruction.BP_AdminHutProcessConstruction_C" (Transformation|GetActorLocation _ownedparcella) AIWorker))))

(fn AIINFSelectAWorker
  (bind _outactors (Actor|GetAllActorsOfClass "/Game/EB/Blueprints/BP_EBWorker.BP_EBWorker_C"))
  ;[1 1 1] Make sure that later on we have check for BOSS
  (for _array_element _outactors
    (if (== (Variables|/Game/EB/Blueprints/TSICharacterMaxParentClassEB.TSICharacterMaxParentClassEB_C|GetTeamNum _array_element) (Variables|Default|GetTeamNumAIOponent))
      (return _array_element))))

(fn AICONSTRGetIndustrialZone
  ;[1 1 1] Represents that buys in here
  (bind _parcella (CallFunction|AICONSTRReturnFreeIndustrialZone))
  (Utilities|Array|Add (Variables|Default|GetOwnedZones) _parcella)
  (Default|ParcellaHandleGetBought _parcella self))

(fn AICONSTRReturnFreeIndustrialZone
  (bind _outactors (Actor|GetAllActorsOfClass "/Game/EB/Blueprints/BP_ParcellaZoneVolumeMaxParentClass.BP_ParcellaZoneVolumeMaxParentClass_C"))
  (for _array_element _outactors
    _)
  (return _array_element))

(fn AICONSTRBHasNonOverSaturatedZone
  (return true))

(fn AICONSTRReturnOwnedParcella
  (return (Utilities|Array|Get(acopy) (Variables|Default|GetOwnedZones))))

(fn STRATEGYSTARTConstructionandHologramMakeItHappend
  (params (HoloArche :type BP%20Construction%20in%20Process%20Max%20Parent%20Class%20Class%20Reference) (HoloLoc :type Vector) (BuilderBuilding :type BP%20EB%20Worker%20Object%20Reference))
  (bind _surface (CallFunction|AICONSTRTraceSurface HoloLoc))
  (bind _returnvalue (Game|SpawnActorfromClass HoloArche (Math|Conversions|ToTransform(Vector) _surface) "Undefined" 0 0 0))
  (CallFunction|AISendWorkerstoWorkandBuild BuilderBuilding _surface)
  (return _returnvalue))

(fn AICONSTRTraceSurface
  (params (InitialLoc :type Vector))
  (bind _outhits (Class|KismetSystemLibrary|LineTraceMultiforObjects (+ (Math|Vector|MakeVector (.x InitialLoc) (.y InitialLoc) (.z InitialLoc)) "0, 0,10000.000000") (+ (Math|Vector|MakeVector (.x InitialLoc) (.y InitialLoc) (.z InitialLoc)) "0, 0,-10000000.000000") (Utilities|Array|MakeArray "ObjectTypeQuery1") false 0 "Persistent" true "(R=1.000000,G=0.000000,B=0.000000,A=1.000000)" "(R=0.000000,G=1.000000,B=0.000000,A=1.000000)" 1e+01))
  (for _array_element _outhits
    (Utilities|Casting|CastToLandscape (.HitActor (Collision|BreakHitResult _array_element)))
    (return (Math|Vector|MakeVector (.X (Math|Vector|BreakVector (.Location (Collision|BreakHitResult _array_element)))) (.Y (Math|Vector|BreakVector (.Location (Collision|BreakHitResult _array_element)))) (.Z (Math|Vector|BreakVector (.Location (Collision|BreakHitResult _array_element))))))))

(fn STRATEGYBisBuiuldingHQAlready
  (for _array_element (Variables|Default|GetSTARTEDConstr5uctionInProcess)
    (Utilities|Casting|CastToBP_AdminHutHologram _array_element)
    (return true))
  (return false))

(fn AISendWorkerstoWorkandBuild
  (params (IndividualWorkerToWork :type TSI%20Character%20Max%20Parent%20Class%20EB%20Object%20Reference) (Loc :type Vector))
  (Rendering|Debug|DrawDebugSphere Loc 1e+02 12 "(R=0.000000,G=1.000000,B=0.161979,A=1.000000)" 1e+01 1.0)
  (Rendering|Debug|DrawDebugSphere (Transformation|GetActorLocation IndividualWorkerToWork) 1e+02 12 "(R=0.000000,G=0.127968,B=1.000000,A=1.000000)" 1e+01 1e+01)
  (bind _asbp_ebaicontroller_max_parent_class (Utilities|Casting|CastToBP_EBAIControllerMaxParentClass (Pawn|GetController IndividualWorkerToWork)))
  (Default|SetDesiredLocation _asbp_ebaicontroller_max_parent_class Loc)
  (Default|GotoStateAIWokerorWhataver _asbp_ebaicontroller_max_parent_class "NewEnumerator1" (Variables|/Game/EB/Blueprints/BP_EBAIControllerMaxParentClass.BP_EBAIControllerMaxParentClass_C|GetAI_StateOfWorkerOrWhataver _asbp_ebaicontroller_max_parent_class)))

(fn AIBHasAIMoneyforWorkers
  (return true))

(fn AIRECRUITINGHandlerecruitUnit
  (params (UnitType :type EN_UnitType%20Enum :default "NewEnumerator0"))
  (bind _adminhut (CallFunction|AIGeterGetAdminHUT))
  (if (Default|STRATEGYBHasNoCoolDownonRecruiting _adminhut)
    (Utilities|IsValid _adminhut
      (:Is%20Valid
        (switch Utilities|FlowControl|Switch|SwitchonEN_UnitType UnitType
          (:NewEnumerator0
            (bind _brecruitedsoldier (Default|STATEGYRecruitUnit _adminhut "/Game/EB/Blueprints/BP_EBWorker.BP_EBWorker_C"))
            (CallFunction|AIECONOMYSpendMoneyOppo 250)
            (return _brecruitedsoldier 0))
          (:NewEnumerator1
            (bind _brecruitedsoldier_2 (Default|STATEGYRecruitUnit _adminhut "/Game/TSIBPTSICntnt/TSIBlueprints/Pawns/TSIDefaultSoldier.TSIDefaultSoldier_C"))
            (CallFunction|AIECONOMYSpendMoneyOppo 250)
            (return _brecruitedsoldier_2 0))
          (:NewEnumerator2
            ;[1 1 1] WIP
            (bind _brecruitedsoldier_3 (Default|STATEGYRecruitUnit _adminhut "/Game/EB/Blueprints/BP_EBWorker.BP_EBWorker_C"))
            (CallFunction|AIECONOMYSpendMoneyOppo 250)
            (return _brecruitedsoldier_3 0)))))
    (else
      (return false 0))))

(fn AIRECRUITINGBHasEnoughWorkers
  (bind _workersnum (LocalVariables|GetWorkersNum))
  (for _array_element (Variables|Default|GetAllActorsOfThisController)
    (Utilities|Casting|CastToBP_EBWorker _array_element)
    (Math|Integer|IncrementInt _workersnum))
  (return (> _workersnum 0)))

(fn AIECONOMYSpendMoneyOppo
  (params (MoneyAmmount :type Integer))
  (Variables|Default|SetAIOPONENT_RPGMoney (Math|Integer|Clamp(Integer) (- (Variables|Default|GetAIOPONENT_RPGMoney) MoneyAmmount) 0 10000)))

(fn AIGeterGetAdminHUT
  (for _array_element (Variables|Default|GetOwnedConstructions)
    (bind _asbp_admin_hut_construction (Utilities|Casting|CastToBP_AdminHutConstruction _array_element))
    (return _asbp_admin_hut_construction))
  (return 0))

(fn BHasMoneyforWorkers
  (params (WorkerUnit :type EN_UnitType%20Enum :default "NewEnumerator0"))
  (switch Utilities|FlowControl|Switch|SwitchonEN_UnitType WorkerUnit
    (:NewEnumerator0
      (return (>= (Variables|Default|GetAIOPONENT_RPGMoney) (Class|KismetSystemLibrary|MakeLiteralInteger 250))))
    (:NewEnumerator1
      (return (>= (Variables|Default|GetAIOPONENT_RPGMoney) (Class|KismetSystemLibrary|MakeLiteralInteger 500))))
    (:NewEnumerator2
      (return (>= (Variables|Default|GetAIOPONENT_RPGMoney) (Class|KismetSystemLibrary|MakeLiteralInteger 750))))))

(fn STRATEGYAddtoOwnedActors
  (params (NewActorToAdd :type Actor%20Object%20Reference))
  ;[1 1 1] This should be called only server side
  (Networking|SwitchHasAuthority
    (:Authority
      (Utilities|Array|Add (Variables|Default|GetAllActorsOfThisController) NewActorToAdd))))