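; BP_Crane is a controllable crane pawn driven entirely by input axis events.
; MoveForward adds movement along the actor's forward vector, while MoveRight steers by subtracting the raw axis value from actor yaw, without delta-time scaling.
; Turn and LookUp feed controller yaw and pitch only when possessed by BP_PlayerControllerRTSMaxPar.
; An earlier strafe movement path remains in the graph but never runs.
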(event EventBeginPlay
  (|CallParentFunction) ; This node is disabled and will not be called.\nDrag off pins to build functionality.
)

(event Collision|EventActorBeginOverlap
  (params (OtherActor :type Actor%20Object%20Reference))
  (|CallParentFunction OtherActor) ; This node is disabled and will not be called.\nDrag off pins to build functionality.
)

(event EventTick
  (params (DeltaSeconds :type Float%20%28single-precision%29))
  (|CallParentFunction DeltaSeconds) ; This node is disabled and will not be called.\nDrag off pins to build functionality.
)

(event Input|AxisEvents|InputAxisMoveRight
  (params (AxisValue :type Float%20%28single-precision%29))
  (bind _returnvalue (Transformation|GetActorRotation))
  (bind (_roll _pitch _yaw) (Math|Rotator|BreakRotator _returnvalue))
  ;[1 1 1] Investigate how this works
  (if (or (> AxisValue 0.0) (< AxisValue 0.0))
    (Transformation|SetActorRotation (Math|Rotator|MakeRotator _roll _pitch (+ _yaw (* AxisValue -1.0))))))

(event Input|AxisEvents|InputAxisMoveForward
  (params (AxisValue :type Float%20%28single-precision%29))
  ;[1 1 1] Investigate how this works
  (Pawn|Input|AddMovementInput (Math|Vector|GetForwardVector (Transformation|GetActorRotation)) AxisValue false))

(event Input|AxisEvents|InputAxisTurn
  (params (AxisValue :type Float%20%28single-precision%29))
  (Utilities|Casting|CastToBP_PlayerControllerRTSMaxPar (Pawn|GetController))
  (Pawn|Input|AddControllerYawInput AxisValue))

(event Input|AxisEvents|InputAxisLookUp
  (params (AxisValue :type Float%20%28single-precision%29))
  (Utilities|Casting|CastToBP_PlayerControllerRTSMaxPar (Pawn|GetController))
  (Pawn|Input|AddControllerPitchInput AxisValue))

(fn ConstructionScript
  (|CallParentFunction))