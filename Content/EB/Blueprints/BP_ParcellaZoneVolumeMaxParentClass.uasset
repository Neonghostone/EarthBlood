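; Parent class for a buyable RTS land parcel ("parcella") that player or AI opponent controllers can own.
; A player worker entering the volume triggers a server-authoritative purchase that deducts Price and sets owner and TeamOwning.
; OnRep_TeamOwning tints the zone material green for the local team, red for others.
; Mouse events drive hover translucency and an options widget, while helpers query contained actors, oil rigs and random points.
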(event OnComponentBeginOverlap(VolumeOfZone)
  (params (OverlappedComponent :type Primitive%20Component%20Object%20Reference) (OtherActor :type Actor%20Object%20Reference) (OtherComp :type Primitive%20Component%20Object%20Reference) (OtherBodyIndex :type Integer) (bFromSweep :type Boolean) (SweepResult :type Hit%20Result%20Structure%20%28by%20ref%29))
  (bind _asbp_ebworker (Utilities|Casting|CastToBP_EBWorker OtherActor))
  (Utilities|Casting|CastToPlayerController (Components|GetOwner _asbp_ebworker))
  (CallFunction|ParcellaHandleGetBought (.AsController (Utilities|Casting|CastToController (Components|GetOwner _asbp_ebworker)))))

(event Custom|ServerHandleParcellaGetBought
  (params (NewOwner :type Controller%20Object%20Reference))
  (CallFunction|ParcellaHandleGetBought NewOwner))

(event Custom|MulticastHandleZoneGetBought
  (params (Value :type Linear%20Color%20Structure))
  ;[1 1 1] Kept as is useful as the begin play
  (bind _returnvalue (Rendering|Material|CreateDynamicMaterialInstance (Variables|Default|GetVolumeMesh) 0 0 "None" :!class /Script/Engine.PrimitiveComponent))
  (Rendering|Material|SetVectorParameterValue _returnvalue "ColorOfZone" Value :!class /Script/Engine.MaterialInstanceDynamic))

(event EventBeginPlay
  (bind _teamowning (Variables|Default|GetTeamOwning))
  (Utilities|FlowControl|Sequence
    (:then_0
      (Networking|SwitchHasAuthority
        (:Authority
          _)
        (:Remote
          _))
      (bind _asuw_parcella_sell_options (Utilities|Casting|CastToUW_ParcellaSellOptions (UserInterface|GetUserWidgetObject (Variables|Default|GetParcellaSellOptions))))
      (Variables|/Game/EB/Blueprints/UW_ParcellaSellOptions.UW_ParcellaSellOptions_C|SetParcellaOwner _asuw_parcella_sell_options self))
    (:then_1
      (Networking|SwitchHasAuthority
        (:Authority
          _)
        (:Remote
          _))
      (bind _asbp_player_controller_rtsmax_par (Utilities|Casting|CastToBP_PlayerControllerRTSMaxPar (Game|GetPlayerController 0)))
      (if (not (== _teamowning 0))
        (if (== _teamowning (Variables|/Game/EB/Blueprints/BP_PlayerControllerRTSMaxPar.BP_PlayerControllerRTSMaxPar_C|GetTeamNum _asbp_player_controller_rtsmax_par))
          (CallFunction|MulticastHandleZoneGetBought "(R=0.000000,G=1.000000,B=0.000000,A=1.000000)")
          (else
            (CallFunction|MulticastHandleZoneGetBought "(R=1.000000,G=0.000000,B=0.000000,A=1.000000)")))))))

(event Collision|EventActorBeginOverlap
  (params (OtherActor :type Actor%20Object%20Reference)))

(event EventTick
  (params (DeltaSeconds :type Float%20%28single-precision%29)))

(event EventRTSMouseInterfunctonMouseOver
  (params (controllerThatMouseOvered :type Player%20Controller%20Object%20Reference))
  (bind _returnvalue (Rendering|Material|CreateDynamicMaterialInstance (Variables|Default|GetVolumeMesh) 0 0 "None" :!class /Script/Engine.PrimitiveComponent))
  (Rendering|Material|SetScalarParameterValue _returnvalue "Transluency" 0.05 :!class /Script/Engine.MaterialInstanceDynamic))

(event EventRTSMouseInterfunctonMouseLeftClick
  (params (ControllerThat0LeftClicked :type Player%20Controller%20Object%20Reference))
  (bind _asbp_player_controller_rtsmax_par (Utilities|Casting|CastToBP_PlayerControllerRTSMaxPar ControllerThat0LeftClicked))
  (Utilities|Casting|CastToSpectatorPawn (Pawn|GetControlledPawn _asbp_player_controller_rtsmax_par))
  (bind _asbp_hudmax_parent_class (Utilities|Casting|CastToBP_HUDMaxParentClass (HUD|GetHUD _asbp_player_controller_rtsmax_par)))
  (bind _returnvalue (UserInterface|CreateWidget "/Game/EB/Blueprints/UW_ParcellaZoneOptions.UW_ParcellaZoneOptions_C" _asbp_player_controller_rtsmax_par))
  (UserInterface|Viewport|AddtoViewport _returnvalue 0)
  (Variables|/Game/EB/Blueprints/BP_HUDMaxParentClass.BP_HUDMaxParentClass_C|SetHUD_ParcellaWidget _asbp_hudmax_parent_class (.AsUW%20Parcella%20Zone%20Options (Utilities|Casting|CastToUW_ParcellaZoneOptions _returnvalue))))

(event EventRTSMouseInterFunctonMouseOut
  (params (ControllerMousseOuted :type Player%20Controller%20Object%20Reference))
  (bind _returnvalue (Rendering|Material|CreateDynamicMaterialInstance (Variables|Default|GetVolumeMesh) 0 0 "None" :!class /Script/Engine.PrimitiveComponent))
  (Rendering|Material|SetScalarParameterValue _returnvalue "Transluency" 0.01 :!class /Script/Engine.MaterialInstanceDynamic))

(fn ConstructionScript
  (Collision|SetCollisionEnabled (Variables|Default|GetVolumeMesh) "NoCollision"))

(fn ParcellaHandleGetBought
  (params (NewOwner :type Controller%20Object%20Reference))
  (bind _price (Variables|Default|GetPrice))
  (bind _price_2 (Variables|Default|GetPrice))
  ;[1 1 1] The parcella industrial zone will get bought by player or oponent, so make sure you cast well
  (if (CallFunction|IsWorkerinParcella)
    (if (Variables|Default|GetbBought)
      _
      (else
        (Networking|SwitchHasAuthority
          (:Authority
            (Actor|SetOwner NewOwner)
            (bind _asbp_player_controller_rtsmax_par (Utilities|Casting|CastToBP_PlayerControllerRTSMaxPar NewOwner)
              (:then
                (Default|RTSRPGSetMoney _asbp_player_controller_rtsmax_par (- (Variables|/Game/EB/Blueprints/BP_PlayerControllerRTSMaxPar.BP_PlayerControllerRTSMaxPar_C|GetRPGMoney _asbp_player_controller_rtsmax_par) _price) (* _price -1))
                (Variables|Default|SetbBought true)
                (CallFunction|MulticastHandleZoneGetBought)
                (Variables|Default|SetTeamOwning (Variables|/Game/EB/Blueprints/BP_PlayerControllerRTSMaxPar.BP_PlayerControllerRTSMaxPar_C|GetTeamNum _asbp_player_controller_rtsmax_par))
                (Actor|SetOwner _asbp_player_controller_rtsmax_par)
                (return true))
              (:CastFailed
                (bind _asbp_ebaiopponent (Utilities|Casting|CastToBP_EBAIRTSControllerOpponent NewOwner))
                (Variables|Default|SetTeamOwning (Math|Conversions|ToByte(Integer) (Variables|/Game/EB/Blueprints/BP_EBAIRTSControllerOpponent.BP_EBAIRTSControllerOpponent_C|GetTeamNumAIOponent _asbp_ebaiopponent)))
                (CallFunction|MulticastHandleZoneGetBought)
                (Default|RTSRPGSetMoney _asbp_ebaiopponent (- (Variables|/Game/EB/Blueprints/BP_EBAIControllerMaxParentClass.BP_EBAIControllerMaxParentClass_C|GetAIOPONENT_RPGMoney _asbp_ebaiopponent) _price_2) (* _price_2 -1))
                (Variables|Default|SetbBought true)
                (Actor|SetOwner _asbp_ebaiopponent)
                (return true))))))))
  (return false))

(fn OnRepTeamOwning
  (bind _asbp_player_controller_rtsmax_par (Utilities|Casting|CastToBP_PlayerControllerRTSMaxPar (Game|GetPlayerController 0)))
  (if (== (Variables|/Game/EB/Blueprints/BP_PlayerControllerRTSMaxPar.BP_PlayerControllerRTSMaxPar_C|GetTeamNum _asbp_player_controller_rtsmax_par) (Variables|Default|GetTeamOwning))
    (CallFunction|MulticastHandleZoneGetBought "(R=0.000000,G=1.000000,B=0.000000,A=1.000000)")
    (else
      (CallFunction|MulticastHandleZoneGetBought "(R=1.000000,G=0.000000,B=0.000000,A=1.000000)"))))

(fn ReturnActorsinParcella
  (return (Collision|GetOverlappingActors "/Script/Engine.Actor" :!class /Script/Engine.Actor)))

(fn IsWorkerinParcella
  (for _array_element (Collision|GetOverlappingActors "/Game/EB/Blueprints/BP_EBWorker.BP_EBWorker_C" :!class /Script/Engine.Actor)
    (Utilities|IsValid _array_element
      (:Is%20Valid
        (return true))))
  (bind _asbp_ebgame_max_par (Utilities|Casting|CastToBP_EBGameMaxPar (Game|GetGameMode)))
  (Default|BroadcastMessageDependingtoWho _asbp_ebgame_max_par 0 true 0 "Get there someone to investigate area! And Buy!" "None" false true "(R=1.000000,G=0.080550,B=0.000000,A=1.000000)" false)
  ;[1 1 1] careful always returns TRUE!!!!!!
  (return false))

(fn GetRandomPointintheBox
  (bind _volumeofzone (Variables|Default|GetVolumeOfZone))
  ;[1 1 1] ATTENTION NOT ALT MODIFIED
  (return (Math|Random|RandomPointinBoundingBox (Transformation|GetWorldLocation _volumeofzone) (Components|Box|GetScaledBoxExtent _volumeofzone))))

(fn AreThereEnoughOilRigs
  (bind _oilrigscount (LocalVariables|GetOilRigsCount))
  (for _array_element (CallFunction|GetAllActorsInsideParcella)
    (Utilities|Casting|CastToBP_OilPumpInProcess _array_element
      (:then
        (Math|Integer|IncrementInt _oilrigscount))
      (:CastFailed
        (Utilities|Casting|CastToBP_BuildingOilPumpConstruction _array_element)
        (Math|Integer|IncrementInt _oilrigscount))))
  (return (not (<= (LocalVariables|GetOilRigsCount) 2))))

(fn GetAllActorsInsideParcella
  (return (Collision|GetOverlappingActors (Variables|Default|GetVolumeOfZone) "/Script/Engine.Actor" :!class /Script/Engine.PrimitiveComponent)))

(fn RTSDoesGetCaughtDoingCrime
  (return false 0 0 "0, 0, 0"))