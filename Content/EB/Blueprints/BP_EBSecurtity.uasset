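; BP_EBSecurtity is a selectable RTS security unit that moves to right-clicked map locations.
; It handles RTS interface events for select and deselect, adding or removing itself from BP_PlayerControllerRTSMaxPar's AllActorsSelected array only when that controller counts it as its own.
; Right-click orders call SimpleMoveToLocation on the unit's own controller, if valid.
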(event EventBeginPlay
  (|CallParentFunction))

(event Collision|EventActorBeginOverlap
  (params (OtherActor :type Actor%20Object%20Reference)))

(event EventTick
  (params (DeltaSeconds :type Float%20%28single-precision%29))
  (|CallParentFunction DeltaSeconds))

(event EventRTSInterfunctHandleRightClickonLSorSMwithSelected
  (params (PlayerControllerUsing :type Player%20Controller%20Object%20Reference) (PlaceOnMap :type Vector :default "0, 0, 0"))
  (bind _returnvalue (Pawn|GetController))
  (if (Utilities|IsValid _returnvalue)
    (AI|Navigation|SimpleMovetoLocation _returnvalue PlaceOnMap)))

(event EventRTSInterfunctUnitGetSelected
  (params (ControllerClicking :type Player%20Controller%20Object%20Reference))
  (bind _asbp_player_controller_rtsmax_par (Utilities|Casting|CastToBP_PlayerControllerRTSMaxPar ControllerClicking))
  (bind _isactoroneofitsactors (Default|STRATEGYIsThisActorOneOfItsActors _asbp_player_controller_rtsmax_par self))
  (if _isactoroneofitsactors
    (Utilities|Array|Add (Variables|/Game/EB/Blueprints/BP_PlayerControllerRTSMaxPar.BP_PlayerControllerRTSMaxPar_C|GetAllActorsSelected _asbp_player_controller_rtsmax_par) self)))

(event EventRTSInterfunctUnitGetDeselected
  (params (ControllerUnselecting :type Player%20Controller%20Object%20Reference))
  (bind _asbp_player_controller_rtsmax_par (Utilities|Casting|CastToBP_PlayerControllerRTSMaxPar ControllerUnselecting))
  (bind _isactoroneofitsactors (Default|STRATEGYIsThisActorOneOfItsActors _asbp_player_controller_rtsmax_par self))
  (if _isactoroneofitsactors
    (if (not (< (Utilities|Array|FindItem (Variables|/Game/EB/Blueprints/BP_PlayerControllerRTSMaxPar.BP_PlayerControllerRTSMaxPar_C|GetAllActorsSelected _asbp_player_controller_rtsmax_par) self) 0))
      (Utilities|Array|RemoveItem (Variables|/Game/EB/Blueprints/BP_PlayerControllerRTSMaxPar.BP_PlayerControllerRTSMaxPar_C|GetAllActorsSelected _asbp_player_controller_rtsmax_par) self))))

(fn ConstructionScript
  (|CallParentFunction))