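; BP_AdminHutConstruction is the RTS admin hut building, handling selection, hover tinting, blinking materials and a work-in-progress sabotage mechanic.
; Selection by the owning player registers it with the controller and spawns recruiting and working-rush widgets; deselection hides them.
; Right-click toggles blinking and stores the controller's selected units as saboteurs.
; Tick randomly samples those within range but only prints debug messages; GetSabotaged is empty.
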(event Custom|Event1
  ;[1 1 1] Functionality pool here on mouse click
  (bind _returnvalue (Rendering|Material|CreateDynamicMaterialInstance (Variables|Default|GetBuildingsMesh) 0 "/Game/RTSTemplateContent/3dArt/Buildings/HutRoofMat.HutRoofMat" "None" :!class /Script/Engine.PrimitiveComponent))
  (Rendering|Material|SetVectorParameterValue _returnvalue "Em" "(R=0.135508,G=0.164325,B=0.578125,A=1.000000)" :!class /Script/Engine.MaterialInstanceDynamic)
  (Rendering|Material|SetMaterial (Variables|Character|GetMesh) 0 (Rendering|Material|GetMaterial (Variables|Default|GetBuildingsMesh) 0))
  (Utilities|FlowControl|Delay 0.5)
  (bind _returnvalue_2 (Rendering|Material|CreateDynamicMaterialInstance (Variables|Default|GetBuildingsMesh) 0 "/Game/RTSTemplateContent/3dArt/Buildings/HutRoofMat.HutRoofMat" "None" :!class /Script/Engine.PrimitiveComponent))
  (Rendering|Material|SetVectorParameterValue _returnvalue_2 "Em" "(R=0.703125,G=0.050578,B=0.000000,A=1.000000)" :!class /Script/Engine.MaterialInstanceDynamic)
  (Rendering|Material|SetMaterial (Variables|Character|GetMesh) 0 (Rendering|Material|GetMaterial (Variables|Default|GetBuildingsMesh) 0)))

(event Custom|Event2
  ;[1 1 1] Functionality pool here on mouse click
  (Utilities|FlowControl|Delay 5.0)
  (Utilities|Time|ClearandInvalidateTimerbyHandle (Variables|Default|GetReturn%20Value)))

(event Custom|GetSabotaged
  (params (Sabotagers :type Array%20of%20Actor%20Object%20References)))

(event Custom|StartSpawningrushWidgetWorking
  (bind _returnvalue (Game|GetPlayerController 0))
  ;[1 1 1] rush widget does not reach to multicast or anything but left it like this
  (bind _asbp_hudmax_parent_class (Utilities|Casting|CastToBP_HUDMaxParentClass (HUD|GetHUD _returnvalue)))
  ;[1 1 1] ASSIGN ON HUD IT DOES NOT TELL BUT ITS OVERRIDEN
  (bind _returnvalue_2 (UserInterface|CreateWidget "/Game/EB/Blueprints/UW_WorkingBuildingWidget.UW_WorkingBuildingWidget_C" _returnvalue))
  (UserInterface|Viewport|AddtoViewport _returnvalue_2 0)
  (bind _returnvalue_3 (UserInterface|CreateWidget "/Game/EB/Blueprints/UW_AdminHutRecruitingHUd.UW_AdminHutRecruitingHUD_C" _returnvalue))
  (Variables|/Game/EB/Blueprints/BP_HUDMaxParentClass.BP_HUDMaxParentClass_C|SetHUD_Admin2RecruitingHUD _asbp_hudmax_parent_class _returnvalue_3)
  (UserInterface|Viewport|AddtoViewport _returnvalue_3 0)
  (Variables|/Game/EB/Blueprints/BP_HUDMaxParentClass.BP_HUDMaxParentClass_C|SetHUD_WorkingRushWidget _asbp_hudmax_parent_class _returnvalue_2))

(event Custom|ServerHandleRightClickOn
  (params (UnitsRightClickingOn :type Array%20of%20Actor%20Object%20References) (PurposeRightClick :type EN_PurposeOfRightClick%20Enum :default "NewEnumerator0"))
  ;[1 1 1] If we want a different purpose with slection menu but for now just right click
  (Development|PrintString (Utilities|String|Append "FROOM Adminhut the slect4ed workers are" (Utilities|String|ToString(Integer) (Utilities|Array|Length UnitsRightClickingOn))))
  (Variables|Default|SetAssignedSabotagers UnitsRightClickingOn))

(event EventBeginPlay)

(event Collision|EventActorBeginOverlap
  (params (OtherActor :type Actor%20Object%20Reference)))

(event EventRTSInterfunctUnitGetSelected
  (params (ControllerClicking :type Player%20Controller%20Object%20Reference))
  (bind _asbp_player_controller_rtsmax_par (Utilities|Casting|CastToBP_PlayerControllerRTSMaxPar ControllerClicking))
  ;[1 1 1] Get selected
  (Development|PrintString "FROM admin hut getting selected")
  (Default|COREUnselectAllOfExistingUnits _asbp_player_controller_rtsmax_par)
  (bind _isactoroneofitsactors (Default|STRATEGYIsThisActorOneOfItsActors _asbp_player_controller_rtsmax_par self))
  (if _isactoroneofitsactors
    (Utilities|Array|Add (Variables|/Game/EB/Blueprints/BP_PlayerControllerRTSMaxPar.BP_PlayerControllerRTSMaxPar_C|GetAllActorsSelected _asbp_player_controller_rtsmax_par) self)
    (CallFunction|DisableBlinking _asbp_player_controller_rtsmax_par)
    (CallFunction|HUDSpawnCorrespondingHUD)))

(event EventHUDSpawnCorrespondingHUD
  ;[1 1 1] ASSIGN ON HUD IT DOES NOT TELL BUT ITS OVERRIDEN
  (CallFunction|StartSpawningrushWidgetWorking)
  (|CallParentFunction))

(event EventRTSInterfunctUnitGetDeselected
  (params (ControllerUnselecting :type Player%20Controller%20Object%20Reference))
  (bind _asbp_player_controller_rtsmax_par (Utilities|Casting|CastToBP_PlayerControllerRTSMaxPar ControllerUnselecting))
  (bind _allactorsselected (Variables|/Game/EB/Blueprints/BP_PlayerControllerRTSMaxPar.BP_PlayerControllerRTSMaxPar_C|GetAllActorsSelected _asbp_player_controller_rtsmax_par))
  ;[1 1 1] Get deselected
  (Utilities|FlowControl|Sequence
    (:then_0
      (bind _isactoroneofitsactors (Default|STRATEGYIsThisActorOneOfItsActors _asbp_player_controller_rtsmax_par self))
      (if _isactoroneofitsactors
        (if (not (< (Utilities|Array|FindItem _allactorsselected self) 0))
          (Utilities|Array|RemoveItem _allactorsselected self)
          (CallFunction|DisableBlinking _asbp_player_controller_rtsmax_par)
          (CallFunction|HUDHideAllCorrespondingHUD))))))

(event EventInitializeBlinkingMaterials
  ;[1 1 1] Registering Blinking Materials
  (CallFunction|RegisterSetOfBlinkingMaterialInstances (Variables|Default|GetBuildingsMesh) (Utilities|Array|MakeArray "/Game/EB/3d/Buildings/HutBlinkingMaterials/M_Hut_Blinking_Slot_1_Instance.M_Hut_Blinking_Slot_1_Instance" "/Game/EB/3d/Buildings/HutBlinkingMaterials/M_Hut_Blinking_Slot_2_Instance.M_Hut_Blinking_Slot_2_Instance" "/Game/EB/3d/Buildings/HutBlinkingMaterials/M_Hut_Blinking_Slot_3_Instance.M_Hut_Blinking_Slot_3_Instance" "/Game/EB/3d/Buildings/HutBlinkingMaterials/M_Hut_Blinking_Slot_4_Instance.M_Hut_Blinking_Slot_4_Instance")))

(event EventHUDHideAllCorrespondingHUD
  (bind _asbp_player_controller_rtsmax_par (Utilities|Casting|CastToBP_PlayerControllerRTSMaxPar (Components|GetOwner)))
  (Default|HideAdminHud _asbp_player_controller_rtsmax_par))

(event EventRTSMouseInterfunctonMouseRightClick
  (params (ControllerThatRightMouseClicked :type Player%20Controller%20Object%20Reference))
  ;[1 1 1] Just i ncase in the future we want to add a selection menu from mouse do this
  (bind _asbp_player_controller_rtsmax_par (Utilities|Casting|CastToBP_PlayerControllerRTSMaxPar ControllerThatRightMouseClicked))
  (CallFunction|ToggleBlinking _asbp_player_controller_rtsmax_par)
  (Development|PrintString (Utilities|String|Append "FROM BP admin hut getting RIGHT clicked PC is" (Utilities|GetDisplayName ControllerThatRightMouseClicked) (Utilities|String|ToString(Integer) (Utilities|Array|Length (Variables|/Game/EB/Blueprints/BP_PlayerControllerRTSMaxPar.BP_PlayerControllerRTSMaxPar_C|GetAllActorsSelected _asbp_player_controller_rtsmax_par)))))
  (CallFunction|ServerHandleRightClickon (Variables|/Game/EB/Blueprints/BP_PlayerControllerRTSMaxPar.BP_PlayerControllerRTSMaxPar_C|GetAllActorsSelected _asbp_player_controller_rtsmax_par) "NewEnumerator0"))

(event EventRTSMouseInterfunctonMouseOver
  (params (controllerThatMouseOvered :type Player%20Controller%20Object%20Reference))
  (bind _returnvalue (Rendering|Material|CreateDynamicMaterialInstance (Variables|Default|GetBuildingsMesh) 0 "/Game/RTSTemplateContent/3dArt/Buildings/HutMat1.HutMat1" "None" :!class /Script/Engine.PrimitiveComponent))
  (Rendering|Material|SetVectorParameterValue _returnvalue "Em" (Class|KismetMathLibrary|LinearColorDesaturated (Math|Color|MakeColor (Math|Random|RandomFloatinRange 0.0 1.0) (Math|Random|RandomFloatinRange 0.0 1.0) (Math|Random|RandomFloatinRange 0.0 1.0)) (Math|Random|RandomFloatinRange 0.0 0.5)) :!class /Script/Engine.MaterialInstanceDynamic)
  (Rendering|Material|SetMaterial (Variables|Character|GetMesh) 0 (Rendering|Material|GetMaterial (Variables|Default|GetBuildingsMesh) 0)))

(event EventTick
  (params (DeltaSeconds :type Float%20%28single-precision%29))
  (for _array_element (CallFunction|IsAnyActorSaboNearbyReturnHowMany)
    (Utilities|Casting|CastToBP_EBWorker _array_element)
    (if (== (Math|Random|RandomInteger 50) 0)
      (Development|PrintString (Utilities|String|Append "FROM AdminHUT THERE IS AN ACTOR NEAR ASSIGNED SSABOTAGE!!!!!" (Utilities|String|ToString(Integer) (Utilities|Array|Length (CallFunction|IsAnyActorSaboNearbyReturnHowMany))))))))

(event EventRTSMouseInterFunctonMouseOut
  (params (ControllerMousseOuted :type Player%20Controller%20Object%20Reference))
  (bind _returnvalue (Rendering|Material|CreateDynamicMaterialInstance (Variables|Default|GetBuildingsMesh) 0 "/Game/RTSTemplateContent/3dArt/Buildings/HutRoofMat.HutRoofMat" "None" :!class /Script/Engine.PrimitiveComponent))
  (Rendering|Material|SetVectorParameterValue _returnvalue "Em" "(R=0.100700,G=0.109200,B=0.157400,A=1.000000)" :!class /Script/Engine.MaterialInstanceDynamic)
  (Rendering|Material|SetMaterial (Variables|Character|GetMesh) 0 (Rendering|Material|GetMaterial (Variables|Default|GetBuildingsMesh) 0)))

(fn ConstructionScript
  (|CallParentFunction))

(fn IsAnyActorSaboNearbyReturnHowMany
  (bind _localactorsnearby (LocalVariables|GetLocalActorsNearby))
  (for _array_element (Variables|Default|GetAssignedSabotagers)
    (if (< (Transformation|GetDistanceTo _array_element) (Variables|Default|GetNearMaxDistanceSabotage))
      (if (== (Math|Random|RandomInteger 50) 0)
        (Development|PrintString "FROMJ ADminHIT actor is nearby!!!!!!!!!!!!!!")
        (Utilities|Array|Add _localactorsnearby _array_element))))
  (return _localactorsnearby))