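; Parent AI controller for RTS workers and AI opponents, holding a worker state, a desired location and opponent money.
; BeginPlay starts looping timers, three scaled by difficulty, then sets starting money, logged to the player's HUD.
; The movement tick moves the pawn without pathfinding by state, holding still while building, and draws a debug sphere.
; Construction functions trigger worker building or animation; attention, aggressive, defensive and spending functions are empty stubs.
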(event EventBeginPlay
  (bind _returnvalue (Pawn|GetControlledPawn))
  (Utilities|Time|SetTimerbyFunctionName 0 "TIMERBASED_AttentionTick" (Math|Float|Absolute(Float) (- (Math|Float|MakeLiteralFloat (Math|Random|RandomFloatinRange 1.1 1.5)) (Math|Float|Clamp(Float) (Variables|Default|GetDifficultyOfAI) -1e+01))) true)
  (Utilities|Time|SetTimerbyFunctionName 0 "TIMERBASED_MovementTick" 0.5 true)
  (Utilities|Time|SetTimerbyFunctionName 0 "TIMERBASED_AgressiveTick" (Math|Float|Absolute(Float) (- (Math|Float|MakeLiteralFloat (Math|Random|RandomFloatinRange 1.1 1.5)) (Math|Float|Clamp(Float) (Variables|Default|GetDifficultyOfAI) -1e+01))) true)
  (Utilities|Time|SetTimerbyFunctionName 0 "TIMERBASED_DefensiveTick" (Math|Float|Absolute(Float) (- (Math|Float|MakeLiteralFloat (Math|Random|RandomFloatinRange 1.1 1.5)) (Math|Float|Clamp(Float) (Variables|Default|GetDifficultyOfAI) -1e+01))) true)
  (Utilities|FlowControl|Delay 0.5)
  (CallFunction|RTSRPGSetMoney 200 -200)
  (Utilities|Casting|CastToBP_EBAIOpponent (Components|GetOwner _returnvalue)
    (:CastFailed
      (Utilities|IsValid _returnvalue
        (:Is%20Valid
          (CallFunction|SetDesiredLocation (Transformation|GetActorLocation _returnvalue)))))))

(event EventTick
  (params (DeltaSeconds :type Float%20%28single-precision%29)))

(fn ConstructionScript)

(fn AIBuildAConstruction
  (params (Construction :type BP%20Construction%20in%20Process%20Max%20Parent%20Class%20Object%20Reference))
  ;[1 1 1] This gets called whenever we get collision with a construction that we are going to build
  (Default|StartBuildingConstruction (.AsBP%20EBWorker (Utilities|Casting|CastToBP_EBWorker (Pawn|GetControlledPawn))) Construction)
  (AI|Navigation|MovetoLocation (Transformation|GetActorLocation (Pawn|GetControlledPawn)) -1.0 true true false true 0)
  (CallFunction|GotoStateAIWokerorWhataver "NewEnumerator2" (Variables|Default|GetAI_StateOfWorkerOrWhataver)))

(fn AIWorkonAConstruction
  ;[1 1 1] Construction when we work at it stop pawn and work
  (Default|StartPlayingAnimation (.AsBP%20EBWorker (Utilities|Casting|CastToBP_EBWorker (Pawn|GetControlledPawn))) "/Game/EB/Animations/AM_WorkingOrBuildingABuilding.AM_WorkingOrBuildingABuilding")
  (AI|Navigation|MovetoLocation (Transformation|GetActorLocation (Pawn|GetControlledPawn)) -1.0 true true false true 0))

(fn AIMovetoLandscape)

(fn TIMERBASEDAttentionTick)

(fn TIMERBASEDMovementTick
  (bind _desiredlocation (Variables|Default|GetDesiredLocation))
  (switch Utilities|FlowControl|Switch|SwitchonEN_StateOfWorker (Variables|Default|GetAI_StateOfWorkerOrWhataver)
    (:NewEnumerator0
      (AI|Navigation|MovetoLocation _desiredlocation -1.0 true false false true 0))
    (:NewEnumerator1
      (AI|Navigation|MovetoLocation _desiredlocation -1.0 true false false true 0))
    (:NewEnumerator2
      (AI|Navigation|MovetoLocation (Transformation|GetActorLocation (Pawn|GetControlledPawn)) -1.0 true false false true 0))
    (:NewEnumerator3
      (AI|Navigation|MovetoLocation _desiredlocation -1.0 true false false true 0)))
  (Rendering|Debug|DrawDebugSphere _desiredlocation 1e+01 12 "(R=0.000000,G=1.000000,B=0.349677,A=1.000000)" 1.0 1e+02)
  (bind _astsicharacter_max_parent_class_eb (Utilities|Casting|CastToTSICharacterMaxParentClassEB (Pawn|GetControlledPawn)))
  (if (== (Variables|/Game/EB/Blueprints/TSICharacterMaxParentClassEB.TSICharacterMaxParentClassEB_C|GetTeamNum _astsicharacter_max_parent_class_eb) 0)
    _))

(fn TIMERBASEDAgressiveTick)

(fn TIMERBASEDDefensiveTick)

(fn SetDesiredLocation
  (params (NewDesLoc :type Vector))
  (Variables|Default|SetDesiredLocation NewDesLoc))

(fn RTSRPGSetMoney
  (params (NewMoney :type Integer) (CostOrGanancy :type Integer))
  (bind _returnvalue (Game|GetPlayerController 0))
  (bind _output_get (Variables|Default|SetAIOPONENT_RPGMoney NewMoney))
  (if (< CostOrGanancy 0)
    ;[1 1 1] Looses money
    (bind _asbp_player_controller_rtsmax_par (Utilities|Casting|CastToBP_PlayerControllerRTSMaxPar _returnvalue))
    (bind _asbp_hudmax_parent_class (Utilities|Casting|CastToBP_HUDMaxParentClass (HUD|GetHUD _asbp_player_controller_rtsmax_par)))
    (Default|HUDLOGAddLogMessage _asbp_hudmax_parent_class (Utilities|String|Append "(name AI) spends " (Utilities|String|ToString(Integer) CostOrGanancy) "has now:" (Utilities|String|ToString(Integer) _output_get)) 2.0)
    (else
      ;[1 1 1] Earns money
      (bind _asbp_player_controller_rtsmax_par_2 (Utilities|Casting|CastToBP_PlayerControllerRTSMaxPar _returnvalue))
      (bind _asbp_hudmax_parent_class_2 (Utilities|Casting|CastToBP_HUDMaxParentClass (HUD|GetHUD _asbp_player_controller_rtsmax_par_2)))
      (Default|HUDLOGAddLogMessage _asbp_hudmax_parent_class_2 (Utilities|String|Append "(name) earns " (Utilities|String|ToString(Integer) NewMoney) "has now:" (Utilities|String|ToString(Integer) _output_get)) 2.0))))

(fn GotoStateAIWokerorWhataver
  (params (NewState :type EN_StateOfWorker%20Enum :default "NewEnumerator0") (PreviousState :type EN_StateOfWorker%20Enum :default "NewEnumerator0"))
  (Variables|Default|SetAI_StateOfWorkerOrWhataver NewState))

(fn MAXAISpendMoney
  (params (MToSpend :type Integer)))