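; Base bullet tracer projectile that moves, applies damage and alerts near-missed characters.
; On authority, Tick line-traces each step, damaging characters once, with random deflected pass-through, and targets; landscape, static meshes and foliage trigger impact effects and destruction.
; GetShotAtCollision overlaps send AI and player controllers the shooter's team, weapon and approximate position.
; A flag hides locally owned client tracers and skips hit handling; bounce and area-alert logic are disabled.
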(event OnComponentBeginOverlap(GetShotAtCollision)
  (params (OverlappedComponent :type Primitive%20Component%20Object%20Reference) (OtherActor :type Actor%20Object%20Reference) (OtherComp :type Primitive%20Component%20Object%20Reference) (OtherBodyIndex :type Integer) (bFromSweep :type Boolean) (SweepResult :type Hit%20Result%20Structure%20%28by%20ref%29))
  (bind _returnvalue (Components|GetOwner))
  (bind _returnvalue_2 (Components|GetOwner))
  (bind _returnvalue_3 (Components|GetOwner))
  (bind _returnvalue_4 (Math|Random|RandomFloatinRange -2e+02 2e+02))
  (bind _returnvalue_5 (Components|GetOwner))
  (bind _returnvalue_6 (!= _returnvalue_2 OtherActor))
  (bind _returnvalue_7 (Transformation|GetActorLocation _returnvalue_3))
  (bind _astsicharacter_max_parent_class_from_lsf (Utilities|Casting|CastToTSICharacterMaxParentClassFromLSF _returnvalue_5))
  (bind _returnvalue_8 (+ (.x _returnvalue_7) _returnvalue_4))
  (bind _returnvalue_9 (+ (.y _returnvalue_7) _returnvalue_4))
  (bind _inventoryreference (Variables|/Game/TSIBPTSICntnt/TSIBlueprints/Pawns/TSICharacterMaxParentClassFromLSF.TSICharacterMaxParentClassFromLSF_C|GetInventoryReference _astsicharacter_max_parent_class_from_lsf))
  (bind _returnvalue_10 (Math|Vector|MakeVector _returnvalue_8 _returnvalue_9 (.z _returnvalue_7)))
  (bind _primaryweapon (Variables|/Game/TSIBPTSICntnt/TSIBlueprints/Inventories/TSIInventoryMaxParentClass.TSIInventoryMaxParentClass_C|GetPrimaryWeapon _inventoryreference))
  (if (!= _returnvalue_3 0)
    (Utilities|IsValid _returnvalue_3
      (:Is%20Valid
        (Utilities|IsValid _inventoryreference
          (:Is%20Valid
            (Networking|SwitchHasAuthority
              (:Authority
                _)
              (:Remote
                _))
            (bind _astsicharacter_max_parent_class_from_lsf_2 (Utilities|Casting|CastToTSICharacterMaxParentClassFromLSF OtherActor))
            (Utilities|FlowControl|Sequence
              (:then_0
                (bind _astsiaicontroller_max_parent_class (Utilities|Casting|CastToTSIAIControllerMaxParentClass (Pawn|GetController _astsicharacter_max_parent_class_from_lsf_2)))
                (if _returnvalue_6
                  (bind _astsicharacter_max_parent_class_from_lsf_3 (Utilities|Casting|CastToTSICharacterMaxParentClassFromLSF _returnvalue))
                  (bind _astsiitem_fire_arm_max_par (Utilities|Casting|CastToTSIItemFireArmMaxPar _primaryweapon))
                  (Default|GetShotat _astsiaicontroller_max_parent_class (Math|Conversions|ToByte(Integer) (Variables|/Game/TSIBPTSICntnt/TSIBlueprints/Pawns/TSICharacterMaxParentClassFromLSF.TSICharacterMaxParentClassFromLSF_C|GetTeamNum _astsicharacter_max_parent_class_from_lsf_3)) _returnvalue_10 _astsiitem_fire_arm_max_par (Components|GetOwner))))
              (:then_1
                (bind _astsiplayer_controller (Utilities|Casting|CastToTSIPlayerController (Pawn|GetController _astsicharacter_max_parent_class_from_lsf_2)))
                (if _returnvalue_6
                  (bind _astsicharacter_max_parent_class_from_lsf_4 (Utilities|Casting|CastToTSICharacterMaxParentClassFromLSF _returnvalue))
                  (bind _astsiitem_fire_arm_max_par_2 (Utilities|Casting|CastToTSIItemFireArmMaxPar _primaryweapon))
                  (Default|GetShotat _astsiplayer_controller (Math|Conversions|ToByte(Integer) (Variables|/Game/TSIBPTSICntnt/TSIBlueprints/Pawns/TSICharacterMaxParentClassFromLSF.TSICharacterMaxParentClassFromLSF_C|GetTeamNum _astsicharacter_max_parent_class_from_lsf_4)) _returnvalue_10 _astsiitem_fire_arm_max_par_2))))))))))

(event EventDestroyed
  ;[1 1 1] A little bit after it got destrpoyed, safety here the cient bullets should automatically destroyed when hit the floor
  (Utilities|FlowControl|Delay 0.2))

(event Collision|EventActorBeginOverlap
  (params (OtherActor :type Actor%20Object%20Reference)))

(event EventTick
  (params (DeltaSeconds :type Float%20%28single-precision%29))
  (bind _returnvalue (Components|GetOwner))
  (bind _returnvalue_2 (Transformation|GetActorLocation))
  (bind _returnvalue_3 (Transformation|GetActorRotation))
  (bind _returnvalue_4 (Components|GetOwner))
  (bind _returnvalue_5 (Components|GetOwner))
  (bind _returnvalue_6 (Transformation|GetActorRotation))
  (bind _bulletspeed (Variables|Default|GetBulletSpeed))
  (bind _returnvalue_7 (Math|Rotator|GetRotationXVector _returnvalue_3))
  (bind _returnvalue_8 (* _bulletspeed DeltaSeconds))
  (bind _returnvalue_9 (* _returnvalue_7 _returnvalue_8))
  (bind _returnvalue_10 (+ _returnvalue_2 _returnvalue_9))
  (if (not (Variables|Default|GetbShouldStatNoAutoVelocity))
    (Networking|SwitchHasAuthority
      (:Authority
        (bind _outhits (Class|KismetSystemLibrary|LineTraceMultiforObjects (Transformation|GetActorLocation) _returnvalue_10 (Utilities|Array|MakeArray "ObjectTypeQuery3" "ObjectTypeQuery1" "ObjectTypeQuery2" "ObjectTypeQuery4") false 0 "None" true "(R=1.000000,G=0.000000,B=0.000000,A=1.000000)" "(R=0.000000,G=1.000000,B=0.000000,A=1.000000)" 1.0))
        (Utilities|FlowControl|Sequence
          (:then_0
            (Transformation|SetActorLocation _returnvalue_10 false false))
          (:then_1
            (bind _array_element (Utilities|Array|ForEachLoopwithBreak _outhits)
              (:LoopBody
                (if (not (Variables|Default|GetbShouldClientOwnerNoSeeNoEffects))
                  (Utilities|FlowControl|Sequence
                    (:then_0
                      (Utilities|Casting|CastToSkeletalMeshComponent (.HitComponent (Collision|BreakHitResult _array_element)))
                      (bind _ascharacter (Utilities|Casting|CastToCharacter (.HitActor (Collision|BreakHitResult _array_element))))
                      (if (!= _ascharacter _returnvalue)
                        (if (not (CallFunction|BAlreadyHitThisTarget _ascharacter))
                          (CallFunction|AddtoAlreadyHitActors _ascharacter)
                          (Utilities|FlowControl|Sequence
                            (:then_0
                              (bind _astsicharacter_max_parent_class_from_lsf (Utilities|Casting|CastToTSICharacterMaxParentClassFromLSF _ascharacter))
                              (Default|InterFunctTakeDamage _astsicharacter_max_parent_class_from_lsf "NewEnumerator0" _returnvalue_5 _array_element)
                              ;[1 1 1] Pass through bullet
                              (if (Math|Random|RandomBool)
                                (Transformation|SetActorRotation (Math|Rotator|MakeRotator (.roll _returnvalue_6) (+ (.pitch _returnvalue_6) (Math|Random|RandomFloatinRange -5.0 5.0)) (+ (.yaw _returnvalue_6) (Math|Random|RandomFloatinRange -5.0 5.0))))
                                (else
                                  ;[1 1 1] Char stops the bullet
                                  (Variables|Default|SetbHitAlreadyLand true)
                                  (CallFunction|DestroytheActor))))
                            (:then_1
                              (bind _astsicharacter_max_parent_class_eb (Utilities|Casting|CastToTSICharacterMaxParentClassEB _ascharacter))
                              (Class|IDamageInterface|InterFunctTakeDamage(Message) _astsicharacter_max_parent_class_eb "NewEnumerator0" _returnvalue_5 _array_element)
                              (Development|PrintString "FROM bulletworker hitting !!!!!!!!!!!!!!!!!!!!!!!!!!!!!!"))))))
                    (:then_1
                      ;[1 1 1] LANDSCAPE HERE
                      (if (not (Variables|Default|GetbHitAlreadyLand))
                        (Utilities|FlowControl|Sequence
                          (:then_0
                            (Utilities|Casting|CastToLandscape (.HitActor (Collision|BreakHitResult _array_element)))
                            (bind _astsicharacter_max_parent_class_from_lsf_2 (Utilities|Casting|CastToTSICharacterMaxParentClassFromLSF _returnvalue_4))
                            (Default|StartSpawningParticle _astsicharacter_max_parent_class_from_lsf_2 (Variables|Default|GetGroundParticle) (.Location (Collision|BreakHitResult _array_element)) "0, 0, 0")
                            (for _array_element_2 (CallFunction|GetAllActorsonBulletFloorExplosionandGetShotatCall 5e+02 (.Location (Collision|BreakHitResult _array_element)))
                              (bind _astsiaicontroller_max_parent_class (Utilities|Casting|CastToTSIAIControllerMaxParentClass _array_element_2))
                              (bind _aspawn (Utilities|Casting|CastToPawn _returnvalue_4))
                              (bind _astsicharacter_max_parent_class_from_lsf_3 (Utilities|Casting|CastToTSICharacterMaxParentClassFromLSF _aspawn))
                              (bind _astsiitem_fire_arm_max_par (Utilities|Casting|CastToTSIItemFireArmMaxPar (Variables|/Game/TSIBPTSICntnt/TSIBlueprints/Inventories/TSIInventoryMaxParentClass.TSIInventoryMaxParentClass_C|GetPrimaryWeapon (Variables|/Game/TSIBPTSICntnt/TSIBlueprints/Pawns/TSICharacterMaxParentClassFromLSF.TSICharacterMaxParentClassFromLSF_C|GetInventoryReference _astsicharacter_max_parent_class_from_lsf_3))))
                              (Utilities|IsValid (Variables|/Game/TSIBPTSICntnt/TSIBlueprints/Inventories/TSIInventoryMaxParentClass.TSIInventoryMaxParentClass_C|GetPrimaryWeapon (Variables|/Game/TSIBPTSICntnt/TSIBlueprints/Pawns/TSICharacterMaxParentClassFromLSF.TSICharacterMaxParentClassFromLSF_C|GetInventoryReference _astsicharacter_max_parent_class_from_lsf_3))
                                (:Is%20Valid
                                  (Default|GetShotat _astsiaicontroller_max_parent_class (Math|Conversions|ToByte(Integer) (Variables|/Game/TSIBPTSICntnt/TSIBlueprints/Pawns/TSICharacterMaxParentClassFromLSF.TSICharacterMaxParentClassFromLSF_C|GetTeamNum _astsicharacter_max_parent_class_from_lsf_3)) (Transformation|GetActorLocation _aspawn) _astsiitem_fire_arm_max_par _aspawn))))
                            ;[1 1 1] Imapct on floor
                            (Audio|PlaySoundatLocation "/Game/TSIBPTSICntnt/TSIAudio/FireArmSounds/FloorImpactSond.FloorImpactSond" (.Location (Collision|BreakHitResult _array_element)) "0, 0, 0" 1.0 1.0 0.0 0 0 0)
                            (Actor|DestroyActor))
                          (:then_1
                            (Utilities|Casting|CastToStaticMeshActor (.HitActor (Collision|BreakHitResult _array_element)))
                            (bind _astsicharacter_max_parent_class_from_lsf_4 (Utilities|Casting|CastToTSICharacterMaxParentClassFromLSF (Components|GetOwner)))
                            (Default|StartSpawningParticle _astsicharacter_max_parent_class_from_lsf_4 "/Game/TSIBPTSICntnt/TSIParticles/Particles/P_Explosion.P_Explosion" (.Location (Collision|BreakHitResult _array_element)) "0, 0, 0")
                            ;;[1 1 1] Here foreach all controllers Play Sound
                            (Audio|PlaySoundatLocation "/Game/TSIBPTSICntnt/TSIAudio/FireArmSounds/FloorImpactSond.FloorImpactSond" (.Location (Collision|BreakHitResult _array_element)) "0, 0, 0" 1.0 1.0 0.0 0 0 0)
                            (CallFunction|DestroytheActor))
                          (:then_2
                            (Utilities|Casting|CastToInstancedFoliageActor (.HitActor (Collision|BreakHitResult _array_element)))
                            (bind _astsicharacter_max_parent_class_from_lsf_5 (Utilities|Casting|CastToTSICharacterMaxParentClassFromLSF (Components|GetOwner)))
                            (Default|StartSpawningParticle _astsicharacter_max_parent_class_from_lsf_5 "/Game/TSIBPTSICntnt/TSIParticles/Particles/P_Explosion.P_Explosion" (.Location (Collision|BreakHitResult _array_element)) "0, 0, 0")
                            (CallFunction|DestroytheActor)))))
                    (:then_2
                      (bind _asbp_tsitarget_max_parent_class (Utilities|Casting|CastToBP_TSITargetMaxParentClass (.HitActor (Collision|BreakHitResult _array_element))))
                      (bind _bpenetrate (CallFunction|BPenetratesTarget _array_element))
                      (Default|ServerTakeDamageTarget _asbp_tsitarget_max_parent_class _array_element)
                      (bind _astsicharacter_max_parent_class_from_lsf_6 (Utilities|Casting|CastToTSICharacterMaxParentClassFromLSF _returnvalue))
                      (Default|StartSpawningParticle _astsicharacter_max_parent_class_from_lsf_6 "/Game/TSIBPTSICntnt/TSIParticles/Particles/P_Explosion.P_Explosion" (.Location (Collision|BreakHitResult _array_element)) "0, 0, 0")
                      (if _bpenetrate
                        (CallFunction|DestroytheActor)))))))))))))

(event EventBeginPlay
  (Utilities|FlowControl|Sequence
    (:then_0
      (Networking|SwitchHasAuthority
        (:Remote
          (bind _astsicharacter_max_parent_class_from_lsf (Utilities|Casting|CastToTSICharacterMaxParentClassFromLSF (Components|GetOwner)))
          (if (and (Variables|Default|GetbShouldClientOwnerNoSeeNoEffects) (Pawn|IsLocallyControlled _astsicharacter_max_parent_class_from_lsf))
            ;[1 1 1] Set no visibility if is client owner
            (Rendering|SetVisibility (Variables|Default|GetBulletTracer) false false)))))))

(fn ConstructionScript)

(fn DestroytheActor
  (Actor|DestroyActor))

(fn BPenetratesTarget
  (params (HitResult :type Hit%20Result%20Structure))
  (return (Math|Random|RandomBool)))

(fn StartSpawningParticle)

(fn HandleSpawnClientSideTracer
  (params (ActorTransform :type Transform))
  ;[1 1 1] Not sure if good
)

(fn BShallBouncefromLandscape
  (params (VecRot :type Vector) (Normal :type Vector))
  (return (Math|Random|RandomBool) (Math|Vector|MirrorVectorbyNormal VecRot Normal)))

(fn BAlreadyHitThisTarget
  (params (ActorToCheck :type Actor%20Object%20Reference))
  (return (Utilities|Array|ContainsItem (Variables|Default|GetHitActorArray) ActorToCheck)))

(fn AddtoAlreadyHitActors
  (params (ActorHIt :type Actor%20Object%20Reference))
  (bind _hitactorarray (Variables|Default|GetHitActorArray))
  ;[1 1 1] Just in case
  (if (not (Utilities|Array|ContainsItem _hitactorarray ActorHIt))
    (Utilities|Array|Add _hitactorarray ActorHIt)))

(fn GetAllActorsonBulletFloorExplosionandGetShotatCall
  (params (Radius :type Float%20%28single-precision%29) (HitLoc :type Vector))
  ;[1 1 1] Causes infinite loop and it is very expensive
)