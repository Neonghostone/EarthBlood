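; Campaign objective zone that spawns the saved garrison for its named location and shows that name on a locator widget, hidden at play start.
; On BeginPlay, the server reads the active campaign's save, matches the place name, caches the holding team and builds squad structs, also passed to attached spawners.
; Soldiers spawn at random landscape-traced points around the actor, each possessed by an AI controller and added to the leader's formation system.
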(event Custom|BeginOverlapUnsleeping
  (params (OverlappedComponent :type Primitive%20Component%20Object%20Reference) (OtherActor :type Actor%20Object%20Reference) (OtherComp :type Primitive%20Component%20Object%20Reference) (OtherBodyIndex :type Integer) (bFromSweep :type Boolean) (SweepResult :type Hit%20Result%20Structure%20%28by%20ref%29)))

(event Custom|SpawnTheCorrespondingSoldiers
  (bind _campaignssavegame (CallFunction|ReturntheSaveGameCampaigns))
  (Networking|SwitchHasAuthority
    (:Authority
      (switch Utilities|FlowControl|Switch|SwitchonEN_ListOfCampaigns (Variables|/Game/TSIBPTSICntnt/TSIBlueprints/SaveSystem/URSaveSystemCampaign.URSaveSystemCampaign_C|GetCampaignBeingPlayedIndex _campaignssavegame)
        (:NewEnumerator0
          (for (_array_element _array_index) (.LocationsObjectivesPlaces (Utilities|Struct|BreakSTRUCT_Campaign (Variables|/Game/TSIBPTSICntnt/TSIBlueprints/SaveSystem/URSaveSystemCampaign.URSaveSystemCampaign_C|GetBlitzgriegShieldCamp1Pgrs _campaignssavegame)))
            (if (not (> _array_index (Math|Conversions|ToInteger(Byte) (Variables|Default|GetRPGSoldiersAmountToSpawn))))
              ;[1 1 1] If the name of place is the one attached
              (if (Utilities|Enum|Equal(Enum) (Variables|Default|GetNameOfPlaceAttached) (.nameoflocobjplace _array_element))
                (Variables|Default|SetTeamNumCachedThatSpawnerIs (Utilities|Array|Get(acopy) (.teamholding _array_element)))
                (bind _finalstruct (CallFunction|GenerateStructwithSoldiersforSquad (.garrisoninit _array_element) (Variables|Default|GetTeamNumCachedThatSpawnerIs)))
                (CallFunction|SpawnSquadOfSoldiers _finalstruct (Variables|Default|GetTeamNumCachedThatSpawnerIs)))))
          ;[1 1 1] Spawn soldiers in attached spawners
          (for _array_element_2 (Variables|Default|GetAllSpawnersOfThisSpawner)
            (bind _finalstruct_2 (CallFunction|GenerateStructwithSoldiersforSquad (.garrisoninit _array_element) (Variables|Default|GetTeamNumCachedThatSpawnerIs)))
            (CallFunction|SpawnSquadOfSoldiers _array_element_2 _finalstruct_2 (Variables|Default|GetTeamNumCachedThatSpawnerIs))))
        (:NewEnumerator1
          (for (_array_element_3 _array_index_2) (.LocationsObjectivesPlaces (Utilities|Struct|BreakSTRUCT_Campaign (Variables|/Game/TSIBPTSICntnt/TSIBlueprints/SaveSystem/URSaveSystemCampaign.URSaveSystemCampaign_C|GetPlaceholderCamp2Pgrs _campaignssavegame)))
            (if (not (> _array_index_2 (Math|Conversions|ToInteger(Byte) (Variables|Default|GetRPGSoldiersAmountToSpawn))))
              ;[1 1 1] If the name of place is the one attached
              (if (Utilities|Enum|Equal(Enum) (Variables|Default|GetNameOfPlaceAttached) (.nameoflocobjplace _array_element_3))
                (Variables|Default|SetTeamNumCachedThatSpawnerIs (Utilities|Array|Get(acopy) (.teamholding _array_element_3)))
                (bind _finalstruct_3 (CallFunction|GenerateStructwithSoldiersforSquad (.garrisoninit _array_element_3) (Variables|Default|GetTeamNumCachedThatSpawnerIs)))
                (CallFunction|SpawnSquadOfSoldiers _finalstruct_3 (Variables|Default|GetTeamNumCachedThatSpawnerIs)))))
          ;[1 1 1] Spawn soldiers in attached spawners
          (for _array_element_4 (Variables|Default|GetAllSpawnersOfThisSpawner)
            (bind _finalstruct_4 (CallFunction|GenerateStructwithSoldiersforSquad (.garrisoninit _array_element_3) (Variables|Default|GetTeamNumCachedThatSpawnerIs)))
            (CallFunction|SpawnSquadOfSoldiers _array_element_4 _finalstruct_4 (Variables|Default|GetTeamNumCachedThatSpawnerIs))))))))

(event EventBeginPlay
  (|CallParentFunction)
  (Collision|BindEventtoOnComponentBeginOverlap (Variables|Default|GetPlaceAreaForUnsleepingAndSpawning) (delegate Custom|BeginOverlapUnsleeping))
  ;[1 1 1] Neongho: Check next frame
  (Utilities|FlowControl|Delay 0.0)
  (CallFunction|SpawntheCorrespondingSoldiers)
  (Rendering|SetVisibility (Variables|Default|GetToClickOnItWidget) false false))

(event Collision|EventActorBeginOverlap
  (params (OtherActor :type Actor%20Object%20Reference))
  (|CallParentFunction OtherActor))

(event EventTick
  (params (DeltaSeconds :type Float%20%28single-precision%29))
  (|CallParentFunction DeltaSeconds) ; This node is disabled and will not be called.\nDrag off pins to build functionality.
)

(fn ConstructionScript
  (|CallParentFunction)
  (bind _asuw_sooldier_rank_and_name_2or_place (Utilities|Casting|CastToUW_SooldierRankAndName2OrPlace (UserInterface|GetWidget (Variables|Default|GetLocationImageToClick))))
  (Rendering|Components|TextRender|SetText (Variables|/Game/TSIBPTSICntnt/TSIBlueprints/UMG/UMGWidgets/UW_SooldierRankAndName2OrPlace.UW_SooldierRankAndName2OrPlace_C|GetLocatorText _asuw_sooldier_rank_and_name_2or_place) (Utilities|Text|ToText(String) (Variables|Default|GetNameOfPlaceAttached))))

(fn ReturnValidRandomPlaceonSpawning)

(fn GetRandomPointinSphere
  (params (Center :type Vector) (Radius :type Float%20%28single-precision%29))
  (bind _returnvalue (* Radius -1.0))
  (bind _returnvalue_2 (* Radius -1.0))
  (bind _returnvalue_3 (Math|Random|RandomFloatinRange _returnvalue Radius))
  (bind _returnvalue_4 (Math|Random|RandomFloatinRange _returnvalue_2 Radius))
  (bind _returnvalue_5 (Math|Vector|MakeVector _returnvalue_4 _returnvalue_3 1e+06))
  (bind _returnvalue_6 (+ Center _returnvalue_5))
  (bind _outhits (Class|KismetSystemLibrary|LineTraceMultiforObjects _returnvalue_6 (+ _returnvalue_6 "0, 0,-100000000.000000") (Utilities|Array|MakeArray "ObjectTypeQuery1" "ObjectTypeQuery2") false 0 "None" true))
  (for _array_element _outhits
    (Utilities|Casting|CastToLandscape (.hitactor _array_element))
    (return (+ (.location _array_element) "0, 0,100.000000"))))

(fn SpawnSquadOfSoldiers
  (params (Squad :type STRUCT%20Squad%20Representation%20Structure) (Team :type Byte :default 0))
  (bind _returnvalue (Math|Conversions|ToInteger(Byte) Team))
  (bind _returnvalue_2 (Transformation|GetActorLocation))
  (bind _finalspawnlocinsphere (CallFunction|GetRandomPointinSphere _returnvalue_2 5e+02))
  (bind _returnvalue_3 (Math|Transform|MakeTransform _finalspawnlocinsphere))
  ;[1 1 1] Not redundancy as it uses sphere
  (bind (_array_element _array_index) (Utilities|Array|ForEachLoopwithBreak (Utilities|Struct|BreakSTRUCT_SquadRepresentation Squad))
    (:LoopBody
      (bind (_array_element_2 _array_index_2) (Utilities|Array|ForEachLoopwithBreak (.ftsoldiers _array_element))
        (:LoopBody
          (if (< _array_index_2 (Math|Conversions|ToInteger(Byte) (Variables|Default|GetRPGSoldiersAmountToSpawn)))
            (if (and (== _array_index 0) (== _array_index_2 0))
              ;;[1 1 1] Leader SL
              (bind _finalsoldier (CallFunction|SpawnSoldieratLocandRotandReturnIt _returnvalue_3 (.customofsoldier _array_element_2) _returnvalue (.soldiername _array_element_2) (.weaponsofsoldier _array_element_2) (Utilities|Select :Index Team :Option%200 0.0 :Option%201 0.0 :Option%202 0.0 :Option%203 0.0 :Option%204 0.0 :Option%205 0.0 :Option%206 0.0 :Option%207 0.0 :Option%208 0.0 :Option%209 0.0 :Option%2010 (CallFunction|TranslateDifficultyfromEnum (CallFunction|GetActualDifficultybyGamemodeandSaveData) true) :Option%2011 (CallFunction|TranslateDifficultyfromEnum (CallFunction|GetActualDifficultybyGamemodeandSaveData) false))))
              (bind _returnvalue_4 (Game|SpawnActorfromClass "/Game/TSIBPTSICntnt/TSIBlueprints/AIControllerClasses/TSIAIControllerMaxParentClass.TSIAIControllerMaxParentClass_C" (Transformation|GetActorTransform _finalsoldier) "AdjustIfPossibleButAlwaysSpawn" 0 "0.000000,0.000000,0.000000" "0.000000,0.000000,0.000000" 0 "None" 0))
              (Pawn|Possess _returnvalue_4 _finalsoldier)
              (bind _returnvalue_5 (Game|SpawnActorfromClass "/Game/TSIBPTSICntnt/TSIBlueprints/FormationSystem/FormationSystemOfLeader.FormationSystemOfLeader_C" (Math|Transform|MakeTransform "0, 0, 0") "AdjustIfPossibleButAlwaysSpawn" _finalsoldier _finalsoldier _finalsoldier 0 0 _finalsoldier))
              (Variables|/Game/TSIBPTSICntnt/TSIBlueprints/Pawns/TSICharacterMaxParentClassFromLSF.TSICharacterMaxParentClassFromLSF_C|SetFormationInfo _finalsoldier _returnvalue_5)
              (LocalVariables|SetLocalLeaderFI _returnvalue_5)
              (Variables|/Game/TSIBPTSICntnt/TSIBlueprints/FormationSystem/FormationSystemOfLeader.FormationSystemOfLeader_C|SetUnitStruct _returnvalue_5 (Utilities|Struct|MakeSTRUCT_UnitActualFormationn _finalsoldier (Utilities|Array|MakeArray)))
              (Default|AddNewMemberCreatingGroup (LocalVariables|GetLocalLeaderFI) _finalsoldier 0 "Alpha")
              (else
                ;;[1 1 1] Normal
                (bind _finalsoldier_2 (CallFunction|SpawnSoldieratLocandRotandReturnIt _returnvalue_3 (.customofsoldier _array_element_2) _returnvalue (.soldiername _array_element_2) (.weaponsofsoldier _array_element_2) (Utilities|Select :Index Team :Option%200 0.0 :Option%201 0.0 :Option%202 0.0 :Option%203 0.0 :Option%204 0.0 :Option%205 0.0 :Option%206 0.0 :Option%207 0.0 :Option%208 0.0 :Option%209 0.0 :Option%2010 (CallFunction|TranslateDifficultyfromEnum (CallFunction|GetActualDifficultybyGamemodeandSaveData) true) :Option%2011 (CallFunction|TranslateDifficultyfromEnum (CallFunction|GetActualDifficultybyGamemodeandSaveData) false))))
                (bind _returnvalue_6 (Game|SpawnActorfromClass "/Game/TSIBPTSICntnt/TSIBlueprints/AIControllerClasses/TSIAIControllerMaxParentClass.TSIAIControllerMaxParentClass_C" (Transformation|GetActorTransform _finalsoldier_2) "AdjustIfPossibleButDontSpawnIfColliding" 0 "0.000000,0.000000,0.000000" "0.000000,0.000000,0.000000" 0 "None" 0))
                (Pawn|Possess _returnvalue_6 _finalsoldier_2)
                (if (> _array_index_2 5)
                  _
                  (else
                    _))
                (Default|AddNewMemberCreatingGroup (LocalVariables|GetLocalLeaderFI) _finalsoldier_2 (Math|Conversions|ToByte(Integer) _array_index) "Alpha")))))))))