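; Parent soldier spawner that creates Green Beret (team 10) and enemy (team 11) AI troops singly, as ghost teams or as squads.
; Placement uses forward offsets or random box points, with squad spawns traced down onto Landscape.
; Squad spawning randomizes loadouts and customization, possesses soldiers with AI controllers and registers them in the leader's formation actor.
; Box and squad spawns randomize AI difficulty by side, using campaign save difficulty in open-world mode.
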(event Custom|SpawnGhostTeam
  (params (TeamOfGhosts :type Byte))
  ;[1 1 1] Attention the individuals are spawned from Ghost arena game info
  (bind _returnvalue (SaveGame|LoadGamefromSlot "campaigns"))
  (bind _asursave_system_campaign (Utilities|Casting|CastToURSaveSystemCampaign _returnvalue))
  ;;[1 1 1] Spawn the Team 10 soldiers berets
  (switch int (Math|Conversions|ToInteger(Byte) TeamOfGhosts)
    (:10
      (for (_array_element _array_index) (Variables|Default|GetAllSpawnersOfThisSpawner)
        (bind _spawnedsoldier (CallFunction|SpawnSoldierandReturnIt _array_element 10 (Math|Conversions|ToByte(Integer) _array_index)))
        (bind _returnvalue_2 (Game|SpawnActorfromClass "/Game/TSIBPTSICntnt/TSIBlueprints/AIControllerClasses/TSIAIControllerMaxParentClass.TSIAIControllerMaxParentClass_C" (Transformation|GetActorTransform _spawnedsoldier) "AdjustIfPossibleButAlwaysSpawn" 0 "0.000000,0.000000,0.000000" "0.000000,0.000000,0.000000" 0 (Utilities|String|StringToName (Variables|/Game/TSIBPTSICntnt/TSIBlueprints/Pawns/TSICharacterMaxParentClassFromLSF.TSICharacterMaxParentClassFromLSF_C|GetSoldierName _spawnedsoldier)) 0))
        (Pawn|Possess _returnvalue_2 _spawnedsoldier)))
    (:11
      ;;[1 1 1] Spawnb the team 11 Fascits soldiers
      (for (_array_element_2 _array_index_2) (Variables|Default|GetAllSpawnersOfThisSpawner)
        (bind _spawnedsoldier_2 (CallFunction|SpawnSoldierandReturnIt _array_element_2 11 (Math|Conversions|ToByte(Integer) _array_index_2)))
        (Game|SpawnActorfromClass "/Game/TSIBPTSICntnt/TSIBlueprints/AIControllerClasses/TSIAIControllerMaxParentClass.TSIAIControllerMaxParentClass_C" (Transformation|GetActorTransform _spawnedsoldier_2) "AdjustIfPossibleButAlwaysSpawn" 0 "0.000000,0.000000,0.000000" "0.000000,0.000000,0.000000" 0 (Utilities|String|StringToName (Variables|/Game/TSIBPTSICntnt/TSIBlueprints/Pawns/TSICharacterMaxParentClassFromLSF.TSICharacterMaxParentClassFromLSF_C|GetSoldierName _spawnedsoldier_2)) 0)))))

(event Custom|GoToStateSpawner
  (params (NewState :type EN_StateOfSpawner%20Enum :default "NewEnumerator0") (PreviousState :type EN_StateOfSpawner%20Enum :default "NewEnumerator0"))
  (Variables|Default|SetStateOFSpawner NewState))

(event EventBeginPlay
  ;[1 1 1] Attention the individuals are spawned from Ghost arena game info
  (Rendering|SetVisibility (Variables|Default|GetToClickOnItWidget) false false))

(event Collision|EventActorBeginOverlap
  (params (OtherActor :type Actor%20Object%20Reference))
  ;[1 1 1] Attention the individuals are spawned from Ghost arena game info
)

(event EventTick
  (params (DeltaSeconds :type Float%20%28single-precision%29))
  ;[1 1 1] Attention the individuals are spawned from Ghost arena game info
)

(fn ConstructionScript)

(fn SpawnSoldierandReturnIt
  (params (TeamNum :type Byte) (SoldierNum :type Byte) (NameOfControllerForSold :type String))
  (bind _returnvalue (Transformation|GetActorTransform))
  (bind _returnvalue_2 (Math|Conversions|ToInteger(Byte) TeamNum))
  (bind _returnvalue_3 (Transformation|GetActorRotation))
  (bind _returnvalue_4 (+ SoldierNum 1))
  (bind _returnvalue_5 (Math|Conversions|ToInteger(Byte) _returnvalue_4))
  (bind _returnvalue_6 (Math|Rotator|GetRotationXVector _returnvalue_3))
  (bind _returnvalue_7 (* _returnvalue_5 300))
  (bind _returnvalue_8 (Math|Conversions|ToFloat(Integer) _returnvalue_7))
  (bind _returnvalue_9 (* _returnvalue_6 _returnvalue_8))
  (bind _returnvalue_10 (+ (.location _returnvalue) _returnvalue_9))
  (bind _returnvalue_11 (Math|Transform|MakeTransform _returnvalue_10))
  (switch int _returnvalue_2
    (:10
      (bind _returnvalue_12 (Game|SpawnActorfromClass :Class "/Game/TSIBPTSICntnt/TSIBlueprints/Pawns/TSICharHighQLGreenBeret.TSICharHighQLGreenBeret_C" :SpawnTransform _returnvalue_11 :CollisionHandlingOverride "Undefined" :TeamNum _returnvalue_2 :Instigator 0))
      (Variables|/Game/TSIBPTSICntnt/TSIBlueprints/Pawns/TSICharacterMaxParentClassFromLSF.TSICharacterMaxParentClassFromLSF_C|SetSoldierName _returnvalue_12 "FROM SPAWNER SpawnSOldierReturn() It 
 detect the controller and set it as ")
      ;[1 1 1] Add it into the map foreach controller
      (bind _outactors (Actor|GetAllActorsOfClass "/Game/TSIBPTSICntnt/TSIBlueprints/PlayerControllers/TSIPlayerController.TSIPlayerController_C"))
      (for _array_element _outactors
        _)
      (return _returnvalue_12))
    (:11
      (bind _returnvalue_13 (Game|SpawnActorfromClass :Class "/Game/TSIBPTSICntnt/TSIBlueprints/Pawns/TSIDimitry.TSIDimitry_C" :SpawnTransform _returnvalue_11 :CollisionHandlingOverride "Undefined" :TeamNum _returnvalue_2 :Instigator 0))
      (Variables|/Game/TSIBPTSICntnt/TSIBlueprints/Pawns/TSICharacterMaxParentClassFromLSF.TSICharacterMaxParentClassFromLSF_C|SetSoldierName _returnvalue_13 "FROM SPAWNER SpawnSOldierReturn() Placeholder detect the controller and set it as ")
      ;[1 1 1] Add it into the map foreach controller
      (bind _outactors_2 (Actor|GetAllActorsOfClass "/Game/TSIBPTSICntnt/TSIBlueprints/PlayerControllers/TSIPlayerController.TSIPlayerController_C"))
      (for _array_element_2 _outactors_2
        _)
      (return _returnvalue_13))))

(fn FunctSpawnGhostTeambyFunct
  (params (TeamNum :type Byte))
  (bind _spawnedsoldiers (LocalVariables|GetSpawnedSoldiers))
  (bind _spawnedsoldiers_2 (LocalVariables|GetSpawnedSoldiers))
  (switch int (Math|Conversions|ToInteger(Byte) TeamNum)
    (:10
      ;[1 1 1] Spawn the Team 10 soldiers berets
      (for _index (range 0 8)
        (bind _spawnedsoldier (CallFunction|SpawnSoldierandReturnIt 10 (Math|Conversions|ToByte(Integer) _index)))
        (Utilities|Array|Add _spawnedsoldiers_2 _spawnedsoldier))
      (return _spawnedsoldiers_2))
    (:11
      ;[1 1 1] Spawnb the team 11 Fascits soldiers
      (for _index_2 (range 0 8)
        (bind _spawnedsoldier_2 (CallFunction|SpawnSoldierandReturnIt 11 (Math|Conversions|ToByte(Integer) _index_2)))
        (Utilities|Array|Add _spawnedsoldiers _spawnedsoldier_2))
      (return _spawnedsoldiers))))

(fn SpawnSoldierandReturnItBox
  (params (TeamNum :type Byte) (SoldierNum :type Byte) (NameOfControllerForSold :type String) (CUSTOMIZATION :type STRUCT%20Customization%20for%20Character%20Structure) (CustomWeapons :type Array%20of%20STRUCT%20Saved%20Item%20Structures))
  (bind _returnvalue (Math|Conversions|ToInteger(Byte) TeamNum))
  (bind _returnvalue_2 (Transformation|GetActorLocation))
  (bind _spawningcollisionbox (Variables|Default|GetSpawningCollisionBox))
  (bind _boxextent (Variables|/Script/Engine.BoxComponent|GetBoxExtent _spawningcollisionbox))
  (bind _returnvalue_3 (Math|Random|RandomPointinBoundingBox _returnvalue_2 _boxextent))
  (bind _returnvalue_4 (Math|Transform|MakeTransform _returnvalue_3))
  (switch int _returnvalue
    (:10
      (bind _returnvalue_5 (Game|SpawnActorfromClass "/Game/TSIBPTSICntnt/TSIBlueprints/Pawns/TSICharHighQLGreenBeret.TSICharHighQLGreenBeret_C" _returnvalue_4 "Undefined" 0 false _returnvalue "" (CallFunction|TranslateDifficultyfromEnum (CallFunction|GetActualDifficultybyGamemodeandSaveData) true) CustomWeapons false "NewEnumerator2" CUSTOMIZATION false false 0))
      (Variables|/Game/TSIBPTSICntnt/TSIBlueprints/Pawns/TSICharacterMaxParentClassFromLSF.TSICharacterMaxParentClassFromLSF_C|SetSoldierName _returnvalue_5 NameOfControllerForSold)
      ;[1 1 1] Add it into the map foreach controller
      (bind _outactors (Actor|GetAllActorsOfClass "/Game/TSIBPTSICntnt/TSIBlueprints/PlayerControllers/TSIPlayerController.TSIPlayerController_C"))
      (for _array_element _outactors
        _)
      (return _returnvalue_5))
    (:11
      (bind _returnvalue_6 (Game|SpawnActorfromClass "/Game/TSIBPTSICntnt/TSIBlueprints/Pawns/TSIDimitry.TSIDimitry_C" _returnvalue_4 "Undefined" 0 true _returnvalue "nazi" (CallFunction|TranslateDifficultyfromEnum (CallFunction|GetActualDifficultybyGamemodeandSaveData) false) CustomWeapons false "NewEnumerator2" CUSTOMIZATION true false 0))
      (Variables|/Game/TSIBPTSICntnt/TSIBlueprints/Pawns/TSICharacterMaxParentClassFromLSF.TSICharacterMaxParentClassFromLSF_C|SetSoldierName _returnvalue_6 NameOfControllerForSold)
      ;[1 1 1] Add it into the map foreach controller
      (bind _outactors_2 (Actor|GetAllActorsOfClass "/Game/TSIBPTSICntnt/TSIBlueprints/PlayerControllers/TSIPlayerController.TSIPlayerController_C"))
      (for _array_element_2 _outactors_2
        _)
      (return _returnvalue_6))))

(fn ReturntheSaveGameCampaigns
  (bind _returnvalue (SaveGame|LoadGamefromSlot "campaigns"))
  (Utilities|IsValid _returnvalue
    (:Is%20Valid
      (bind _asursave_system_campaign (Utilities|Casting|CastToURSaveSystemCampaign _returnvalue))
      (return _asursave_system_campaign))
    (:Is%20Not%20Valid
      (bind _outactors (Actor|GetAllActorsOfClass "/Game/TSIBPTSICntnt/TSIBlueprints/PlayerControllers/TSIPlayerController.TSIPlayerController_C"))
      (Default|AddLeftUpSideMessage _outactors "ERROR(ArealSpawner) Save game is not valid" 2.0)
      (return 0))))

(fn SpawnSoldieratLocandRotandReturnIt
  (params (SpawningLocRotAndScale :type Transform) (CharCustom :type STRUCT%20Customization%20for%20Character%20Structure) (Team :type Integer) (NameOfSoldier :type String) (ItemsForSoldier :type Array%20of%20STRUCT%20Saved%20Item%20Structures) (Difficulty :type Float%20%28single-precision%29))
  (bind _returnvalue (Game|SpawnActorfromClass (CallFunction|ReturnSoldierClassbyTeam (Math|Conversions|ToByte(Integer) Team)) SpawningLocRotAndScale "AdjustIfPossibleButAlwaysSpawn" 0 true Team NameOfSoldier Difficulty ItemsForSoldier false "NewEnumerator2" CharCustom true false 0))
  (return _returnvalue))

(fn ReturnSoldierClassbyTeam
  (params (Team :type Byte))
  (switch int (Math|Conversions|ToInteger(Byte) Team)
    (:0
      _)
    (:1
      _)
    (:2
      _)
    (:3
      _)
    (:10
      _)
    (:11
      (return "/Game/TSIBPTSICntnt/TSIBlueprints/Pawns/TSICharHighQLCommonEnemy.TSICharHighQLCommonEnemy_C")))
  (return "/Game/TSIBPTSICntnt/TSIBlueprints/Pawns/TSICharHighQLGreenBeret.TSICharHighQLGreenBeret_C"))

(fn SpawnSquadOfSoldiers
  (params (Squad :type STRUCT%20Squad%20Representation%20Structure) (Team :type Byte))
  (bind (_weaponsofsoldier _charsoldiercustom) (CallFunction|GenerateRandomCustomizationandWeaponsPerSoldier Team))
  (bind _returnvalue (Math|Conversions|ToInteger(Byte) Team))
  (bind _returnvalue_2 (Transformation|GetActorLocation))
  (bind _diff (CallFunction|GetActualDifficultybyGamemodeandSaveData))
  (bind _diff_2 (CallFunction|GetActualDifficultybyGamemodeandSaveData))
  (bind _newdiffi (CallFunction|TranslateDifficultyfromEnum _diff false))
  (bind _newdiffi_2 (CallFunction|TranslateDifficultyfromEnum _diff_2 true))
  (bind _finalspawnlocinsphere (CallFunction|GetRandomPointinBox _returnvalue_2))
  (bind _returnvalue_3 (Math|Transform|MakeTransform _finalspawnlocinsphere))
  (bind _returnvalue_4 (Utilities|Select :Index Team :Option%200 0.0 :Option%201 0.0 :Option%202 0.0 :Option%203 0.0 :Option%204 0.0 :Option%205 0.0 :Option%206 0.0 :Option%207 0.0 :Option%208 0.0 :Option%209 0.0 :Option%2010 _newdiffi_2 :Option%2011 _newdiffi))
  ;[1 1 1] REDUNDANCY should be in max parent class rewrite this
  (bind (_array_element _array_index) (Utilities|Array|ForEachLoopwithBreak (Utilities|Struct|BreakSTRUCT_SquadRepresentation Squad))
    (:LoopBody
      (bind (_array_element_2 _array_index_2) (Utilities|Array|ForEachLoopwithBreak (.ftsoldiers _array_element))
        (:LoopBody
          (if (< _array_index_2 (Math|Conversions|ToInteger(Byte) (Variables|Default|GetRPGSoldiersAmountToSpawn)))
            (if (and (== _array_index 0) (== _array_index_2 0))
              ;;[1 1 1] Leader SL
              (bind _finalsoldier (CallFunction|SpawnSoldieratLocandRotandReturnIt _returnvalue_3 _charsoldiercustom _returnvalue (.soldiername _array_element_2) _weaponsofsoldier _returnvalue_4))
              (bind _returnvalue_5 (Game|SpawnActorfromClass "/Game/TSIBPTSICntnt/TSIBlueprints/AIControllerClasses/TSIAIControllerMaxParentClass.TSIAIControllerMaxParentClass_C" (Transformation|GetActorTransform _finalsoldier) "AdjustIfPossibleButAlwaysSpawn" 0 "0.000000,0.000000,0.000000" "0.000000,0.000000,0.000000" 0 "None" _finalsoldier))
              (Pawn|Possess _returnvalue_5 _finalsoldier)
              (bind _returnvalue_6 (Game|SpawnActorfromClass "/Game/TSIBPTSICntnt/TSIBlueprints/FormationSystem/FormationSystemOfLeader.FormationSystemOfLeader_C" (Math|Transform|MakeTransform "0, 0, 0") "AdjustIfPossibleButAlwaysSpawn" _finalsoldier _finalsoldier _finalsoldier 0 0 _finalsoldier))
              (Variables|/Game/TSIBPTSICntnt/TSIBlueprints/Pawns/TSICharacterMaxParentClassFromLSF.TSICharacterMaxParentClassFromLSF_C|SetFormationInfo _finalsoldier _returnvalue_6)
              (LocalVariables|SetLocalLeaderFI _returnvalue_6)
              (Variables|/Game/TSIBPTSICntnt/TSIBlueprints/FormationSystem/FormationSystemOfLeader.FormationSystemOfLeader_C|SetUnitStruct _returnvalue_6 (Utilities|Struct|MakeSTRUCT_UnitActualFormationn _finalsoldier (Utilities|Array|MakeArray)))
              (Default|AddNewMemberCreatingGroup (LocalVariables|GetLocalLeaderFI) _finalsoldier 0 "Alpha")
              (else
                ;;[1 1 1] Normal
                (bind _finalsoldier_2 (CallFunction|SpawnSoldieratLocandRotandReturnIt _returnvalue_3 _charsoldiercustom _returnvalue (.soldiername _array_element_2) _weaponsofsoldier _returnvalue_4))
                (bind _returnvalue_7 (Game|SpawnActorfromClass "/Game/TSIBPTSICntnt/TSIBlueprints/AIControllerClasses/TSIAIControllerMaxParentClass.TSIAIControllerMaxParentClass_C" (Transformation|GetActorTransform _finalsoldier_2) "AdjustIfPossibleButAlwaysSpawn" 0 "0.000000,0.000000,0.000000" "0.000000,0.000000,0.000000" 0 "None" _finalsoldier_2))
                (Pawn|Possess _returnvalue_7 _finalsoldier_2)
                (Default|AddNewMemberCreatingGroup (LocalVariables|GetLocalLeaderFI) _finalsoldier_2 (Math|Conversions|ToByte(Integer) _array_index) "Alpha")))))))))

(fn GenerateStructwithSoldiersforSquad
  (params (Soldiers :type Array%20of%20Names) (TeamNum :type Byte))
  (bind (_weaponsofsoldier _charsoldiercustom) (CallFunction|GenerateRandomCustomizationandWeaponsPerSoldier TeamNum))
  (bind _localsquad (LocalVariables|GetLocalSquad))
  (bind _groups (Utilities|Struct|BreakSTRUCT_SquadRepresentation _localsquad))
  (Utilities|Array|AddUnique _groups (Utilities|Struct|MakeSTRUCT_SquadRepresentationFireteam "AlphaOneFL"))
  (bind _array_element (Utilities|Array|ForEachLoopwithBreak Soldiers)
    (:LoopBody
      (Utilities|Array|AddUnique (.FTSoldiers (Utilities|Struct|BreakSTRUCT_SquadRepresentationFireteam (Utilities|Array|Get(acopy) _groups))) (Utilities|Struct|MakeSTRUCT_SquadRepresentationSoldier (Utilities|String|ToString(Name) _array_element) false _weaponsofsoldier _charsoldiercustom TeamNum)))
    (:Completed
      (return _localsquad))))

(fn GetRandomPointinBox
  (params (Location :type Vector))
  (bind _spawningcollisionbox (Variables|Default|GetSpawningCollisionBox))
  (bind _boxextent (Variables|/Script/Engine.BoxComponent|GetBoxExtent _spawningcollisionbox))
  (bind _returnvalue (Math|Random|RandomPointinBoundingBox Location _boxextent))
  (bind _outhits (Class|KismetSystemLibrary|LineTraceMultiforObjects _returnvalue (+ _returnvalue "0, 0,-100000000.000000") (Utilities|Array|MakeArray "ObjectTypeQuery1" "ObjectTypeQuery2") false 0 "None" true))
  (for _array_element _outhits
    (Utilities|Casting|CastToLandscape (.hitactor _array_element))
    (return (+ (.location _array_element) "0, 0,100.000000"))))

(fn GenerateRandomCustomizationandWeaponsPerSoldier
  (params (TeamNum :type Byte))
  ;[1 1 1] WIP Can be used
  (return (Utilities|Select :Index TeamNum :Option%200 0 :Option%201 0 :Option%202 0 :Option%203 0 :Option%204 0 :Option%205 0 :Option%206 0 :Option%207 0 :Option%208 0 :Option%209 0 :Option%2010 (Utilities|Array|MakeArray (Utilities|Struct|MakeSTRUCT_SavedItem 0 0 "/Game/TSIBPTSICntnt/TSIBlueprints/Items/FireArms/Rifles/WeaponsFromMarketPlaceAndInuse/TSIArchetypeRifleM16A4New.TSIArchetypeRifleM16A4New_C")) :Option%2011 (Utilities|Array|MakeArray (Utilities|Struct|MakeSTRUCT_SavedItem 0 0 "/Game/TSIBPTSICntnt/TSIBlueprints/Items/FireArms/Rifles/OldWeapons/TSIArchetypeAK74.TSIArchetypeAK74_C"))) (Utilities|Select :Index TeamNum :Option%200 "" :Option%201 "" :Option%202 "" :Option%203 "" :Option%204 "" :Option%205 "" :Option%206 "" :Option%207 "" :Option%208 "" :Option%209 "" :Option%2010 (Utilities|Struct|MakeSTRUCT_CustomizationForCharacter "NewEnumerator0" "NewEnumerator0" "(R=1.000000,G=1.000000,B=1.000000,A=1.000000)" "(0.000000,0.000000,0.000000,0.000000,0.000000)" 0.0 0.8 0.0 0.0 0.0 0.0 "NewEnumerator0" "NewEnumerator0" "NewEnumerator0" "NewEnumerator0" "NewEnumerator0" "NewEnumerator2") :Option%2011 (Utilities|Struct|MakeSTRUCT_CustomizationForCharacter "NewEnumerator0" "NewEnumerator0" "(R=1.000000,G=1.000000,B=1.000000,A=1.000000)" "(0.000000,0.000000,0.000000,0.000000,0.000000)" 0.0 0.8 0.0 0.0 0.0 0.0 "NewEnumerator0" (.OutItem (Utilities|Array|Random (Utilities|Array|MakeArray "NewEnumerator1" "NewEnumerator1" "NewEnumerator0"))) (.OutItem (Utilities|Array|Random (Utilities|Array|MakeArray "NewEnumerator0" "NewEnumerator1" "NewEnumerator2"))) (.OutItem (Utilities|Array|Random (Utilities|Array|MakeArray "NewEnumerator4" "NewEnumerator2" "NewEnumerator1" "NewEnumerator0" "NewEnumerator0" "NewEnumerator0"))) "NewEnumerator0" (.OutItem (Utilities|Array|Random (Utilities|Array|MakeArray "NewEnumerator5" "NewEnumerator4" "NewEnumerator5" "NewEnumerator3" "NewEnumerator1" "NewEnumerator1" "NewEnumerator5" "NewEnumerator0" "NewEnumerator5" "NewEnumerator1" "NewEnumerator1")))))))

(fn GetActualDifficultybyGamemodeandSaveData
  (Utilities|Casting|CastToTSIGameInfoOpenWorldMPMaxPar (Game|GetGameMode)
    (:then
      (bind _returnvalue (SaveGame|LoadGamefromSlot "campaigns"))
      (bind _asursave_system_campaign (Utilities|Casting|CastToURSaveSystemCampaign _returnvalue))
      (return (Default|GetDifficultybyActiveCampaign _asursave_system_campaign)))
    (:CastFailed
      (return "NewEnumerator0"))))

(fn TranslateDifficultyfromEnum
  (params (EnDiffi :type EN_Difficulty%20Enum :default "NewEnumerator0") (bYourTeam :type Boolean))
  (bind _returnvalue (Math|Random|RandomFloatinRange 0.5 1.0))
  (bind _returnvalue_2 (Math|Random|RandomFloatinRange -2.0 0.0))
  (bind _returnvalue_3 (Math|Random|RandomFloatinRange 0.0 0.5))
  ;[1 1 1] PARAM Your team not used, yet
  (switch Utilities|FlowControl|Switch|SwitchonEN_Difficulty EnDiffi
    (:NewEnumerator0
      (if bYourTeam
        (return _returnvalue)
        (else
          (return _returnvalue_2))))
    (:NewEnumerator1
      (if bYourTeam
        (return _returnvalue_3)
        (else
          (return _returnvalue_3))))
    (:NewEnumerator2
      (if bYourTeam
        (return _returnvalue_2)
        (else
          (return _returnvalue))))))