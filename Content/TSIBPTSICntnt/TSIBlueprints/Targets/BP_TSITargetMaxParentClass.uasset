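; Parent Blueprint for targets that get knocked down when damaged.
; TakeDamageTarget passes its hit result to GetDown, which yaws the actor to the inverse of the hit normal, pitches it to -90 degrees and calls TargetDown.
; The fall is an instant rotation snap, with an unused LerpRotator and disconnected debug print left in the graph.
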(event Custom|TakeDamageTarget
  (params (HitResult :type Hit%20Result%20Structure))
  (CallFunction|GetDown HitResult))

(event Custom|GetDown
  (params (HitResult :type Hit%20Result%20Structure))
  (bind _returnvalue (Transformation|GetActorRotation))
  (Transformation|SetActorRotation (Math|Rotator|MakeRotator 0.0 0.0 (.yaw (Math|Conversions|RotationFromXVector (* (.Normal (Collision|BreakHitResult HitResult)) -1)))))
  (Transformation|SetActorRotation (Math|Rotator|MakeRotator (.roll _returnvalue) -9e+01 (.yaw _returnvalue)))
  (Default|CallTargetDown))

(event EventBeginPlay)

(event Collision|EventActorBeginOverlap
  (params (OtherActor :type Actor%20Object%20Reference)))

(event EventTick
  (params (DeltaSeconds :type Float%20%28single-precision%29)))

(fn ConstructionScript)