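; Pawn component for the world compass system that gives a player an on-screen compass and POI discovery messages.
; After a short BeginPlay delay, locally controlled player pawns create the compass widget with a north offset and start a looping timer.
; The timer rebuilds AllPOIs from BP_MasterPOI actors overlapping the owner.
; Client_FoundPOI shows a discovery widget with the POI's name for types removed after discovery.
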(event Custom|Client_FoundPOI
  (params (POI :type BP%20Master%20POI%20Object%20Reference))
  ;[1 1 1] Show HUD message when a Unknown POI is reached to indicate player discovered it
  (switch Utilities|FlowControl|Switch|SwitchonE_CompassPOI_Type (Variables|/Game/WorldCompassSystem/Blueprints/BP_MasterPOI.BP_MasterPOI_C|GetType POI)
    (:NewEnumerator0
      (bind _returnvalue (UserInterface|CreateWidget "/Game/WorldCompassSystem/Blueprints/WB_POI_Discovered.WB_POI_Discovered_C" 0 (Variables|/Game/WorldCompassSystem/Blueprints/BP_MasterPOI.BP_MasterPOI_C|GetName POI)))
      (UserInterface|Viewport|AddtoViewport _returnvalue 0))))

(event Custom|Client_CreateCompassWidget
  ;[1 1 1] Create and add compass to players screen
  (bind _returnvalue (UserInterface|CreateWidget "/Game/WorldCompassSystem/Blueprints/WB_Compass.WB_Compass_C" 0 (Variables|Public|GetNorth%20Direction%20Offset)))
  (UserInterface|Viewport|AddtoViewport _returnvalue 0))

(event EventBeginPlay
  (Utilities|FlowControl|Delay 2.0)
  (bind _aspawn (Utilities|Casting|CastToPawn (Components|GetOwner)))
  (if (and (Pawn|IsLocallyControlled _aspawn) (Pawn|IsPlayerControlled _aspawn))
    (CallFunction|ClientCreateCompassWidget)
    (Utilities|Time|SetTimerbyFunctionName 0 "GetPOIsInRange" 1.0 true)))

(fn GetPOIsinRange
  (Utilities|Array|Clear (Variables|Public|GetAllPOIs))
  (for _array_element (Collision|GetOverlappingActors (Components|GetOwner) "/Game/WorldCompassSystem/Blueprints/BP_MasterPOI.BP_MasterPOI_C" :!class /Script/Engine.Actor)
    (bind _asbp_master_poi (Utilities|Casting|CastToBP_MasterPOI _array_element))
    (Utilities|Array|Add (Variables|Public|GetAllPOIs) _asbp_master_poi)))