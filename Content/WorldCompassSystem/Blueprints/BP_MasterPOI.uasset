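; BP_MasterPOI is the base point-of-interest actor for the world compass system, with lifetime behavior chosen by its Type.
; Timed Removal destroys it after a set delay from BeginPlay.
; Removes After Discovered waits for a player-controlled Character to overlap DiscoverRange, notifies that character's BP_CompassComponent, then destroys the POI.
; The construction script sizes VisibilityCollision to twice the maximum icon visibility distance.
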(event OnComponentBeginOverlap(DiscoverRange)
  (params (OverlappedComponent :type Primitive%20Component%20Object%20Reference) (OtherActor :type Actor%20Object%20Reference) (OtherComp :type Primitive%20Component%20Object%20Reference) (OtherBodyIndex :type Integer) (bFromSweep :type Boolean) (SweepResult :type Hit%20Result%20Structure%20%28by%20ref%29))
  (switch Utilities|FlowControl|Switch|SwitchonE_CompassPOI_Type (Variables|Default|GetType)
    (:NewEnumerator0
      (bind _ascharacter (Utilities|Casting|CastToCharacter OtherActor))
      (if (Pawn|IsPlayerControlled _ascharacter)
        (Default|ClientFoundPOI (Actor|GetComponentbyClass _ascharacter "/Game/WorldCompassSystem/Blueprints/BP_CompassComponent.BP_CompassComponent_C") self)
        (Actor|DestroyActor)))))

(event EventBeginPlay
  (switch Utilities|FlowControl|Switch|SwitchonE_CompassPOI_Type (Variables|Default|GetType)
    (:NewEnumerator3
      (Utilities|FlowControl|Delay (Variables|Default|GetTimedRemovalValue))
      (Actor|DestroyActor))))

(fn ConstructionScript
  (Components|Sphere|SetSphereRadius (Variables|Default|GetVisibilityCollision) (* (Variables|Default|GetMaxIconVisibilityDistance) 2.0) true))